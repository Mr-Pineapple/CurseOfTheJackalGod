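; AC_AIComponent is an actor component that gives its owning character faction-based melee combat AI, weapons, damage reactions and death.
; A combat loop picks the nearest living enemy, moves to it, plays a random attack montage, then strafes or restarts.
; AttackTrace deals sphere-trace point damage, while TakeDamage handles frontal blocking, directional hit or knockdown montages and death.
; MC_ events wrap effects, and a delay-based TimelineMacro drives timed rotation and strafing.
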(event `Initiate`
  (params (OwningCharacter :type "Character Object Reference") (staticMeshesToFade :type "Array of StaticMeshComponent Object Reference") (skeletalMeshesToFade :type "Array of SkeletalMeshComponent Object Reference"))
  (set `self.OwningCharacter` OwningCharacter)
  ;[0 0 0] Initiation event. Call from begin play of owning character and plug in the references from there
  (set `self.Static Meshes to Fade` staticMeshesToFade)
  (set `self.Skeletal Meshes to Fade` skeletalMeshesToFade)
  (`self.Setup Weapons`)
  (`self.MC_PlayMontage` (`self.SpawnAnimation`))
  (if (not (`self.inactive`))
    (`self.PlaySound` (`self.SpawnSound`) (`Actor.K2_GetActorLocation` (`self.OwningCharacter`)))
    (`KismetSystemLibrary.K2_SetTimerDelegate` (delegate `Combat Start`) 5.0 true)))

(event `Combat Start`
  (`self.StartCombat`))

(event `TakeDamage`
  (params (B :type "Float (double-precision)") (Location :type "Vector Structure") (AttackingActor :type "Actor Object Reference") (`Knockdown?` :type Boolean))
  (if (`self.isBlocking`)
    (if (`self.checkIfActorIsInFront` AttackingActor)
      (`self.MC_PlayMontage` (`self.BlockHit`))
      (else
        (`self.Event_DamageFX` Location AttackingActor `Knockdown?` :!label _label)
        (set `self.currentHealth` (+ (`self.currentHealth`) B))
        (`self.resetCombat`)
        (if (< (`self.currentHealth`) 1.0)
          (`self.Death`))))
    (else
      (goto _label))))

(event `_HitFX`
  (params (SystemTemplate :type "NiagaraSystem Object Reference") (Location :type "Vector Structure") (Hitsound :type "SoundBase Object Reference"))
  (`self.MC_HitFX` SystemTemplate Location Hitsound)
  (if (`self.useGroundBlood`)
    (`|SpawnActorFromClass` "/Game/AI_Component/Decal_GroundBlood.Decal_GroundBlood_C" (`KismetMathLibrary.MakeTransform` (- (`Actor.K2_GetActorLocation` (`self.OwningCharacter`)) (0.0 0.0 100.0)) (`KismetMathLibrary.MakeRotator` 0.0 0.0 (`KismetMathLibrary.RandomFloatInRange` 0.0 360.0))) "Undefined" "MultiplyWithRoot" null null)))

(event `Event_DamageFX`
  (params (Location :type "Vector Structure") (AttackingActor :type "Actor Object Reference") (`Knockdown?` :type Boolean))
  (`self._HitFX` (`KismetArrayLibrary.Array_Random` (`self.HitEffects`)) Location (`self.Hitsound`))
  (if `Knockdown?`
    (`self.decideKnockdownDirection` AttackingActor)
    (else
      (`self.decideDamageDirection` AttackingActor)))
  (if (`self.useHitstop`)
    (`self.MC_Hitstop`)))

(event `MC_HitFX`
  (params (SystemTemplate :type "NiagaraSystem Object Reference") (Location :type "Vector Structure") (Hitsound :type "SoundBase Object Reference"))
  (`NiagaraFunctionLibrary.SpawnSystemAttached` SystemTemplate (`Character.CapsuleComponent` (`self.OwningCharacter`)) "pelvis" (0.0 0.0 0.0) (`KismetMathLibrary.RandomRotator` true) "KeepRelativeOffset" true)
  (`GameplayStatics.PlaySoundAtLocation` Hitsound (0.0 0.0 0.0) (struct) 1.0 1.0 0.0 null null null null))

(event `Death`
  (bind _owningcharacter (`self.OwningCharacter`))
  (`self.MC_DeathSound`)
  (set `/Game/COMMON/COMPONENTS/AI_Component/AC_AI_TargetComponent.dead` true (`Actor.GetComponentByClass` (`self.OwningCharacter`) "/Game/COMMON/COMPONENTS/AI_Component/AC_AI_TargetComponent.AC_AI_TargetComponent_C"))
  (`MovementComponent.StopMovementImmediately` (`Character.CharacterMovement` _owningcharacter))
  (`Pawn.DetachFromControllerPendingDestroy` _owningcharacter)
  (`self.MC_playMontage` (`self.deathAnimation`))
  (`self.MC_SetCollisionResponseToChannel`)
  (`KismetSystemLibrary.Delay` 4.0)
  (`Actor.K2_DestroyActor` (`self.OwningCharacter`))
  (`self.On Destroyed`))

(event `MC_DeathSound`
  (`GameplayStatics.PlaySoundAtLocation` (`self.deathSound`) (`Actor.K2_GetActorLocation` (`self.OwningCharacter`)) (struct) 1.0 1.0 0.0 null null null null))

(event `MC_Hitstop`
  (bind _mesh (`Character.Mesh` (`self.OwningCharacter`)))
  (set `SkeletalMeshComponent.GlobalAnimRateScale` 0.2 _mesh)
  (`KismetSystemLibrary.RetriggerableDelay` 0.2)
  (set `SkeletalMeshComponent.GlobalAnimRateScale` 1.0 _mesh))

(event `MC_PlayMontage`
  (params (AnimMontage :type "AnimMontage Object Reference"))
  (bind _returnvalue (`Character.PlayAnimMontage` (`self.OwningCharacter`) AnimMontage 1.0 "None"))
  (set `self.montageDelay` _returnvalue))

(event `PlayMontage`
  (params (AnimMontage :type "AnimMontage Object Reference"))
  (`self.MC_PlayMontage` AnimMontage))

(event `MC_SetCollisionResponseToChannel`
  (`PrimitiveComponent.SetCollisionResponseToChannel` (`Character.CapsuleComponent` (`self.OwningCharacter`)) "ECC_Pawn" "ECR_Ignore"))

(event `PlaySound`
  (params (Sound :type "SoundBase Object Reference") (Location :type "Vector Structure"))
  (`self.MC_PlaySound` Sound Location))

(event `MC_PlaySound`
  (params (Sound :type "SoundBase Object Reference") (Location :type "Vector Structure"))
  (`GameplayStatics.PlaySoundAtLocation` Sound Location (struct) 1.0 1.0 0.0 null null null null))

(event `Strafing`
  (params (Seconds :type "Float (double-precision)"))
  (if (`self.targetDeathCheck`)
    (`self.resetCombat`)
    (else
      (`self.decideStrafeDirection`)
      (set `CharacterMovementComponent.bOrientRotationToMovement` false (`Character.CharacterMovement` (`self.OwningCharacter`)))
      (`self.setMaxWalkspeed` 175.0)
      (bind _progress (`self.TimelineMacro` Seconds :!label _label_2)
        (:`Update`
          (if (`self.targetDeathCheck`)
            (set `CharacterMovementComponent.bOrientRotationToMovement` true (`Character.CharacterMovement` (`self.OwningCharacter`)) :!label _label_3)
            (`self.resetCombat`)
            (goto _label_2 :!via `Stop`)
            (elif (`/Game/COMMON/COMPONENTS/AI_Component/AC_AI_TargetComponent.dead` (`Actor.GetComponentByClass` (`self.OwningCharacter`) "/Game/COMMON/COMPONENTS/AI_Component/AC_AI_TargetComponent.AC_AI_TargetComponent_C"))
              (goto _label_2 :!via `Stop`)
              (else
                (`Actor.K2_SetActorRotation` (`self.OwningCharacter`) (`KismetMathLibrary.RLerp` (`Actor.K2_GetActorRotation` (`self.OwningCharacter`)) (`self.helper_GetTargetRotation`) _progress true) false)
                (`Pawn.AddMovementInput` (`self.OwningCharacter`) (`self.StrafingDirectionVector`) 1.0 false)))))
        (:`Finish`
          (goto _label_3))))))

(event `StartCombat`
  ;[0 0 0] Combat initiation
  ;;[0 0 0] Search for targets and assign new target
  (`self.searchForTargets` :!label _label_4)
  (`self.findClosestTarget`)
  ;;[0 0 0] set to run speed if target iis far away
  (`self.checkTargetDistance`)
  (`self.randomizeWalkSpeed`)
  (`|AIMoveTo` (`self.OwningCharacter`) (0.0 0.0 0.0) (`self.TargetUnit`) 150.0 true
    (:`OnSuccess`
      (if (`self.canTakeAction`)
        (if (or (`/Game/COMMON/COMPONENTS/AI_Component/AC_AI_TargetComponent.dead` (`Actor.GetComponentByClass` (`self.OwningCharacter`) "/Game/COMMON/COMPONENTS/AI_Component/AC_AI_TargetComponent.AC_AI_TargetComponent_C")) (`self.targetDeathCheck`))
          (`self.resetCombat`)
          (else
            (`self.PlayMontage` (`KismetArrayLibrary.Array_Random` (`self.AttackMontages`)))
            (`KismetSystemLibrary.Delay` (- (`self.montageDelay`) 0.2))
            ;;[0 0 0] Another target death check
            (if (`self.targetDeathCheck`)
              (`self.resetCombat`)
              (elif (`self.canTakeAction`)
                (if (> (`self.strafeChance`) (`KismetMathLibrary.RandomFloatInRange` 0.0 100.0))
                  (`self.Strafing` (`KismetMathLibrary.RandomFloatInRange` 1.0 2.0))
                  (else
                    (`self.resetCombat`)))
                (else
                  (`self.resetCombat`))))))
        (else
          ;[0 0 0] Retry doing action if we are already taking action untill  variable is set to true (Controlled via animation state added to animations)
          (`KismetSystemLibrary.RetriggerableDelay` 0.2)
          (`self.resetCombat`))))))

(event `RotateToTarget`
  (bind _owningcharacter (`self.OwningCharacter`))
  (bind (_returnvalue_roll _returnvalue_pitch) (`KismetMathLibrary.BreakRotator` (`Actor.K2_GetActorRotation` _owningcharacter)))
  (bind (_returnvalue_roll_2 _returnvalue_pitch_2 _returnvalue_yaw) (`KismetMathLibrary.BreakRotator` (`KismetMathLibrary.FindLookAtRotation` (`Actor.K2_GetActorLocation` _owningcharacter) (`Actor.K2_GetActorLocation` (`self.TargetUnit`)))))
  (`/Engine/EditorBlueprintResources/StandardMacros.IsValid` (`self.TargetUnit`)
    (:`Is Valid`
      (bind _progress (`self.TimelineMacro` 0.5 :!label _label_5)
        (:`Update`
          (if (`/Game/COMMON/COMPONENTS/AI_Component/AC_AI_TargetComponent.dead` (`Actor.GetComponentByClass` (`self.OwningCharacter`) "/Game/COMMON/COMPONENTS/AI_Component/AC_AI_TargetComponent.AC_AI_TargetComponent_C"))
            (goto _label_5 :!via `Stop`)
            (elif (`self.targetDeathCheck`)
              (`self.resetCombat`)
              (goto _label_5 :!via `Stop`)
              (else
                (`Actor.K2_SetActorRotation` (`self.OwningCharacter`) (`KismetMathLibrary.RLerp` (`Actor.K2_GetActorRotation` (`self.OwningCharacter`)) (`KismetMathLibrary.MakeRotator` _returnvalue_roll _returnvalue_pitch _returnvalue_yaw) _progress true) false)))))))))

(event `resetCombat`
  ;[0 0 0] Combat initiation
  ;;[0 0 0] dont execute multiple times untill reset
  (`|ExecutionSequence`
    (:`then_0`
      (goto _label_4))
    (:`then_1`
      (`self.StartCombat`))))

(fn `attackTrace`
  (locals (hitEnemy :type "Actor Object Reference"))
  (bind _owningcharacter (`self.OwningCharacter`))
  (bind _returnvalue (`Actor.K2_GetActorLocation` _owningcharacter))
  (bind _outhits (`KismetSystemLibrary.SphereTraceMulti` _returnvalue (+ _returnvalue (* (`Actor.GetActorForwardVector` _owningcharacter) (`self.attackRange`))) 10.0 "TraceTypeQuery3" false (`|MakeArray` (`self.GetOwner`))))
  (for _array_element _outhits
    (bind (_bblockinghit _binitialoverlap _time _distance _location _impactpoint _normal _impactnormal _physmat _hitactor) (`GameplayStatics.BreakHitResult` _array_element))
    (set `local.hitEnemy` _hitactor)
    (if (not (`KismetArrayLibrary.Array_Contains` (`self.AlreadyDamagedActors`) _hitactor))
      (bind _returnvalue_2 (`Actor.GetComponentByClass` _hitactor "/Game/COMMON/COMPONENTS/AI_Component/AC_AI_TargetComponent.AC_AI_TargetComponent_C"))
      (`/Engine/EditorBlueprintResources/StandardMacros.IsValid` _returnvalue_2
        (:`Is Valid`
          (if (`|EnumInequality` (`/Game/COMMON/COMPONENTS/AI_Component/AC_AI_TargetComponent.Faction` _returnvalue_2) (`/Game/COMMON/COMPONENTS/AI_Component/AC_AI_TargetComponent.Faction` (`Actor.GetComponentByClass` (`self.OwningCharacter`) "/Game/COMMON/COMPONENTS/AI_Component/AC_AI_TargetComponent.AC_AI_TargetComponent_C")))
            (`KismetArrayLibrary.Array_Add` (`self.AlreadyDamagedActors`) (`local.hitEnemy`))
            ;[0 0 0] remember to do - damage otherwise AI will heal when fighting eachother. use "point damage" event on player to get damage
            (`GameplayStatics.ApplyPointDamage` (`local.hitEnemy`) (`self.attackDamage`) _impactnormal _array_element null (`self.OwningCharacter`) "/Script/Engine.DamageType")
            (if (`self.useHitstop`)
              (`self.MC_Hitstop`)))))))
  (`KismetArrayLibrary.Array_Clear` (`self.AlreadyDamagedActors`)))

(fn `checkIfActorIsInFront`
  (params (ActorToCheck :type "Actor Object Reference"))
  (returns (`inFront?` :type Boolean))
  (bind (_returnvalue_roll _returnvalue_pitch _returnvalue_yaw) (`KismetMathLibrary.BreakRotator` (`Actor.K2_GetActorRotation` (`self.OwningCharacter`))))
  (bind (_returnvalue_roll_2 _returnvalue_pitch_2 _returnvalue_yaw_2) (`KismetMathLibrary.BreakRotator` (`KismetMathLibrary.FindLookAtRotation` (`Actor.K2_GetActorLocation` (`self.OwningCharacter`)) (`Actor.K2_GetActorLocation` ActorToCheck))))
  (bind _returnvalue (/ (- _returnvalue_yaw_2 _returnvalue_yaw) 90.0))
  (`/Engine/EditorBlueprintResources/StandardMacros.IsValid` ActorToCheck
    (:`Is Valid`
      (return (and (< _returnvalue 1.0) (> _returnvalue -1.0))))))

(fn `checkTargetDistance`
  (if (> (`Actor.GetDistanceTo` (`self.OwningCharacter`) (`self.TargetUnit`)) 800.0)
    (`self.setMaxWalkspeed` (`self.RunSpeed`)))
  (return))

(fn `decideDamageDirection`
  (params (AttackingActor :type "Actor Object Reference"))
  (locals (ReactionRotation :type "Float (single-precision)" :default 0.0))
  (bind _reactionrotation (`local.ReactionRotation`))
  (bind (_outlocation _outrotation) (`Actor.GetActorEyesViewPoint` (`self.OwningCharacter`)))
  (bind (_returnvalue_roll _returnvalue_pitch _returnvalue_yaw) (`KismetMathLibrary.BreakRotator` (`KismetMathLibrary.NormalizedDeltaRotator` _outrotation (`KismetMathLibrary.FindLookAtRotation` _outlocation (`Actor.K2_GetActorLocation` AttackingActor)))))
  (set `local.ReactionRotation` _returnvalue_yaw)
  (`/Engine/EditorBlueprintResources/StandardMacros.IsValid` AttackingActor
    (:`Is Valid`
      (set `self.ChosenHitMontage` (select `bool` (`KismetMathLibrary.InRange_FloatFloat` _reactionrotation -45.0 45.0 false false) :`false` (select `bool` (`KismetMathLibrary.InRange_FloatFloat` _reactionrotation 45.0 135.0) :`false` (select `bool` (`KismetMathLibrary.InRange_FloatFloat` _reactionrotation -135.0 -45.0) :`false` (`KismetArrayLibrary.Array_Random` (`self.hitReactionsB`)) :`true` (`KismetArrayLibrary.Array_Random` (`self.hitReactionsR`))) :`true` (`KismetArrayLibrary.Array_Random` (`self.hitReactionsL`))) :`true` (`KismetArrayLibrary.Array_Random` (`self.hitReactionsF`))))
      ;[0 0 0] Play the chosen hit reaction
      (`/Engine/EditorBlueprintResources/StandardMacros.IsValid` (`self.OwningCharacter`)
        (:`Is Valid`
          (`self.PlayMontage` (`self.ChosenHitMontage`))
          (return))))))

(fn `decideKnockdownDirection`
  (params (AttackingActor :type "Actor Object Reference"))
  (locals (ReactionRotation :type "Float (single-precision)" :default 0.0))
  (bind (_outlocation _outrotation) (`Actor.GetActorEyesViewPoint` (`self.OwningCharacter`)))
  (bind (_returnvalue_roll _returnvalue_pitch _returnvalue_yaw) (`KismetMathLibrary.BreakRotator` (`KismetMathLibrary.NormalizedDeltaRotator` _outrotation (`KismetMathLibrary.FindLookAtRotation` _outlocation (`Actor.K2_GetActorLocation` AttackingActor)))))
  (set `local.ReactionRotation` _returnvalue_yaw)
  (`/Engine/EditorBlueprintResources/StandardMacros.IsValid` AttackingActor
    (:`Is Valid`
      (set `self.ChosenHitMontage` (select `bool` (`KismetMathLibrary.InRange_FloatFloat` (`local.ReactionRotation`) -90.0 90.0 false false) :`false` (`KismetArrayLibrary.Array_Random` (`self.KnockdownB`)) :`true` (`KismetArrayLibrary.Array_Random` (`self.KnockdownF`))))
      ;[0 0 0] Play the chosen hit reaction
      (`/Engine/EditorBlueprintResources/StandardMacros.IsValid` (`self.OwningCharacter`)
        (:`Is Valid`
          (`self.PlayMontage` (`self.ChosenHitMontage`))
          (return))))))

(fn `decideStrafeDirection`
  (bind _owningcharacter (`self.OwningCharacter`))
  (bind _returnvalue (`Actor.GetActorRightVector` _owningcharacter))
  (switch `int` (`KismetMathLibrary.RandomIntegerInRange` 0 2)
    (:`0`
      ;[0 0 0] 0 = Right
      ; 1 = Left
      ; 2 = Back
      (set `self.StrafingDirectionVector` _returnvalue))
    (:`1`
      (set `self.StrafingDirectionVector` (* _returnvalue -1.0)))
    (:`2`
      (set `self.StrafingDirectionVector` (* (`Actor.GetActorForwardVector` _owningcharacter) -1.0))))
  (return))

(fn `findClosestTarget`
  (locals (ClosestTarget :type "Float (double-precision)"))
  (set `local.ClosestTarget` 10000.0)
  (for _array_element (`self.AllTargets`)
    (bind _returnvalue (`Actor.GetDistanceTo` (`self.OwningCharacter`) _array_element))
    (if (< _returnvalue (`local.ClosestTarget`))
      (set `local.ClosestTarget` _returnvalue)
      (set `self.TargetUnit` _array_element))))

(fn `helper_GetTargetRotation`
  (returns (ReturnValue :type "Rotator Structure"))
  (bind _targetunit (`self.TargetUnit`))
  (bind _owningcharacter (`self.OwningCharacter`))
  (bind (_returnvalue_roll _returnvalue_pitch) (`KismetMathLibrary.BreakRotator` (`Actor.K2_GetActorRotation` _owningcharacter)))
  (bind (_returnvalue_roll_2 _returnvalue_pitch_2 _returnvalue_yaw) (`KismetMathLibrary.BreakRotator` (`KismetMathLibrary.FindLookAtRotation` (`Actor.K2_GetActorLocation` _owningcharacter) (`Actor.K2_GetActorLocation` _targetunit))))
  (`/Engine/EditorBlueprintResources/StandardMacros.IsValid` _targetunit
    (:`Is Valid`
      (return (`KismetMathLibrary.MakeRotator` _returnvalue_roll _returnvalue_pitch _returnvalue_yaw)))))

(fn `randomizeWalkSpeed`
  (if (> (`KismetMathLibrary.RandomFloatInRange` 0.0 100.0) 50.0)
    (`self.setMaxWalkspeed` (`self.WalkSpeed`))
    (else
      (`self.setMaxWalkspeed` (`self.RunSpeed`)))))

(fn `searchForTargets`
  (`|ExecutionSequence`
    (:`then_0`
      (`KismetArrayLibrary.Array_Clear` (`self.AllTargets`))
      ;[1 1 1] Get All AI Character Classes
      (bind _outactors (`GameplayStatics.GetAllActorsOfClass` "/Game/COMMON/ENTITIES/Character1.Character1_C"))
      (for _array_element _outactors
        (bind _returnvalue (`Actor.GetComponentByClass` _array_element "/Game/COMMON/COMPONENTS/AI_Component/AC_AI_TargetComponent.AC_AI_TargetComponent_C"))
        (`/Engine/EditorBlueprintResources/StandardMacros.IsValid` _returnvalue
          (:`Is Valid`
            (if (and (not (`/Game/COMMON/COMPONENTS/AI_Component/AC_AI_TargetComponent.dead` _returnvalue)) (`|EnumInequality` (`/Game/COMMON/COMPONENTS/AI_Component/AC_AI_TargetComponent.Faction` _returnvalue) (`/Game/COMMON/COMPONENTS/AI_Component/AC_AI_TargetComponent.Faction` (`Actor.GetComponentByClass` (`self.OwningCharacter`) "/Game/COMMON/COMPONENTS/AI_Component/AC_AI_TargetComponent.AC_AI_TargetComponent_C"))))
              (`KismetArrayLibrary.Array_Add` (`self.AllTargets`) _array_element))))))
    (:`then_1`
      (bind _outactors_2 (`GameplayStatics.GetAllActorsOfClass` "/Game/COMMON/ENTITIES/Character2.Character2_C"))
      (for _array_element_2 _outactors_2
        (bind _returnvalue_2 (`Actor.GetComponentByClass` _array_element_2 "/Game/COMMON/COMPONENTS/AI_Component/AC_AI_TargetComponent.AC_AI_TargetComponent_C"))
        (`/Engine/EditorBlueprintResources/StandardMacros.IsValid` _returnvalue_2
          (:`Is Valid`
            (if (and (not (`/Game/COMMON/COMPONENTS/AI_Component/AC_AI_TargetComponent.dead` _returnvalue_2)) (`|EnumInequality` (`/Game/COMMON/COMPONENTS/AI_Component/AC_AI_TargetComponent.Faction` _returnvalue_2) (`/Game/COMMON/COMPONENTS/AI_Component/AC_AI_TargetComponent.Faction` (`Actor.GetComponentByClass` (`self.OwningCharacter`) "/Game/COMMON/COMPONENTS/AI_Component/AC_AI_TargetComponent.AC_AI_TargetComponent_C"))))
              (`KismetArrayLibrary.Array_Add` (`self.AllTargets`) _array_element_2))))))
    (:`then_2`
      (bind _outactors_3 (`GameplayStatics.GetAllActorsOfClass` "/Game/COMMON/ENTITIES/Character3.Character3_C"))
      (for _array_element_3 _outactors_3
        (bind _returnvalue_3 (`Actor.GetComponentByClass` _array_element_3 "/Game/COMMON/COMPONENTS/AI_Component/AC_AI_TargetComponent.AC_AI_TargetComponent_C"))
        (`/Engine/EditorBlueprintResources/StandardMacros.IsValid` _returnvalue_3
          (:`Is Valid`
            (if (and (not (`/Game/COMMON/COMPONENTS/AI_Component/AC_AI_TargetComponent.dead` _returnvalue_3)) (`|EnumInequality` (`/Game/COMMON/COMPONENTS/AI_Component/AC_AI_TargetComponent.Faction` _returnvalue_3) (`/Game/COMMON/COMPONENTS/AI_Component/AC_AI_TargetComponent.Faction` (`Actor.GetComponentByClass` (`self.OwningCharacter`) "/Game/COMMON/COMPONENTS/AI_Component/AC_AI_TargetComponent.AC_AI_TargetComponent_C"))))
              (`KismetArrayLibrary.Array_Add` (`self.AllTargets`) _array_element_3))))))
    (:`then_3`
      (bind _outactors_4 (`GameplayStatics.GetAllActorsOfClass` "/Game/COMMON/ENTITIES/Character4.Character4_C"))
      (for _array_element_4 _outactors_4
        (bind _returnvalue_4 (`Actor.GetComponentByClass` _array_element_4 "/Game/COMMON/COMPONENTS/AI_Component/AC_AI_TargetComponent.AC_AI_TargetComponent_C"))
        (`/Engine/EditorBlueprintResources/StandardMacros.IsValid` _returnvalue_4
          (:`Is Valid`
            (if (and (not (`/Game/COMMON/COMPONENTS/AI_Component/AC_AI_TargetComponent.dead` _returnvalue_4)) (`|EnumInequality` (`/Game/COMMON/COMPONENTS/AI_Component/AC_AI_TargetComponent.Faction` _returnvalue_4) (`/Game/COMMON/COMPONENTS/AI_Component/AC_AI_TargetComponent.Faction` (`Actor.GetComponentByClass` (`self.OwningCharacter`) "/Game/COMMON/COMPONENTS/AI_Component/AC_AI_TargetComponent.AC_AI_TargetComponent_C"))))
              (`KismetArrayLibrary.Array_Add` (`self.AllTargets`) _array_element_4)))))
      (return))))

(fn `setMaxWalkspeed`
  (params (`Max Walk Speed` :type "Float (single-precision)"))
  (set `CharacterMovementComponent.MaxWalkSpeed` `Max Walk Speed` (`Character.CharacterMovement` (`self.OwningCharacter`))))

(fn `Setup Weapons`
  (bind _static_meshes_to_fade (`self.Static Meshes to Fade`))
  ;[0 0 0] Create Main hand and Off hand static meshes. Repeat the logic for additional meshes if you want more for cosmetic reasons
  (bind _returnvalue (`|AddComponentByClass` :`self` (`self.OwningCharacter`) :`Class` "/Script/Engine.StaticMeshComponent"))
  (bind _output_get (set `self.mainHand` _returnvalue))
  (`StaticMeshComponent.SetStaticMesh` _output_get (`self.mainHandMesh`))
  (`SceneComponent.K2_AttachToComponent` _returnvalue (`Character.Mesh` (`self.OwningCharacter`)) (`self.mainHandEquipSocket`) "SnapToTarget" "SnapToTarget" "SnapToTarget" true)
  (bind _returnvalue_2 (`|AddComponentByClass` :`self` (`self.OwningCharacter`) :`Class` "/Script/Engine.StaticMeshComponent"))
  (bind _output_get_2 (set `self.offHand` _returnvalue_2))
  (`StaticMeshComponent.SetStaticMesh` _output_get_2 (`self.offHandMesh`))
  (`SceneComponent.K2_AttachToComponent` _returnvalue_2 (`Character.Mesh` (`self.OwningCharacter`)) (`self.offHandEquipSocket`) "SnapToTarget" "SnapToTarget" "SnapToTarget" true)
  ;;[0 0 0] Since we use tracing for damage we dont want collision to interfere
  (`PrimitiveComponent.SetCollisionEnabled` (`self.offHand`) "NoCollision")
  (`PrimitiveComponent.SetCollisionEnabled` (`self.mainHand`) "NoCollision")
  ;[0 0 0] Repeat for any additional added static meshes
  (`KismetArrayLibrary.Array_Add` _static_meshes_to_fade (`self.offHand`))
  (`KismetArrayLibrary.Array_Add` _static_meshes_to_fade (`self.mainHand`)))

(fn `targetDeathCheck`
  (returns (dead :type Boolean))
  (bind _targetunit (`self.TargetUnit`))
  (`/Engine/EditorBlueprintResources/StandardMacros.IsValid` _targetunit
    (:`Is Valid`
      (return (`/Game/COMMON/COMPONENTS/AI_Component/AC_AI_TargetComponent.dead` (`Actor.GetComponentByClass` _targetunit "/Game/COMMON/COMPONENTS/AI_Component/AC_AI_TargetComponent.AC_AI_TargetComponent_C"))))
    (:`Is Not Valid`
      (`self.resetCombat`))))
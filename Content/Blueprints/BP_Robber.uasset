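; BP_Robber is the player character for a stealth heist, with jewel carrying, ragdoll, return to start, and detection and timer widgets.
; It holds logic for movement, interface-based interaction and takedowns, dodge roll, pause and timeline-blended crouch with an overhead check before standing.
; Mantling sphere-traces for a ledge, picks a montage by distance and switches to flying mode.
; Motion warping aligns mantles and takedowns, and body-part meshes follow the main mesh's pose.
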(event `self.ReceiveBeginPlay`
  ;[1 1 1] Input and Movement
  (`EnhancedInputSubsystemInterface.AddMappingContext` (pcsubsystem `EnhancedInputLocalPlayerSubsystem` (`GameplayStatics.GetPlayerController` 0)) null 0 (struct))
  (bind _returnvalue (`|CreateWidget` "/Game/UI/WB_DetectionMeter.WB_DetectionMeter_C"))
  (bind _output_get (set `self.Detected Meter Widget` _returnvalue))
  (`UserWidget.AddToViewport` _output_get 0)
  (bind _returnvalue_2 (`|CreateWidget` "/Game/UI/WB_Timer.WB_Timer_C"))
  (bind _output_get_2 (set `self.Timer Widget` _returnvalue_2))
  (`UserWidget.AddToViewport` _output_get_2 0))

(event `Ragdoll`
  (`PrimitiveComponent.SetSimulatePhysics` (`self.Mesh`) true)
  (`self.DisableInput` null))

(event `Resume`
  (bind _returnvalue (`GameplayStatics.GetPlayerController` 0))
  (set `self.paused?` false)
  (set `PlayerController.bShowMouseCursor` false _returnvalue)
  (`WidgetBlueprintLibrary.SetInputMode_GameOnly` _returnvalue)
  (`GameplayStatics.SetGamePaused` false))

(event `Equip Jewel`
  (`SceneComponent.SetVisibility` (`self.Jewel`) true false)
  (set `self.hasJewel` true))

(event `Go To Start`
  (bind _returnvalue (`GameplayStatics.GetActorOfClass` "/Script/Engine.PlayerStart"))
  (`self.K2_SetActorLocation` (`self.K2_GetActorLocation` _returnvalue)))

(fn `Uncrouch Obstacle Detection`
  (returns (`Hit?` :type Boolean))
  (bind _returnvalue (`self.K2_GetActorLocation`))
  (bind (_outhit _returnvalue_2) (`KismetSystemLibrary.SphereTraceSingle` :`Start` _returnvalue :`End` (+ _returnvalue (* (`KismetMathLibrary.GetUpVector` (`self.K2_GetActorRotation`)) 115.0)) :`Radius` 15.0 :`TraceChannel` "TraceTypeQuery1" :`DrawDebugType` "ForDuration"))
  (return _returnvalue_2))

(fn `UserConstructionScript`
  (`SkinnedMeshComponent.SetLeaderPoseComponent` (`self.Torso`) (`self.Mesh`) false false)
  (`SkinnedMeshComponent.SetLeaderPoseComponent` (`self.Head`) (`self.Mesh`) false false)
  (`SkinnedMeshComponent.SetLeaderPoseComponent` (`self.Hands`) (`self.Mesh`) false false)
  (`SkinnedMeshComponent.SetLeaderPoseComponent` (`self.Foot`) (`self.Mesh`) false false)
  (`SkinnedMeshComponent.SetLeaderPoseComponent` (`self.Pants`) (`self.Mesh`) false false))
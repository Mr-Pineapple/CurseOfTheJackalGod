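; BP_JeremyStatue is a statue prop with a skeletal mesh, apparently an unfinished setup for a head that looks at the player.
; On BeginPlay it finds the Character1 actor and stores its mesh world location and the statue's Head socket location, once.
; A FindLookAtRotation between those points is left unconnected and Tick is disabled, so nothing rotates.
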(event `self.ReceiveBeginPlay`
  (bind _returnvalue (`GameplayStatics.GetActorOfClass` "/Game/COMMON/ENTITIES/Characters/Character1.Character1_C"))
  (bind _output_get (set `self.Character1ref` _returnvalue))
  (set `self.Player World Location` (`SceneComponent.K2_GetComponentLocation` (`Character.Mesh` _output_get)))
  (set `self.HeadReference` (`SceneComponent.GetSocketLocation` (`self.SkeletalMesh`) "Head")))

(fn `UserConstructionScript`)
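; Puzzle trigger volume that raises BP_Door actors when any of four playable character classes enters its box.
; All doors in the level are cached at BeginPlay.
; On overlap, a loop over them restarts one shared VerticalTranslation timeline per door.
; The timeline update sets the current loop element's relative Z to a fixed height, using its world X and Y, without an interpolated value.
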(event `self.ReceiveBeginPlay`
  (bind _outactors (`GameplayStatics.GetAllActorsOfClass` "/Game/BP_Door.BP_Door_C"))
  (set `self.BP_Doors` _outactors))

(event `self.Box.OnComponentBeginOverlap`
  (params (OverlappedComponent :type "PrimitiveComponent Object Reference") (OtherActor :type "Actor Object Reference") (OtherComp :type "PrimitiveComponent Object Reference") (OtherBodyIndex :type Integer) (bFromSweep :type Boolean) (SweepResult :type "HitResult Structure (by ref)"))
  (cast `/Game/COMMON/ENTITIES/Character1` OtherActor
    (:`then`
      _)
    (:`CastFailed`
      (cast `/Game/COMMON/ENTITIES/Character2` OtherActor
        (:`then`
          _)
        (:`CastFailed`
          (cast `/Game/COMMON/ENTITIES/Character3` OtherActor
            (:`then`
              _)
            (:`CastFailed`
              (cast `/Game/COMMON/ENTITIES/Character4` OtherActor)))))))
  (for _array_element (`self.BP_Doors`)
    (`Timeline|VerticalTranslation` :!via `PlayFromStart`
      (:`Update`
        (bind (_returnvalue_x _returnvalue_y) (`KismetMathLibrary.BreakVector` (`self.K2_GetActorLocation` _array_element)))
        (`self.K2_SetActorRelativeLocation` _array_element (`KismetMathLibrary.MakeVector` _returnvalue_x _returnvalue_y 2000.0) false false)))))

(fn `UserConstructionScript`)
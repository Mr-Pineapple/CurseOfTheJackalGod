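; Player stealth component that handles rock throwing, smoke bombs, their inventory counts and HUD hints.
; While aiming, a looping timer predicts the rock's projectile path, stores its points and eases the camera pitch toward the landing spot.
; Mouse or gamepad Y adjusts throw distance, and a montage notify spawns the rock with the predicted velocity.
; Throwing disables movement, and the node restoring walking is unconnected, as is the behind-the-victim assassination check.
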(fn `Aim Distance Gamepad`
  (params (A :type "Float (double-precision)"))
  (bind _returnvalue (`KismetMathLibrary.FInterpTo` (`self.Rock_Direction`) (+ (`self.Rock_Direction`) (* A -1.0)) (`GameplayStatics.GetWorldDeltaSeconds`) 1.0))
  (if (`self.Rock_Aiming`)
    (if (and (> _returnvalue -0.75) (< _returnvalue 1.5))
      (set `self.Rock_Direction` _returnvalue))))

(fn `AimDistance_Mouse`
  (params (A :type "Float (double-precision)"))
  (bind _returnvalue (`KismetMathLibrary.FInterpTo` (`self.Rock_Direction`) (+ (`self.Rock_Direction`) (* A 1.3)) (`GameplayStatics.GetWorldDeltaSeconds`) 1.0))
  (if (`self.Rock_Aiming`)
    (if (and (> _returnvalue -0.5) (< _returnvalue 0.9))
      (set `self.Rock_Direction` _returnvalue))))

(fn `RockTrajectory`
  (returns (OutPathPositions :type "Array of Vector Structure") (Distance :type "Float (single-precision)") (Location :type "Vector Structure"))
  (bind _throwlocationref (`self.ThrowLocationRef`))
  (bind _rock_direction (`self.Rock_Direction`))
  (bind _returnvalue (`KismetMathLibrary.GetForwardVector` (`SceneComponent.K2_GetComponentRotation` _throwlocationref)))
  (bind _output_get (set `self.Rock_Velocity` (* (+ _returnvalue (* _returnvalue _rock_direction)) (`self.Rock_ProjectileSpeed`))))
  (bind (_outhit _outpathpositions) (`GameplayStatics.Blueprint_PredictProjectilePath_ByTraceChannel` (+ (`SceneComponent.K2_GetComponentLocation` _throwlocationref) _returnvalue) _output_get true 10.0 "ECC_Visibility" false (`|MakeArray` (`self.Rock_Ref`) :!type "Actor Object Reference") "None" 0.0 (`KismetMathLibrary.Lerp` 3.0 14.0 (+ _rock_direction 0.5))))
  (bind (_bblockinghit _binitialoverlap _time _distance _location) (`GameplayStatics.BreakHitResult` _outhit))
  (return _outpathpositions _distance _location))

(fn `StealthInterface_DeleteSplines`
  (params (SplineArray :type "Array of SplineMeshComponent Object Reference (by ref)"))
  (return))

(fn `ThrowRock_PitchTowardsTarget`
  (params (Location :type "Vector Structure"))
  (bind _returnvalue (`GameplayStatics.GetPlayerCharacter` 0))
  (bind _returnvalue_2 (`Pawn.GetController` _returnvalue))
  (bind _returnvalue_3 (`Controller.GetControlRotation` _returnvalue_2))
  (bind (_returnvalue_roll _returnvalue_pitch _returnvalue_yaw) (`KismetMathLibrary.BreakRotator` (`KismetMathLibrary.FindLookAtRotation` (`SceneComponent.K2_GetComponentLocation` (`self.CameraRef`)) Location)))
  (`/Engine/EditorBlueprintResources/StandardMacros.IsValid` _returnvalue
    (:`Is Valid`
      (`/Engine/EditorBlueprintResources/StandardMacros.IsValid` _returnvalue_2
        (:`Is Valid`
          (`Controller.SetControlRotation` _returnvalue_2 (`KismetMathLibrary.MakeRotator` (.roll _returnvalue_3) (.pitch (`KismetMathLibrary.RInterpTo` _returnvalue_3 (`KismetMathLibrary.MakeRotator` _returnvalue_roll _returnvalue_pitch _returnvalue_yaw) (`GameplayStatics.GetWorldDeltaSeconds`) 7.0)) (.yaw _returnvalue_3))))))))
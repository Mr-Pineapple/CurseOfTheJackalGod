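; Smoke bomb actor that plays a Niagara explosion on spawn and notifies characters caught inside it.
; Shortly after BeginPlay it sends an entered message to overlapping Characters through the first component implementing SmokeBomb_BPI.
; After a fixed lifetime it sends an exited message to those overlapping then, and destroys itself.
; Overlaps are sampled only at those two moments, so movement in or out between them is untracked.
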(event `self.ReceiveBeginPlay`
  (`NiagaraFunctionLibrary.SpawnSystemAtLocation` "/Game/COMMON/Pickups/PoisonSeed_Explosion_NS.PoisonSeed_Explosion_NS" (`self.K2_GetActorLocation`))
  (`KismetSystemLibrary.Delay` 0.2)
  (for _array_element (`self.GetOverlappingActors` "/Script/Engine.Character")
    (bind _returnvalue (`self.GetComponentsByInterface` _array_element "/Game/COMMON/Pickups/SmokeBomb_BPI.SmokeBomb_BPI_C"))
    (if (`KismetArrayLibrary.Array_IsValidIndex` _returnvalue)
      (bind _output (`|GetArrayItem` _returnvalue))
      (`/Engine/EditorBlueprintResources/StandardMacros.IsValid` _output
        (:`Is Valid`
          (message `/Game/COMMON/Pickups/SmokeBomb_BPI.EnteredSmokeBomb` _output)))))
  (`KismetSystemLibrary.Delay` 7.0)
  (for _array_element_2 (`self.GetOverlappingActors` "/Script/Engine.Character")
    (bind _returnvalue_2 (`self.GetComponentsByInterface` _array_element_2 "/Game/COMMON/Pickups/SmokeBomb_BPI.SmokeBomb_BPI_C"))
    (if (`KismetArrayLibrary.Array_IsValidIndex` _returnvalue_2)
      (bind _output_2 (`|GetArrayItem` _returnvalue_2))
      (`/Engine/EditorBlueprintResources/StandardMacros.IsValid` _output_2
        (:`Is Valid`
          (message `/Game/COMMON/Pickups/SmokeBomb_BPI.ExitedSmokeBomb` _output_2)))))
  (`self.K2_DestroyActor`))

(fn `UserConstructionScript`)
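; Guard enemy character that chases, attacks and can be targeted for lock-on or killed by a player takedown.
; Catch plays a montage whose notify sphere-traces ahead to damage the player; damage taken drains health until the actor is destroyed.
; An overlap radius shows the takedown prompt; Takedown plays the victim montage, returns alignment transforms, flags the AI controller dead and triggers delayed ragdoll.
; Modular body meshes follow the main mesh pose.
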(event `self.Takedown Radius.OnComponentBeginOverlap`
  (params (OverlappedComponent :type "PrimitiveComponent Object Reference") (OtherActor :type "Actor Object Reference") (OtherComp :type "PrimitiveComponent Object Reference") (OtherBodyIndex :type Integer) (bFromSweep :type Boolean) (SweepResult :type "HitResult Structure (by ref)"))
  ;[1 1 1] Begin Overlap Event
  (if (and (`self.ActorHasTag` OtherActor "Player") (not (`self.dead`)))
    (`SceneComponent.SetVisibility` (`self.Takedown Prompt Widget`) true false)))

(event `self.Takedown Radius.OnComponentEndOverlap`
  (params (OverlappedComponent :type "PrimitiveComponent Object Reference") (OtherActor :type "Actor Object Reference") (OtherComp :type "PrimitiveComponent Object Reference") (OtherBodyIndex :type Integer))
  ;[1 1 1] End Overlap Event
  (if (`self.ActorHasTag` OtherActor "Player")
    (`SceneComponent.SetVisibility` (`self.Takedown Prompt Widget`) false false)))

(event `/Game/COMMON/Blueprints/Interfaces/BPI_Guard.Run`
  ;[1 1 1] Run Speed
  (set `CharacterMovementComponent.MaxWalkSpeed` 500.0 (`self.CharacterMovement`)))

(event `/Game/COMMON/Blueprints/Interfaces/BPI_Guard.Catch`
  (bind _returnvalue (`self.K2_GetActorLocation`))
  ;[1 1 1] Catch Attack
  (if (not (`self.is attacking`))
    (`|PlayMontage` (`self.Mesh`) "/Game/COMMON/UTILITIES/Animations/Robber/Catch/Catch_Montage.Catch_Montage"
      (:`then`
        (set `self.is attacking` true))
      (:`OnCompleted`
        (set `self.is attacking` false))
      (:`OnNotifyBegin`
        (bind (_outhit _returnvalue_2) (`KismetSystemLibrary.SphereTraceSingleForObjects` _returnvalue (+ _returnvalue (* (`self.GetActorForwardVector`) 135.0)) 30.0 (`|MakeArray` "ObjectTypeQuery3" :!type "EObjectTypeQuery Enum") false (`|MakeArray` self :!type "Actor Object Reference") "ForDuration"))
        (if _returnvalue_2
          (bind (_bblockinghit _binitialoverlap _time _distance _location _impactpoint _normal _impactnormal _physmat _hitactor) (`GameplayStatics.BreakHitResult` _outhit))
          (if (`self.ActorHasTag` _hitactor "Player")
            (bind _ascharacter_1 (cast `/Game/COMMON/ENTITIES/Character1` _hitactor))
            (`GameplayStatics.ApplyDamage` _ascharacter_1 10.0 null self "/Script/Engine.DamageType")))))))

(event `self.ReceiveAnyDamage`
  (params (Damage :type "Float (single-precision)") (DamageType :type "DamageType Object Reference") (InstigatedBy :type "Controller Object Reference") (DamageCauser :type "Actor Object Reference"))
  ;[1 1 1] AnyDamage Event
  (set `self.Health` (- (`self.Health`) Damage))
  (if (<= (`self.Health`) 0.0)
    (`self.K2_DestroyActor`)))

(event `/Game/COMMON/Blueprints/Interfaces/BPITargeting.OnTargeted`
  (params (`bIsTargeted?` :type Boolean))
  ;[1 1 1] Target Lockon Widget
  (`SceneComponent.SetVisibility` (`self.LockonWidget`) `bIsTargeted?` false))

(event `Takedown Ragdoll`
  ;[1 1 1] Take Down Ragdoll
  (`KismetSystemLibrary.Delay` 1.27)
  (`PrimitiveComponent.SetSimulatePhysics` (`self.Mesh`) true)
  (`CharacterMovementComponent.SetMovementMode` (`self.CharacterMovement`) "MOVE_None" 0))

(fn `CanBeTargeted`
  (returns (ReturnValue :type Boolean))
  (return (> (`self.Health`) 0.0)))

(fn `Takedown`
  (returns (`REF Pose` :type "Vector Structure") (Rotation :type "Rotator Structure") (`Can Takedown` :type Boolean) (Actor :type "Actor Object Reference"))
  (if (`self.can takedown`)
    (`self.PlayAnimMontage` "/Game/COMMON/UTILITIES/Animations/Robber/Takedowns/Takedown_Victim_Montage.Takedown_Victim_Montage")
    (`self.Takedown Ragdoll`)
    (`SceneComponent.SetVisibility` (`self.Takedown Prompt Widget`) false false)
    (set `self.dead` true)
    (bind _asbp_ai_guard (cast `/Game/COMMON/AI/AI_Guard/BP_AI_Guard` (`AIBlueprintHelperLibrary.GetAIController` self)))
    (set `/Game/COMMON/AI/AI_Guard/BP_AI_Guard.dead` true _asbp_ai_guard)
    (return (`SceneComponent.K2_GetComponentLocation` (`self.REF`)) (`self.K2_GetActorRotation`) (`self.can takedown`) null)))

(fn `UserConstructionScript`
  (`SkinnedMeshComponent.SetLeaderPoseComponent` (`self.Torso`) (`self.Mesh`) false false)
  (`SkinnedMeshComponent.SetLeaderPoseComponent` (`self.Pants`) (`self.Mesh`) false false)
  (`SkinnedMeshComponent.SetLeaderPoseComponent` (`self.Foot`) (`self.Mesh`) false false)
  (`SkinnedMeshComponent.SetLeaderPoseComponent` (`self.Head`) (`self.Mesh`) false false)
  (`SkinnedMeshComponent.SetLeaderPoseComponent` (`self.Hands`) (`self.Mesh`) false false))
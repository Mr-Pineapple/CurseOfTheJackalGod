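; BP_CollapsingFloor is a trap platform that tilts down after something steps on it, then resets.
; Box begin overlap waits briefly to allow a jump-off, then a timeline pitches the Cube down 90 degrees.
; Box end overlap waits longer, then plays a separate timeline in reverse to raise it.
; Both set absolute world rotation with zero yaw and roll, and overlaps are not filtered by actor.
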(event `self.Box.OnComponentBeginOverlap`
  (params (OverlappedComponent :type "PrimitiveComponent Object Reference") (OtherActor :type "Actor Object Reference") (OtherComp :type "PrimitiveComponent Object Reference") (OtherBodyIndex :type Integer) (bFromSweep :type Boolean) (SweepResult :type "HitResult Structure (by ref)"))
  ;[1 1 1] Gives Player Chance To Jump Off Platform
  (`KismetSystemLibrary.Delay` 0.7)
  ;[1 1 1] Rotates Platform Down 90 Degrees Over Course of 0.75 Seconds
  (bind (_direction _newtrack_0) (`Timeline|FloorDownTimeline` :`NewTime` 1.0 :!via `PlayFromStart`)
    (:`Update`
      (`SceneComponent.K2_SetWorldRotation` (`self.Cube`) (`KismetMathLibrary.MakeRotator` 0.0 (* _newtrack_0 -90.0)) false false))))

(event `self.Box.OnComponentEndOverlap`
  (params (OverlappedComponent :type "PrimitiveComponent Object Reference") (OtherActor :type "Actor Object Reference") (OtherComp :type "PrimitiveComponent Object Reference") (OtherBodyIndex :type Integer))
  ;[1 1 1] Rotates Playform to Original Position After Delay
  (`KismetSystemLibrary.Delay` 2.0)
  (bind (_direction _newtrack_0) (`Timeline|Timeline` :!via `ReverseFromEnd`)
    (:`Update`
      (`SceneComponent.K2_SetWorldRotation` (`self.Cube`) (`KismetMathLibrary.MakeRotator` 0.0 (* _newtrack_0 -90.0)) false false))))

(fn `UserConstructionScript`)
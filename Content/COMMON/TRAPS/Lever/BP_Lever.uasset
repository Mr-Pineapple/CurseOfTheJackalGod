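; BP_Lever is a one-shot lever that opens a linked door for a set time.
; PullLever sets LeverPulled, which is never reset here, plays the down animation and calls OpenDoor on ActorToEffect if it is a BP_Door1.
; After TimeDown, it plays the same animation backwards using a negative play rate from position 1.0, then calls CloseDoor.
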(event `PullLever`
  (bind _lever (`self.Lever`))
  (bind _actortoeffect (`self.ActorToEffect`))
  (if (not (`self.LeverPulled`))
    (set `self.LeverPulled` true)
    ;[1 1 1] Play Lever Down Animation
    (`SkeletalMeshComponent.PlayAnimation` (`self.Lever`) "/Game/COMMON/TRAPS/Lever/LeverAnim/LeverDown.LeverDown" false)
    ;[1 1 1] Open / Close Door
    (`/Engine/EditorBlueprintResources/StandardMacros.IsValid` _actortoeffect
      (:`Is Valid`
        (bind _asbp_door_1 (cast `/Game/COMMON/PUZZLES/BP_Door1` _actortoeffect))
        (`/Game/COMMON/PUZZLES/BP_Door1.OpenDoor` _asbp_door_1)
        (`KismetSystemLibrary.Delay` (`self.timeDown`))
        ;;[0.1719 0.1719 0.1719] Play Reverse Lever Animation
        (`SkeletalMeshComponent.PlayAnimation` _lever "/Game/COMMON/TRAPS/Lever/LeverAnim/LeverDown.LeverDown" false)
        (`SkeletalMeshComponent.SetPlayRate` _lever -1.0)
        (`SkeletalMeshComponent.SetPosition` _lever 1.0 true)
        (`/Engine/EditorBlueprintResources/StandardMacros.IsValid` _asbp_door_1
          (:`Is Valid`
            (`/Game/COMMON/PUZZLES/BP_Door1.CloseDoor` _asbp_door_1)))))))

(fn `UserConstructionScript`)
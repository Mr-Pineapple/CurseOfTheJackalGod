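; Timed floor spike trap that kills player characters who enter its Radius trigger.
; An overlap casts the actor to one of four character classes, stores it, sets SpikesOut and, after a one-second delay, plays the spike animation.
; It then calls Death on every stored character without rechecking overlap, and clears SpikesOut after a further delay.
; Stored references are never cleared, and SpikesOut is never read here.
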(event `self.Radius.OnComponentBeginOverlap`
  (params (OverlappedComponent :type "PrimitiveComponent Object Reference") (OtherActor :type "Actor Object Reference") (OtherComp :type "PrimitiveComponent Object Reference") (OtherBodyIndex :type Integer) (bFromSweep :type Boolean) (SweepResult :type "HitResult Structure (by ref)"))
  (bind _skeletalmesh (`self.SkeletalMesh`))
  (`|ExecutionSequence`
    (:`then_0`
      (bind _ascharacter_1 (cast `/Game/COMMON/ENTITIES/Characters/Character1` OtherActor)))
    (:`then_1`
      (bind _ascharacter_2 (cast `/Game/COMMON/ENTITIES/Characters/Character2` OtherActor)))
    (:`then_2`
      (bind _ascharacter_3 (cast `/Game/COMMON/ENTITIES/Characters/Character3` OtherActor)))
    (:`then_3`
      (bind _ascharacter_4 (cast `/Game/COMMON/ENTITIES/Characters/Character4` OtherActor))))
  (set `self.SpikesOut` true)
  (`/Engine/EditorBlueprintResources/StandardMacros.IsValid` _skeletalmesh
    (:`Is Valid`
      (`KismetSystemLibrary.Delay` 1.0)
      (`SkeletalMeshComponent.PlayAnimation` _skeletalmesh "/Game/COMMON/TRAPS/FloorSpikes/SpikeTrap_HideAnimation_Anim.SpikeTrap_HideAnimation_Anim" false)
      (`|ExecutionSequence`
        (:`then_0`
          (`/Engine/EditorBlueprintResources/StandardMacros.IsValid` _ascharacter_1
            (:`Is Valid`
              (`/Game/COMMON/ENTITIES/Characters/Character1.Death` _ascharacter_1)
              (`KismetSystemLibrary.Delay` 3.0)
              (set `self.SpikesOut` false))))
        (:`then_1`
          (`/Engine/EditorBlueprintResources/StandardMacros.IsValid` _ascharacter_2
            (:`Is Valid`
              (`/Game/COMMON/ENTITIES/Characters/Character2.Death` _ascharacter_2)
              (`KismetSystemLibrary.Delay` 3.0)
              (set `self.SpikesOut` false))))
        (:`then_2`
          (`/Engine/EditorBlueprintResources/StandardMacros.IsValid` _ascharacter_3
            (:`Is Valid`
              (`/Game/COMMON/ENTITIES/Characters/Character3.Death` _ascharacter_3)
              (`KismetSystemLibrary.Delay` 3.0)
              (set `self.SpikesOut` false))))
        (:`then_3`
          (`/Engine/EditorBlueprintResources/StandardMacros.IsValid` _ascharacter_4
            (:`Is Valid`
              (`/Game/COMMON/ENTITIES/Characters/Character4.Death` _ascharacter_4)
              (`KismetSystemLibrary.Delay` 3.0)
              (set `self.SpikesOut` false))))))))

(fn `UserConstructionScript`)
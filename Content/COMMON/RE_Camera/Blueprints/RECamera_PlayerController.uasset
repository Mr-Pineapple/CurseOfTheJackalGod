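; Player controller for a camera-actor system (RE_Camera) that switches the view between Camera_BP actors placed in the level.
; On BeginPlay it selects the camera tagged "Start".
; Interface-driven target changes pass a short retriggerable delay, blend at the new camera's own blend time and notify the player pawn.
; Look input sends yaw and pitch to the current camera and maintains a moving flag, exposed with that camera through an interface getter.
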(event `self.ReceiveBeginPlay`
  ;[1 1 1 0.05 15] Begin Play
  (`self.Set Starting Camera`))

(event `/Game/COMMON/RE_Camera/Blueprints/Interfaces/BPI_PlayerController.BPI_SetTarget`
  (params (NewTarget :type "Actor Object Reference"))
  ;[1 1 1 0.05 15] Interface Event - Checks if the new target is already the Current Camera
  (`KismetSystemLibrary.RetriggerableDelay` 0.05)
  (if (not (== NewTarget (`self.Current Camera`)))
    ;[1 1 1 0.05 15] Gets the new targets blend speed via an interface
    (bind _returnvalue (message `/Game/COMMON/RE_Camera/Blueprints/Interfaces/BPI_Camera.BPI_Get_BlendSpeed` NewTarget))
    ;[1 1 1 0.05 15] Sets the view target to the new camera
    (`self.SetViewTargetWithBlend` NewTarget _returnvalue)
    ;[1 1 1 0.05 15] Calls interface on the Player
    (message `/Game/COMMON/UTILITIES/BPI_Player.BPI_SetTarget` (`GameplayStatics.GetPlayerPawn` 0) NewTarget)
    ;[1 1 1 0.05 15] Sets reference Variable to the new target
    (set `self.Current Camera` NewTarget)))

(event `EnhancedInput|/Game/COMMON/RE_Camera/Input/Actions/IA_Look`
  (params (ActionValue :type "Vector2D Structure") (ElapsedSeconds :type "Float (double-precision)") (TriggeredSeconds :type "Float (double-precision)") (InputAction :type "InputAction Object Reference" :default "/Game/COMMON/RE_Camera/Input/Actions/IA_Look.IA_Look"))
  (bind (_x _y) (`KismetMathLibrary.BreakVector2D` ActionValue))
  ;[1 1 1 0.05 15] Look Input - Sets the Moving Camera Variable on Triggered & Completed. Interface Events are called on the current camera on triggered.
  (:`Triggered`
    (set `self.Moveing Camera?` true)
    (message `/Game/COMMON/RE_Camera/Blueprints/Interfaces/BPI_Camera.BPI_AddYaw` (`self.Current Camera`) _x)
    (message `/Game/COMMON/RE_Camera/Blueprints/Interfaces/BPI_Camera.BPI_AddPitch` (`self.Current Camera`) _y))
  (:`Completed`
    (`KismetSystemLibrary.RetriggerableDelay` 0.025)
    (set `self.Moveing Camera?` false)))

(fn `BPI_Get_Essential_CameraValues`
  (returns (CurrentCamera :type "Actor Object Reference") (`MoveingCamera?` :type Boolean))
  (return (`self.Current Camera`) (`self.Moveing Camera?`)))

(fn `Set Starting Camera`
  (locals (Current :type "/Game/COMMON/RE_Camera/Blueprints/Camera_BP Object Reference"))
  ;[1 1 1 0.05 15] Gets every Camera actor in the scene
  (bind _outactors (`GameplayStatics.GetAllActorsOfClass` "/Game/COMMON/RE_Camera/Blueprints/Camera_BP.Camera_BP_C"))
  ;[1 1 1 0.05 15] This goes through all the actors the previous node returned
  (for _array_element _outactors
    (set `local.Current` _array_element)
    ;[1 1 1 0.05 15] Checks Current Actor for the Start Tag ( Indicates the Camera the level starts with )
    (if (`self.ActorHasTag` (`local.Current`) "Start")
      ;[1 1 1 0.05 15] Breaks the For Each Loop ( so that it longer goes through the actors ) then sets the player controllers view target to the actor found
      (`|ExecutionSequence`
        (:`then_0`
          (break))
        (:`then_1`
          (`self.SetViewTargetWithBlend` (`local.Current`))
          ;[1 1 1 0.05 15] Calls interface event on the player
          (message `/Game/COMMON/UTILITIES/BPI_Player.BPI_SetTarget` (`GameplayStatics.GetPlayerPawn` 0) (`local.Current`))
          ;[1 1 1 0.05 15] Sets Variable for referencing later
          (set `self.Current Camera` (`local.Current`)))))))

(fn `UserConstructionScript`)
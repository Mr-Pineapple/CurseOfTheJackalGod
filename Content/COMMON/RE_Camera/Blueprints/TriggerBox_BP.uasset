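; Camera trigger box that points a player's controller at its assigned CameraTarget while that player is inside the volume.
; When a Player-tagged actor enters, it stores the actor and starts a looping timer that repeatedly sends CameraTarget through a Blueprint interface message.
; The message goes to player controller 0 if it instigates the stored actor, otherwise to controller 1.
; Any end overlap clears the timer while the stored player is valid.
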(event `self.Box.OnComponentBeginOverlap`
  (params (OverlappedComponent :type "PrimitiveComponent Object Reference") (OtherActor :type "Actor Object Reference") (OtherComp :type "PrimitiveComponent Object Reference") (OtherBodyIndex :type Integer) (bFromSweep :type Boolean) (SweepResult :type "HitResult Structure (by ref)"))
  ;[1 1 1 0.05 15] Checks if the Other Actor is the Player then Sets the Target to the desired Camera Target
  (if (`self.ActorHasTag` OtherActor "Player")
    (set `self.Player` OtherActor)
    (bind _returnvalue (`KismetSystemLibrary.K2_SetTimerDelegate` (delegate `Set Target`) 0.25 true))
    (set `self.New Target Timer` _returnvalue)))

(event `Set Target`
  (bind _returnvalue (`GameplayStatics.GetPlayerController` 0))
  ;[1 1 1 0.05 15] Checks if the Other Actor is the Player then Sets the Target to the desired Camera Target
  (if (== (`self.GetInstigatorController` (`self.Player`)) _returnvalue)
    (message `/Game/COMMON/RE_Camera/Blueprints/Interfaces/BPI_PlayerController.BPI_SetTarget` _returnvalue (`self.Camera Target`))
    (else
      (message `/Game/COMMON/RE_Camera/Blueprints/Interfaces/BPI_PlayerController.BPI_SetTarget` (`GameplayStatics.GetPlayerController` 1) (`self.Camera Target`)))))

(event `self.Box.OnComponentEndOverlap`
  (params (OverlappedComponent :type "PrimitiveComponent Object Reference") (OtherActor :type "Actor Object Reference") (OtherComp :type "PrimitiveComponent Object Reference") (OtherBodyIndex :type Integer))
  ;[1 1 1 0.05 15] Checks if the Other Actor is the Player then Sets the Target to the desired Camera Target
  (`self.Player`
    (:`then`
      (`KismetSystemLibrary.K2_ClearAndInvalidateTimerHandle` (`self.New Target Timer`)))
    (:`else`)))

(fn `UserConstructionScript`)
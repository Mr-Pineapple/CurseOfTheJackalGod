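; Puzzle trigger actor that shifts its static mesh vertically when a playable character class overlaps its box.
; A DoOnce limits it to the first overlap, then a cast chain checks for Character1 through Character4 to play the VerticalTranslation timeline.
; The timeline's Height is added to the mesh's relative Z on Finished, not per update, so the mesh moves in one step, with a debug print.
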(event `self.ReceiveBeginPlay`)

(event `self.Box.OnComponentBeginOverlap`
  (params (OverlappedComponent :type "PrimitiveComponent Object Reference") (OtherActor :type "Actor Object Reference") (OtherComp :type "PrimitiveComponent Object Reference") (OtherBodyIndex :type Integer) (bFromSweep :type Boolean) (SweepResult :type "HitResult Structure (by ref)"))
  (bind _staticmesh (`self.StaticMesh`))
  (bind (_relativelocation_x _relativelocation_y _relativelocation_z) (`KismetMathLibrary.BreakVector` (`SceneComponent.RelativeLocation` _staticmesh)))
  (`/Engine/EditorBlueprintResources/StandardMacros.DoOnce` false
    (:`Completed`
      (cast `/Game/COMMON/ENTITIES/Characters/Character1` OtherActor
        (:`then`
          (bind (_direction _height) (`Timeline|VerticalTranslation` :!via `PlayFromStart` :!label _label)
            (:`Finished`
              (bind _returnvalue (+ _relativelocation_z _height))
              (`SceneComponent.K2_SetRelativeLocation` _staticmesh (`KismetMathLibrary.MakeVector` _relativelocation_x _relativelocation_y _returnvalue) false false)
              (`KismetSystemLibrary.PrintString` (`KismetStringLibrary.Conv_DoubleToString` _returnvalue)))))
        (:`CastFailed`
          (cast `/Game/COMMON/ENTITIES/Characters/Character2` OtherActor
            (:`then`
              (goto _label :!via `PlayFromStart`))
            (:`CastFailed`
              (cast `/Game/COMMON/ENTITIES/Characters/Character3` OtherActor
                (:`then`
                  (goto _label :!via `PlayFromStart`))
                (:`CastFailed`
                  (cast `/Game/COMMON/ENTITIES/Characters/Character4` OtherActor)
                  (goto _label :!via `PlayFromStart`))))))))))

(fn `UserConstructionScript`)
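; BP_Door1 is a puzzle door that opens and closes by moving its mesh along relative Z.
; OpenDoor stores the current Z, then a timeline lerps toward the current height plus DOORHEIGHT.
; CloseDoor restarts a second timeline that lerps back to the stored Z.
; Both lerps read the live mesh position each update, so movement compounds instead of interpolating between fixed endpoints.
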(event `OpenDoor`
  (bind (_relativelocation_x _relativelocation_y _relativelocation_z) (`KismetMathLibrary.BreakVector` (`SceneComponent.RelativeLocation` (`self.DoorMesh`))))
  ;[1 1 1] Used for opening the door -
  (set `self.originalDoorLocation` _relativelocation_z)
  (bind (_direction _newtrack_0) (`Timeline|Timeline`)
    (:`Update`
      (`SceneComponent.K2_SetRelativeLocation` (`self.DoorMesh`) (`KismetMathLibrary.MakeVector` 0.0 0.0 (`KismetMathLibrary.Lerp` _relativelocation_z (+ (`self.DOOR_HEIGHT`) _relativelocation_z) _newtrack_0)) false false))))

(event `CloseDoor`
  (bind (_relativelocation_x _relativelocation_y _relativelocation_z) (`KismetMathLibrary.BreakVector` (`SceneComponent.RelativeLocation` (`self.DoorMesh`))))
  (bind (_direction _newtrack_0) (`Timeline|Timeline_0` :!via `PlayFromStart`)
    (:`Update`
      (`SceneComponent.K2_SetRelativeLocation` (`self.DoorMesh`) (`KismetMathLibrary.MakeVector` 0.0 0.0 (`KismetMathLibrary.Lerp` _relativelocation_z (`self.originalDoorLocation`) _newtrack_0)) false false))))

(fn `UserConstructionScript`)
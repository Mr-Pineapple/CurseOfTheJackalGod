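; SmokeBomb_BP is a smoke bomb pickup utility actor that disables nearby enemies' movement as soon as it spawns.
; On BeginPlay it spawns a Niagara explosion at its own location, then sphere-overlaps around the Character3 actor rather than around itself.
; A cast chain calls DisableEnemyMovementOverTime on each guard, AI demo character or boss found, with leftover debug prints on the guard branch.
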(event `self.ReceiveBeginPlay`
  (`NiagaraFunctionLibrary.SpawnSystemAtLocation` "/Game/CLIENT/UTILITIES/Particles/PoisonSeed_Explosion_NS.PoisonSeed_Explosion_NS" (`self.K2_GetActorLocation`))
  (bind _returnvalue (`GameplayStatics.GetActorOfClass` "/Game/COMMON/ENTITIES/Characters/Character3.Character3_C"))
  (`/Engine/EditorBlueprintResources/StandardMacros.IsValid` _returnvalue
    (:`Is Valid`
      (bind _outactors (`KismetSystemLibrary.SphereOverlapActors` (`self.K2_GetActorLocation` _returnvalue) 1000.0 (`self.Object Type`) null (`|MakeArray` self :!type "Actor Object Reference")))
      (for _array_element _outactors
        (bind _asbp_guard (cast `/Game/COMMON/ENTITIES/AI/AI_Guard/BP_Guard` _array_element)
          (:`then`
            (`/Engine/EditorBlueprintResources/StandardMacros.IsValid` _asbp_guard
              (:`Is Valid`
                (`/Game/COMMON/ENTITIES/AI/AI_Guard/BP_Guard.Disable Enemy Movement Over Time` _asbp_guard)
                (`KismetSystemLibrary.PrintString` "guard"))
              (:`Is Not Valid`
                (`KismetSystemLibrary.PrintString` "fail"))))
          (:`CastFailed`
            (bind _asbp_ai_demo_character (cast `/Game/COMMON/COMPONENTS/AI_Component/Demo/DemoAi/BP_AI_DemoCharacter` _array_element)
              (:`then`
                (`/Engine/EditorBlueprintResources/StandardMacros.IsValid` _asbp_ai_demo_character
                  (:`Is Valid`
                    (`/Game/COMMON/COMPONENTS/AI_Component/Demo/DemoAi/BP_AI_DemoCharacter.Disable Enemy Movement Over Time` _asbp_ai_demo_character))))
              (:`CastFailed`
                (bind _asbp_enemy_boss (cast `/Game/COMMON/ENTITIES/AI/Enemies/BossEnemy/BP_Enemy_Boss` _array_element))
                (`/Engine/EditorBlueprintResources/StandardMacros.IsValid` _asbp_enemy_boss
                  (:`Is Valid`
                    (`/Game/COMMON/ENTITIES/AI/Enemies/BossEnemy/BP_Enemy_Boss.Disable Enemy Movement Over Time` _asbp_enemy_boss)))))))))))

(fn `UserConstructionScript`)
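; Rock actor in the pickups utilities that damages specific enemy characters when its collision component hits them.
; On hit, a chain of casts checks for a guard, AI demo character or boss, then applies the same fixed damage and destroys the rock.
; Hits on any other actor have no effect, and the construction script only calls the parent version.
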(event `self.Collision.OnComponentHit`
  (params (HitComponent :type "PrimitiveComponent Object Reference") (OtherActor :type "Actor Object Reference") (OtherComp :type "PrimitiveComponent Object Reference") (NormalImpulse :type "Vector Structure") (Hit :type "HitResult Structure (by ref)"))
  (bind _asbp_guard (cast `/Game/COMMON/ENTITIES/AI/AI_Guard/BP_Guard` OtherActor)
    (:`then`
      (`GameplayStatics.ApplyDamage` _asbp_guard 100.0 null self)
      (`self.K2_DestroyActor`))
    (:`CastFailed`
      (bind _asbp_ai_demo_character (cast `/Game/AI_Component/Demo/DemoAi/BP_AI_DemoCharacter` OtherActor)
        (:`then`
          (`GameplayStatics.ApplyDamage` _asbp_ai_demo_character 100.0 null self)
          (`self.K2_DestroyActor`))
        (:`CastFailed`
          (bind _asbp_enemy_boss (cast `/Game/Enemies/BossEnemy/BP_Enemy_Boss` OtherActor))
          (`GameplayStatics.ApplyDamage` _asbp_enemy_boss 100.0 null self)
          (`self.K2_DestroyActor`))))))

(fn `UserConstructionScript`
  (`parent.UserConstructionScript`))
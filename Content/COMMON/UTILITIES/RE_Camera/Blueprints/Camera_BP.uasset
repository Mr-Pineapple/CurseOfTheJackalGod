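; Fixed-position camera actor for a Resident Evil-style camera system, optionally tagged "Start" to mark the first camera.
; On Tick, while the player controller reports it as current, it eases its rotation toward the player, follows yaw/pitch input, or optionally resets when idle.
; Look-at and input rotations are clamped to MinRot and MaxRot.
; Interface functions receive input and expose blend speed and movement directions.
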(event `self.ReceiveBeginPlay`
  ;[1 1 1 1 20] ACTOR MUST HAVE START TAG TO BE CONSIDERED THE FIRST CAMERA
  (if (`self.Start Camera?`)
    (`KismetArrayLibrary.Array_Add` (`self.Tags`) "Start")))

(event `/Game/COMMON/UTILITIES/RE_Camera/Blueprints/Interfaces/BPI_Camera.BPI_AddYaw`
  (params (Value :type "Float (double-precision)"))
  ;[1 1 1 0.05 15] Interface Input Values
  (set `self.Yaw Value` Value))

(event `self.ReceiveTick`
  (params (DeltaSeconds :type "Float (single-precision)"))
  ;[1 1 1 0.05 15] Check if the Current Camera is this camera
  (`|ExecutionSequence`
    (:`then_0`
      (bind _currentcamera (message `/Game/COMMON/UTILITIES/RE_Camera/Blueprints/Interfaces/BPI_PlayerController.BPI_Get_Essential_CameraValues` (`GameplayStatics.GetPlayerController` 0)))
      (if (== _currentcamera self)
        (if (`self.Draw Debug on Screen?`)
          _
          (else
            _))
        ;[1 1 1 0.05 15] Checks if Auto Look at Player is enabled, picking rotation mode
        (if (`self.Auto Look At Player?`)
          ;[1 1 1 0.05 15] Auto Look at Player Rotation
          (`SceneComponent.K2_SetRelativeRotation` (`self.Camera`) (`KismetMathLibrary.RInterpTo` (`SceneComponent.RelativeRotation` (`self.Camera`)) (`self.Calculate Auto Look Based Rotation`) (`GameplayStatics.GetWorldDeltaSeconds`) 5.0) false false)
          (else
            ;[1 1 1 0.05 15] Gets reference to player controller; checking if using input
            (bind (_currentcamera_2 _movingcamera_) (message `/Game/COMMON/UTILITIES/RE_Camera/Blueprints/Interfaces/BPI_PlayerController.BPI_Get_Essential_CameraValues` (`GameplayStatics.GetPlayerController` 0)))
            (if _movingcamera_
              ;[1 1 1 0.05 15] Camera Input Rotation
              (`SceneComponent.K2_SetRelativeRotation` (`self.Camera`) (`KismetMathLibrary.RInterpTo` (`SceneComponent.RelativeRotation` (`self.Camera`)) (`self.Calculate Input Based Rotation`) (`GameplayStatics.GetWorldDeltaSeconds`) 15.0) false false)
              (else
                ;[1 1 1 0.05 15] Checks if using Auto Rotation Reset
                (if (`self.Auto Reset Camera Position?`)
                  ;[1 1 1 0.05 15] Reset Rotation
                  (`SceneComponent.K2_SetRelativeRotation` (`self.Camera`) (`KismetMathLibrary.RInterpTo` (`SceneComponent.RelativeRotation` (`self.Camera`)) (struct) (`GameplayStatics.GetWorldDeltaSeconds`) 1.0) false false))))))))))

(event `/Game/COMMON/UTILITIES/RE_Camera/Blueprints/Interfaces/BPI_Camera.BPI_AddPitch`
  (params (Value :type "Float (double-precision)"))
  ;[1 1 1 0.05 15] Interface Input Values
  (set `self.Pitch Value` Value))

(fn `BPI_Get_BlendSpeed`
  (returns (ReturnValue :type "Float (double-precision)"))
  (return (`self.Blend Speed`)))

(fn `BPI_Get_Movement_Directions`
  (returns (`Forward Direciton` :type "ArrowComponent Object Reference") (`Left/Right Direction` :type "ArrowComponent Object Reference"))
  (return (`self.Front Direction`) (`self.Left / Right Direction`)))

(fn `Calculate Auto Look Based Rotation`
  (returns (ReturnValue :type "Rotator Structure"))
  (bind (_x _y) (`KismetMathLibrary.BreakVector2D` (`self.Max_Rot`)))
  (bind (_x_2 _y_2) (`KismetMathLibrary.BreakVector2D` (`self.Min_Rot`)))
  (return (`KismetMathLibrary.MakeRotator` (.roll (`SceneComponent.RelativeRotation` (`self.Camera`))) (`KismetMathLibrary.FClamp` (.pitch (`KismetMathLibrary.FindLookAtRotation` (`self.K2_GetActorLocation`) (`self.K2_GetActorLocation` (`GameplayStatics.GetPlayerPawn` 0)))) _x_2 _x) (`KismetMathLibrary.FClamp` (.yaw (`KismetMathLibrary.FindLookAtRotation` (`self.K2_GetActorLocation`) (`self.K2_GetActorLocation` (`GameplayStatics.GetPlayerPawn` 0)))) _y_2 _y))))

(fn `Calculate Input Based Rotation`
  (returns (ReturnValue :type "Rotator Structure"))
  (bind (_x _y) (`KismetMathLibrary.BreakVector2D` (`self.Max_Rot`)))
  (bind (_x_2 _y_2) (`KismetMathLibrary.BreakVector2D` (`self.Min_Rot`)))
  (return (`KismetMathLibrary.MakeRotator` (.roll (`SceneComponent.RelativeRotation` (`self.Camera`))) (`KismetMathLibrary.FClamp` (+ (.pitch (`SceneComponent.RelativeRotation` (`self.Camera`))) (* (/ (`self.Pitch Value`) 4.0) -1.0)) _x_2 _x) (`KismetMathLibrary.FClamp` (+ (.yaw (`SceneComponent.RelativeRotation` (`self.Camera`))) (* (/ (`self.Yaw Value`) 4.0) 1.0)) _y_2 _y))))

(fn `UserConstructionScript`)
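; BP_CameraTrack2 is a rail camera that follows an owner character along a spline and looks at it, ticking only while an owner is valid.
; The character's spine position on the Path spline, minus a lag distance, gives a time that samples the separate CameraTrack spline.
; Camera location and rotation interpolate toward that target, snapping when the owner is set.
; The lag distance eases larger when the character moves fast against the path direction.
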(event `self.ReceiveTick`
  (params (DeltaSeconds :type "Float (single-precision)"))
  (bind _camowner2 (`self.CamOwner2`)
    (:`then`
      (`self.UpdateCamera2` (`SceneComponent.GetSocketLocation` (`Character.Mesh` _camowner2) "spine_04"))
      (`self.InterpLocation`)
      (`self.InterpRotation`)
      (`self.UpdateMovementLagOffset`))
    (:`else`)))

(fn `GetTimeAlongSplineAtNearbyLocation2`
  (params (WorldLocation :type "Vector Structure") (DistanceLag :type "Float (double-precision)"))
  (returns (ReturnValue :type "Float (single-precision)"))
  (bind _returnvalue (`SplineComponent.FindInputKeyClosestToWorldLocation` (`self.Path`) (`local.WorldLocation`)))
  (bind _returnvalue_2 (`self.GetVelocity` (`self.CamOwner2`)))
  (set `self.Lag Direction` (`KismetMathLibrary.SelectInt` (`KismetMathLibrary.SelectInt` 1 2 (== (`KismetMathLibrary.Conv_RotatorToVector` (`SplineComponent.GetRotationAtSplineInputKey` (`self.Path`) _returnvalue "World")) (`KismetMathLibrary.Normal` _returnvalue_2) :`ErrorTolerance` 1.0)) 0 (> (`KismetMathLibrary.VSize` (`KismetMathLibrary.MakeVector` (.x _returnvalue_2) (.y _returnvalue_2))) 300.0)))
  (return (`SplineComponent.GetTimeAtDistanceAlongSpline` (`self.Path`) (- (`SplineComponent.GetDistanceAlongSplineAtSplineInputKey` (`self.Path`) _returnvalue) (`local.DistanceLag`)))))

(fn `InterpLocation`
  (if (not (== (`self.DesiredLocation`) (`SceneComponent.K2_GetComponentLocation` (`self.Camera`)) :`ErrorTolerance` 1.0))
    (`SceneComponent.K2_SetWorldLocation` (`self.Camera`) (`KismetMathLibrary.VInterpTo` (`SceneComponent.K2_GetComponentLocation` (`self.Camera`)) (`self.DesiredLocation`) (`GameplayStatics.GetWorldDeltaSeconds`) (`self.MovementLagSpeed`)) false false)))

(fn `InterpRotation`
  (bind _returnvalue (`SceneComponent.K2_GetComponentRotation` (`self.Camera`)))
  (if (not (== (`self.DesiredRotation`) _returnvalue :`ErrorTolerance` 0.01))
    (`SceneComponent.K2_SetWorldRotation` (`self.Camera`) (`KismetMathLibrary.RInterpTo` _returnvalue (`self.DesiredRotation`) (`GameplayStatics.GetWorldDeltaSeconds`) (`self.RotationLagSpeed`)) false false)))

(fn `SetCamOwner`
  (params (Character :type "/Game/COMMON/ENTITIES/Characters/Character2 Object Reference"))
  (bind _output_get (set `self.CamOwner2` Character))
  (`/Engine/EditorBlueprintResources/StandardMacros.IsValid` _output_get
    (:`Is Valid`
      (`self.SetActorTickEnabled` true)
      (`self.UpdateCamera2` (`SceneComponent.GetSocketLocation` (`Character.Mesh` (`self.CamOwner2`)) "spine_04"))
      (`SceneComponent.K2_SetWorldLocationAndRotation` (`self.Camera`) (`self.DesiredLocation`) (`self.DesiredRotation`) false true))
    (:`Is Not Valid`
      (`self.SetActorTickEnabled` false))))

(fn `SetCamOwner2`
  (params (Character :type "/Game/COMMON/ENTITIES/Characters/Character2 Object Reference"))
  (bind _output_get (set `self.CamOwner2` Character))
  (`/Engine/EditorBlueprintResources/StandardMacros.IsValid` _output_get
    (:`Is Valid`
      (`self.SetActorTickEnabled` true)
      (`self.UpdateCamera2` (`SceneComponent.GetSocketLocation` (`Character.Mesh` (`self.CamOwner2`)) "spine_04"))
      (`SceneComponent.K2_SetWorldLocationAndRotation` (`self.Camera`) (`self.DesiredLocation`) (`self.DesiredRotation`) false true))
    (:`Is Not Valid`
      (`self.SetActorTickEnabled` false))))

(fn `UpdateCamera2`
  (params (WorldRotation :type "Vector Structure"))
  (set `self.DesiredLocation` (`SplineComponent.GetLocationAtTime` (`self.CameraTrack`) (`self.GetTimeAlongSplineAtNearbyLocation2` WorldRotation (`self.MovementLagOffset`)) "World" false))
  (set `self.DesiredRotation` (`KismetMathLibrary.FindLookAtRotation` (`SceneComponent.K2_GetComponentLocation` (`self.Camera`)) (`self.K2_GetActorLocation` (`self.CamOwner2`)))))

(fn `UpdateMovementLagOffset`
  (bind _maxmovementlagoffset (`self.MaxMovementLagOffset`))
  (set `self.MovementLagOffset` (`KismetMathLibrary.FInterpTo` (`self.MovementLagOffset`) (select `int` (`self.Lag Direction`) :`0` _maxmovementlagoffset :`1` _maxmovementlagoffset :`2` (* _maxmovementlagoffset 1.5)) (`GameplayStatics.GetWorldDeltaSeconds`) (`self.MovementLagOffsetSpeed`))))

(fn `UserConstructionScript`)
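; Master projectile Blueprint for weapons, acting as either a bullet or an explosive based on the IsExplosive flag.
; On BeginPlay its collision ignores the instigator and weapon while moving.
; Bullets apply point-of-contact damage and impact effects on Hit, while explosives apply radial damage and explosion effects when ProjectileMovement stops.
; Both paths credit the instigator's controller, hide the actor, then destroy it after a short delay.
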(event `self.ReceiveBeginPlay`
  (bind _projectilecollision (`self.ProjectileCollision`))
  ;[1 1 1] Event Begin Play Set Projectile To Ignore Instigator
  (`PrimitiveComponent.IgnoreActorWhenMoving` _projectilecollision (`self.GetInstigator`) true)
  (`PrimitiveComponent.IgnoreActorWhenMoving` _projectilecollision null true)
  (`PrimitiveComponent.IgnoreActorWhenMoving` _projectilecollision (`self.WeaponRef`) true)
  (`PrimitiveComponent.IgnoreActorWhenMoving` _projectilecollision null true))

(event `self.ReceiveHit`
  (params (MyComp :type "PrimitiveComponent Object Reference") (Other :type "Actor Object Reference") (OtherComp :type "PrimitiveComponent Object Reference") (bSelfMoved :type Boolean) (HitLocation :type "Vector Structure") (HitNormal :type "Vector Structure") (NormalImpulse :type "Vector Structure") (Hit :type "HitResult Structure (by ref)"))
  ;[1 1 1] Event Hit
  (if (not (`self.IsExplosive?`))
    (`GameplayStatics.ApplyDamage` (`.HitActor` (`GameplayStatics.BreakHitResult` Hit)) (`KismetMathLibrary.Conv_IntToDouble` (`self.Damage`)) (`self.GetInstigatorController`) self)
    (`self.SetActorHiddenInGame` true)
    (`self.BulletImpactFX` Hit)
    (`KismetSystemLibrary.Delay` 0.2)
    (`self.K2_DestroyActor`)))

(event `self.ProjectileMovement.OnProjectileStop`
  (params (ImpactResult :type "HitResult Structure (by ref)"))
  ;[1 1 1] On Projectile Stop
  (if (`self.IsExplosive?`)
    (`self.OnStop` ImpactResult)))

(event `OnStop`
  (params (HitResult :type "HitResult Structure"))
  ;[1 1 1] On Projectile Stop
  (`GameplayStatics.ApplyRadialDamage` :`BaseDamage` (`KismetMathLibrary.Conv_IntToDouble` (`self.Damage`)) :`Origin` (`self.K2_GetActorLocation`) :`DamageRadius` (`self.Damage Radius`) :`DamageCauser` self :`InstigatedByController` (`self.GetInstigatorController`))
  (`self.SetActorHiddenInGame` true)
  (`self.ExplosionFX` HitResult)
  (`KismetSystemLibrary.Delay` 0.2)
  (`self.K2_DestroyActor`))

(event `BulletImpactFX`
  (params (HitResults :type "HitResult Structure"))
  (bind (_bblockinghit _binitialoverlap _time _distance _location _impactpoint _normal _impactnormal) (`GameplayStatics.BreakHitResult` HitResults))
  ;[1 1 1] Bullet FX
  (`GameplayStatics.PlaySoundAtLocation` (`self.BulletImpactSound`) _impactpoint (struct) 1.0 1.0 0.0 null null null null)
  (`GameplayStatics.SpawnEmitterAtLocation` (`self.BulletImpactParticle`) _impactpoint (`KismetMathLibrary.MakeRotFromZ` _impactnormal)))

(event `ExplosionFX`
  (params (HitResult :type "HitResult Structure"))
  (bind _returnvalue (`self.K2_GetActorLocation`))
  ;[1 1 1] Explosive FX
  (`GameplayStatics.PlaySoundAtLocation` (`self.ExplosionSound`) _returnvalue (struct) 1.0 1.0 0.0 null null null null)
  (`GameplayStatics.SpawnEmitterAtLocation` (`self.ExplosionParticle`) _returnvalue (`self.K2_GetActorRotation`)))

(fn `UserConstructionScript`)
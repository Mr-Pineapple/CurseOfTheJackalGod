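; Base weapon Blueprint handling firing, ammo, reload and effects for single, auto and multi-round weapons.
; Each shot sphere-traces with spread from the character's aim point, then re-traces from the muzzle toward that result, applying hitscan damage or spawning a projectile.
; Shots report noise and damage to AI perception, then feed per-mode effects, using gates and DoOnce macros for looping or one-off FX.
; Reloading refills the clip from reserve ammo, which enemy weapons generally don't deplete.
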(event `self.ReceiveBeginPlay`
  ;[1 1 1] Event Begin Play
  (set `self.CurrentMaxAmmo` (`self.MaxAmmo`))
  (set `self.CurrentAmmoInClip` (`self.MaxAmmoClipSize`)))

(event `SetOwnerAndInstigator`
  (bind _characterref (`self.CharacterRef`))
  (bind _characterref_2 (`self.CharacterRef`))
  (bind _handsocketname (`self.HandSocketName`))
  ;[1 1 1] Set Owner and Instigator Of Weapon
  (`self.SetOwner` self _characterref_2)
  (set `self.Instigator` _characterref_2)
  (switch `/Game/COMMON/WeaponBlueprints/Weapons/E_WeaponTypes` (`self.WeaponType`)
    (:`NewEnumerator0`
      (bind _output_get (set `self.CurrentSocketName` (`/Game/COMMON/WeaponBlueprints/Weapons/BP_Weapon_Master.CurrentSocketName` (`/Game/COMMON/ENTITIES/Character1.PrimaryWeaponRef` _characterref))))
      (bind _output_get_2 (set `/Game/COMMON/ENTITIES/Character1.PrimaryWeaponRef` self _characterref))
      (if (== _output_get _handsocketname)
        (set `/Game/COMMON/ENTITIES/Character1.CurrentWeaponRef` _output_get_2 _characterref)))
    (:`NewEnumerator1`
      (bind _output_get_3 (set `self.CurrentSocketName` (`/Game/COMMON/WeaponBlueprints/Weapons/BP_Weapon_Master.CurrentSocketName` (`/Game/COMMON/ENTITIES/Character1.SecondaryWeaponRef` _characterref))))
      (bind _output_get_4 (set `/Game/COMMON/ENTITIES/Character1.SecondaryWeaponRef` self _characterref))
      (if (== _output_get_3 _handsocketname)
        (set `/Game/COMMON/ENTITIES/Character1.CurrentWeaponRef` _output_get_4 _characterref)))))

(event `StartWeaponFire`
  ;[1 1 1] Weapon Firing / Reload
  ;;[1 1 1] On/Off Weapon Fire/Diverts Logic If Weapon Is For Enemy AI
  (switch `/Game/COMMON/WeaponBlueprints/Weapons/E_FiringModes` (`self.FiringMode`)
    (:`NewEnumerator0`
      _)
    (:`NewEnumerator1`
      (`self.AutoFire` :!label _label
        (:`Out`
          _)))
    (:`NewEnumerator2`
      (`self.MultiFire`
        (:`Out`
          _))))
  (bind (_outhit _returnvalue _muzzlesocketlocation) (`self.Weapon Sphere Trace`))
  (`self.ShootingInfo` _outhit _returnvalue _muzzlesocketlocation))

(event `StopWeaponFire`
  ;[1 1 1] Weapon Firing / Reload
  ;;[1 1 1] On/Off Weapon Fire/Diverts Logic If Weapon Is For Enemy AI
  (`|ExecutionSequence`
    (:`then_0`
      (goto _label :!via `CloseGate`))
    (:`then_1`
      (`self.OfWeaponFire`))))

(event `OnReload`
  ;[1 1 1] Weapon Firing / Reload
  ;;[1 1 1] On Weapon Reload
  (`self.ReloadSound`)
  (`KismetSystemLibrary.Delay` (`self.ReloadDelay`))
  (`self.ReloadAddAmmo`))

(event `ReloadSound`
  ;[1 1 1] Weapon Firing / Reload
  ;;[1 1 1] On Weapon Reload
  (`GameplayStatics.SpawnSoundAttached` (`self.ReloadWeaponSound`) (`self.SK_Weapon`) (`self.MuzzleSocketName`) (0.0 0.0 0.0) (struct) "KeepRelativeOffset" false 1.0 1.0 0.0 null null))

(event `ShootingInfo`
  (params (HitResult :type "HitResult Structure") (Hit :type Boolean) (MuzzleSocketLocation :type "Vector Structure"))
  ;[1 1 1] Weapon Firing / Reload
  ;;[1 1 1] Shoot Info
  (bind (_hitresultout _hitout) (`self.ShootInfo` HitResult Hit MuzzleSocketLocation))
  (switch `/Game/COMMON/WeaponBlueprints/Weapons/E_FiringModes` (`self.FiringMode`)
    (:`NewEnumerator0`
      (`self.SingleFireWeaponFX` _hitresultout _hitout))
    (:`NewEnumerator1`
      (`self.AutoFireWeaponFX` _hitresultout _hitout))
    (:`NewEnumerator2`
      (`self.MultiFireweaponFX` _hitresultout _hitout)
      (`/Engine/EditorBlueprintResources/StandardMacros.DoOnce` false :!label _label_2
        (:`Completed`
          _))))
  (`KismetSystemLibrary.Delay` 0.1)
  (`self.DecrementAmmo`)
  (if (<= (`self.CurrentAmmoInClip`) 0)
    (if (`PlayerController.IsInputKeyDown` (`GameplayStatics.GetPlayerController` 0) "LeftMouseButton")
      (`self.StopWeaponFire`))))

(event `OfWeaponFire`
  ;[1 1 1] Weapon Firing / Reload
  ;;[1 1 1] Off Weapon Fire
  (`|ExecutionSequence`
    (:`then_0`
      (goto _label_2 :!via `Reset`))
    (:`then_1`
      (`KismetSystemLibrary.Delay` (`self.SingleFireCooldown`))
      (set `self.IsWeaponCooldownActive?` false))
    (:`then_2`
      (`self.OffWeaponFire`))))

(event `SingleFireWeaponFX`
  (params (HitResult :type "HitResult Structure") (Hit :type Boolean))
  ;[1 1 1] Weapon Firing / Reload
  ;;[1 1 1] Weapon FX Based On Firing Mode Type
  (`self.SingleFireFX` HitResult Hit))

(event `AutoFireWeaponFX`
  (params (HitResult :type "HitResult Structure") (Hit :type Boolean))
  ;[1 1 1] Weapon Firing / Reload
  ;;[1 1 1] Weapon FX Based On Firing Mode Type
  (`self.AutoFireFX` HitResult Hit)
  (`|ExecutionSequence`
    (:`then_0`
      (`self.AutoFireSpawnFX` :!label _label_3))
    (:`then_1`
      (`self.AutoFireSoundControl` :!label _label_4))))

(event `OffWeaponFire`
  ;[1 1 1] Weapon Firing / Reload
  ;;[1 1 1] Weapon FX Based On Firing Mode Type
  (`|ExecutionSequence`
    (:`then_0`
      (goto _label_3 :!via `ResetDoOnce`))
    (:`then_1`
      (goto _label_4 :!via `ResetDoOnce`))
    (:`then_2`
      (goto _label_4 :!via `FadeOut`))
    (:`then_3`
      (`self.DestroyAutoFireFX`))
    (:`then_4`
      (goto _label_5 :!via `ResetDoOnce`))))

(event `MultiFireweaponFX`
  (params (HitResult :type "HitResult Structure") (Hit :type Boolean))
  ;[1 1 1] Weapon Firing / Reload
  ;;[1 1 1] Weapon FX Based On Firing Mode Type
  (`|ExecutionSequence`
    (:`then_0`
      (`self.MultiFireFX` HitResult Hit))
    (:`then_1`
      (`self.MultiFireFXControl` :!label _label_5))))

(fn `AutoFireFX`
  (params (HitResultIn :type "HitResult Structure (by ref)") (HitIn :type Boolean))
  (bind (_bblockinghit _binitialoverlap _time _distance _location _impactpoint _normal _impactnormal) (`GameplayStatics.BreakHitResult` HitResultIn))
  (if (`self.IsHitscan?`)
    (if HitIn
      (`GameplayStatics.PlaySoundAtLocation` (`self.HitscanImpactSound`) _impactpoint (struct) 1.0 1.0 0.0 null null null null)
      (`GameplayStatics.SpawnEmitterAtLocation` (`self.HitscanImpactParticle`) _impactpoint (`KismetMathLibrary.MakeRotFromZ` _impactnormal)))))

(fn `DecrementAmmo`
  (set `self.CurrentAmmoInClip` (`KismetMathLibrary.Clamp` (- (`self.CurrentAmmoInClip`) 1) 0 (`self.MaxAmmoClipSize`))))

(fn `MultiFireFX`
  (params (HitResultsIn :type "HitResult Structure (by ref)") (HitIn :type Boolean))
  (bind (_bblockinghit _binitialoverlap _time _distance _location _impactpoint _normal _impactnormal) (`GameplayStatics.BreakHitResult` HitResultsIn))
  (if (`self.IsHitscan?`)
    (if HitIn
      (`GameplayStatics.PlaySoundAtLocation` (`self.HitscanImpactSound`) _impactpoint (struct) 1.0 1.0 0.0 null null null null)
      (`GameplayStatics.SpawnEmitterAtLocation` (`self.HitscanImpactParticle`) _impactpoint (`KismetMathLibrary.MakeRotFromZ` _impactnormal)))))

(fn `ReloadAddAmmo`
  (set `self.AmmoNeededForReload` (- (`self.MaxAmmoClipSize`) (`self.CurrentAmmoInClip`)))
  (if (<= (`self.CurrentMaxAmmo`) (`self.AmmoNeededForReload`))
    (set `self.CurrentAmmoInClip` (+ (`self.CurrentAmmoInClip`) (`self.CurrentMaxAmmo`)))
    (set `self.CurrentMaxAmmo` 0)
    (else
      (if (not (`self.IsEnemyWeapon?`))
        (set `self.CurrentMaxAmmo` (- (`self.CurrentMaxAmmo`) (`self.AmmoNeededForReload`))))
      (set `self.CurrentAmmoInClip` (`self.MaxAmmoClipSize`)))))

(fn `ShootInfo`
  (params (HitResultIn :type "HitResult Structure (by ref)") (HitIn :type Boolean) (MuzzleSocketLocation :type "Vector Structure"))
  (returns (HitResultOut :type "HitResult Structure") (HitOut :type Boolean))
  (bind (_bblockinghit _binitialoverlap _time _distance _location _impactpoint _normal _impactnormal _physmat _hitactor) (`GameplayStatics.BreakHitResult` HitResultIn))
  (bind (_bblockinghit_2 _binitialoverlap_2 _time_2 _distance_2 _location_2 _impactpoint_2 _normal_2 _impactnormal_2 _physmat_2 _hitactor_2 _hitcomponent _hitbonename _bonename _hititem _elementindex _faceindex _tracestart _traceend) (`GameplayStatics.BreakHitResult` HitResultIn))
  (if (`self.IsHitscan?`)
    (`GameplayStatics.ApplyDamage` _hitactor (`KismetMathLibrary.Conv_IntToDouble` (`self.Damage`)) (`self.GetInstigatorController`) self)
    (else
      (`|SpawnActorFromClass` (`self.Projectile`) (`KismetMathLibrary.MakeTransform` MuzzleSocketLocation (`KismetMathLibrary.FindLookAtRotation` MuzzleSocketLocation (`KismetMathLibrary.SelectVector` _impactpoint_2 _traceend HitIn))) "AlwaysSpawn" "SelectDefaultAtRuntime" (`self.GetOwner`) self (`self.GetInstigator`))))
  (`self.MakeNoise` self 1.0 null _location 0.0 "None")
  (`AISense_Damage.ReportDamageEvent` _hitactor self 50.0 (`self.K2_GetActorLocation`) _location)
  (return HitResultIn HitIn))

(fn `SingleFireFX`
  (params (HitResultIn :type "HitResult Structure (by ref)") (HitIn :type Boolean))
  (bind (_bblockinghit _binitialoverlap _time _distance _location _impactpoint _normal _impactnormal) (`GameplayStatics.BreakHitResult` HitResultIn))
  (bind _sk_weapon (`self.SK_Weapon`))
  (`GameplayStatics.SpawnSoundAttached` (`self.SingleFireSound`) _sk_weapon "None" (0.0 0.0 0.0) (struct) "SnapToTarget" false 1.0 1.0 0.0 null null)
  (bind _returnvalue (`GameplayStatics.SpawnEmitterAttached` (`self.SingleFireMuzzleFlash`) _sk_weapon (`self.MuzzleSocketName`) (0.0 0.0 0.0) (struct) (1.0 1.0 1.0) "SnapToTarget"))
  (`/Engine/EditorBlueprintResources/StandardMacros.IsValid` (`self.CharacterRef`)
    (:`Is Valid`
      (`PrimitiveComponent.SetOwnerNoSee` _returnvalue true))
    (:`Is Not Valid`
      _))
  (if (`self.IsHitscan?`)
    (if HitIn
      (`GameplayStatics.PlaySoundAtLocation` (`self.HitscanImpactSound`) _impactpoint (struct) 1.0 1.0 0.0 null null null null)
      (`GameplayStatics.SpawnEmitterAtLocation` (`self.HitscanImpactParticle`) _impactpoint (`KismetMathLibrary.MakeRotFromZ` _impactnormal)))))

(fn `UserConstructionScript`
  (bind _returnvalue (`PrimitiveComponent.CreateDynamicMaterialInstance` (`self.SK_Weapon`) 0 "/Game/RESOURCES/MATERIALS/M_Default_Weapon.M_Default_Weapon" "None"))
  (set `self.DynaMat` _returnvalue))

(fn `Weapon Sphere Trace`
  (returns (OutHit :type "HitResult Structure") (ReturnValue :type Boolean) (MuzzleSocketLocation :type "Vector Structure"))
  (bind _characterref (`self.CharacterRef`))
  (bind _spheretraceradius (`self.SphereTraceRadius`))
  (bind _array (`|MakeArray` _characterref :!type "Actor Object Reference"))
  (bind _weapontracestartlocation (`/Game/COMMON/ENTITIES/Character1.WeaponTraceStartLocation` _characterref))
  (bind _returnvalue (`SceneComponent.K2_GetComponentLocation` _weapontracestartlocation))
  (`/Engine/EditorBlueprintResources/StandardMacros.IsValid` _characterref
    (:`Is Valid`
      (bind (_outhit _returnvalue_2) (`KismetSystemLibrary.SphereTraceSingle` _returnvalue (`self.AddRandomSpread` (+ _returnvalue (* (`KismetMathLibrary.GetForwardVector` (`SceneComponent.K2_GetComponentRotation` _weapontracestartlocation)) (`self.SphereTraceRange`)))) _spheretraceradius "TraceTypeQuery3" false _array "ForDuration"))
      (bind (_bblockinghit _binitialoverlap _time _distance _location _impactpoint _normal _impactnormal _physmat _hitactor _hitcomponent _hitbonename _bonename _hititem _elementindex _faceindex _tracestart _traceend) (`GameplayStatics.BreakHitResult` _outhit))
      (bind (_outhit_2 _returnvalue_3) (`KismetSystemLibrary.SphereTraceSingle` (`SceneComponent.GetSocketLocation` (`self.SK_Weapon`) (`self.MuzzleSocketName`)) (`KismetMathLibrary.SelectVector` _impactpoint _traceend _returnvalue_2) _spheretraceradius "TraceTypeQuery3" false _array "ForDuration"))
      (return _outhit_2 _returnvalue_3 (`SceneComponent.GetSocketLocation` (`self.SK_Weapon`) (`self.MuzzleSocketName`))))))
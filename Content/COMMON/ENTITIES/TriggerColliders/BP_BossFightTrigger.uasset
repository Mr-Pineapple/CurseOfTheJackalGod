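; Trigger actor that starts the boss fight when any of the four playable character classes enters one of its three box volumes.
; Each box runs its own copy of the same logic, gated by a separate DoOnce, so it can fire once per box.
; It finds BPDoor4 via GetActorOfClass and closes it, then finds BP_Enemy_Boss and adds its health bar widget to the player screen.
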(event `self.Box.OnComponentBeginOverlap`
  (params (OverlappedComponent :type "PrimitiveComponent Object Reference") (OtherActor :type "Actor Object Reference") (OtherComp :type "PrimitiveComponent Object Reference") (OtherBodyIndex :type Integer) (bFromSweep :type Boolean) (SweepResult :type "HitResult Structure (by ref)"))
  (cast `/Game/COMMON/ENTITIES/Characters/Character1` OtherActor
    (:`then`
      _)
    (:`CastFailed`
      (cast `/Game/COMMON/ENTITIES/Characters/Character2` OtherActor
        (:`then`
          _)
        (:`CastFailed`
          (cast `/Game/COMMON/ENTITIES/Characters/Character3` OtherActor
            (:`then`
              _)
            (:`CastFailed`
              (cast `/Game/COMMON/ENTITIES/Characters/Character4` OtherActor)))))))
  (`/Engine/EditorBlueprintResources/StandardMacros.DoOnce` false
    (:`Completed`
      (bind _returnvalue (`GameplayStatics.GetActorOfClass` "/Game/COMMON/ENTITIES/Doors/BPDoor4.BPDoor4_C"))
      (`/Engine/EditorBlueprintResources/StandardMacros.IsValid` _returnvalue
        (:`Is Valid`
          (`/Game/COMMON/ENTITIES/Doors/BPDoor4.CloseDoor` _returnvalue)
          (bind _returnvalue_2 (`GameplayStatics.GetActorOfClass` "/Game/COMMON/ENTITIES/AI/Enemies/BossEnemy/BP_Enemy_Boss.BP_Enemy_Boss_C"))
          (`/Engine/EditorBlueprintResources/StandardMacros.IsValid` _returnvalue_2
            (:`Is Valid`
              (bind _bosshealthbarwidgetref (`/Game/COMMON/ENTITIES/AI/Enemies/BossEnemy/BP_Enemy_Boss.BossHealthbarWidgetRef` _returnvalue_2))
              (`/Engine/EditorBlueprintResources/StandardMacros.IsValid` _bosshealthbarwidgetref
                (:`Is Valid`
                  (`UserWidget.AddToPlayerScreen` _bosshealthbarwidgetref 0))))))))))

(event `self.Box2.OnComponentBeginOverlap`
  (params (OverlappedComponent :type "PrimitiveComponent Object Reference") (OtherActor :type "Actor Object Reference") (OtherComp :type "PrimitiveComponent Object Reference") (OtherBodyIndex :type Integer) (bFromSweep :type Boolean) (SweepResult :type "HitResult Structure (by ref)"))
  (cast `/Game/COMMON/ENTITIES/Characters/Character1` OtherActor
    (:`then`
      _)
    (:`CastFailed`
      (cast `/Game/COMMON/ENTITIES/Characters/Character2` OtherActor
        (:`then`
          _)
        (:`CastFailed`
          (cast `/Game/COMMON/ENTITIES/Characters/Character3` OtherActor
            (:`then`
              _)
            (:`CastFailed`
              (cast `/Game/COMMON/ENTITIES/Characters/Character4` OtherActor)))))))
  (`/Engine/EditorBlueprintResources/StandardMacros.DoOnce` false
    (:`Completed`
      (bind _returnvalue (`GameplayStatics.GetActorOfClass` "/Game/COMMON/ENTITIES/Doors/BPDoor4.BPDoor4_C"))
      (`/Engine/EditorBlueprintResources/StandardMacros.IsValid` _returnvalue
        (:`Is Valid`
          (`/Game/COMMON/ENTITIES/Doors/BPDoor4.CloseDoor` _returnvalue)
          (bind _returnvalue_2 (`GameplayStatics.GetActorOfClass` "/Game/COMMON/ENTITIES/AI/Enemies/BossEnemy/BP_Enemy_Boss.BP_Enemy_Boss_C"))
          (`/Engine/EditorBlueprintResources/StandardMacros.IsValid` _returnvalue_2
            (:`Is Valid`
              (bind _bosshealthbarwidgetref (`/Game/COMMON/ENTITIES/AI/Enemies/BossEnemy/BP_Enemy_Boss.BossHealthbarWidgetRef` _returnvalue_2))
              (`/Engine/EditorBlueprintResources/StandardMacros.IsValid` _bosshealthbarwidgetref
                (:`Is Valid`
                  (`UserWidget.AddToPlayerScreen` _bosshealthbarwidgetref 0))))))))))

(event `self.Box1.OnComponentBeginOverlap`
  (params (OverlappedComponent :type "PrimitiveComponent Object Reference") (OtherActor :type "Actor Object Reference") (OtherComp :type "PrimitiveComponent Object Reference") (OtherBodyIndex :type Integer) (bFromSweep :type Boolean) (SweepResult :type "HitResult Structure (by ref)"))
  (cast `/Game/COMMON/ENTITIES/Characters/Character1` OtherActor
    (:`then`
      _)
    (:`CastFailed`
      (cast `/Game/COMMON/ENTITIES/Characters/Character2` OtherActor
        (:`then`
          _)
        (:`CastFailed`
          (cast `/Game/COMMON/ENTITIES/Characters/Character3` OtherActor
            (:`then`
              _)
            (:`CastFailed`
              (cast `/Game/COMMON/ENTITIES/Characters/Character4` OtherActor)))))))
  (`/Engine/EditorBlueprintResources/StandardMacros.DoOnce` false
    (:`Completed`
      (bind _returnvalue (`GameplayStatics.GetActorOfClass` "/Game/COMMON/ENTITIES/Doors/BPDoor4.BPDoor4_C"))
      (`/Engine/EditorBlueprintResources/StandardMacros.IsValid` _returnvalue
        (:`Is Valid`
          (`/Game/COMMON/ENTITIES/Doors/BPDoor4.CloseDoor` _returnvalue)
          (bind _returnvalue_2 (`GameplayStatics.GetActorOfClass` "/Game/COMMON/ENTITIES/AI/Enemies/BossEnemy/BP_Enemy_Boss.BP_Enemy_Boss_C"))
          (`/Engine/EditorBlueprintResources/StandardMacros.IsValid` _returnvalue_2
            (:`Is Valid`
              (bind _bosshealthbarwidgetref (`/Game/COMMON/ENTITIES/AI/Enemies/BossEnemy/BP_Enemy_Boss.BossHealthbarWidgetRef` _returnvalue_2))
              (`/Engine/EditorBlueprintResources/StandardMacros.IsValid` _bosshealthbarwidgetref
                (:`Is Valid`
                  (`UserWidget.AddToPlayerScreen` _bosshealthbarwidgetref 0))))))))))

(fn `UserConstructionScript`)
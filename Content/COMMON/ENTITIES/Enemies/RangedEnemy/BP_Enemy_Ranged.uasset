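; Ranged enemy built on a parent enemy class, spawning a rifle on BeginPlay and attaching it to a hand socket.
; Attack focuses the player and plays a montage whose notify fires a traced bullet from the weapon toward the target through BPCAttacks, ending on completion or interruption.
; Overrides set movement speeds and ideal combat range, while damage and health queries delegate to BPCDamageSystem and Heal is a stub returning zero.
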(event `self.ReceiveBeginPlay`
  (`parent.ReceiveBeginPlay`)
  (`self.EquipWeapon`))

(event `/Game/COMMON/ENTITIES/Enemies/AI/BPI_EnemyAI.EquipWeapon`
  ;[1 1 1] Equip Weapon
  (bind _returnvalue (`|SpawnActorFromClass` "/Game/COMMON/ENTITIES/BP_Weapon_Rifle.BP_Weapon_Rifle_C" (`KismetMathLibrary.MakeTransform` (0.0 0.0 0.0)) "Undefined" "MultiplyWithRoot" null null))
  (bind _output_get (set `self.WeaponActor` _returnvalue))
  (`self.K2_AttachToComponent` _output_get (`self.Mesh`) "hand_r_rifle_socket" "SnapToTarget" "SnapToTarget" "SnapToTarget" true)
  (set `self.IsWieldingWeapon` true)
  (`self.OnWeaponEquipped`))

(event `/Game/COMMON/ENTITIES/Enemies/AI/BPI_EnemyAI.Attack`
  (params (AttackTarget :type "Actor Object Reference"))
  ;[1 1 1] Fire Rifle
  (`self.FocusPlayerAndAttack`)
  (`parent.Attack` AttackTarget)
  (bind _notifyname (`|PlayMontage` (`self.Mesh`))
    (:`OnCompleted`
      (`self.AttackEnd` AttackTarget :!label _label))
    (:`OnInterrupted`
      (goto _label))
    (:`OnNotifyBegin`
      (switch `name` _notifyname
        (:`Fire`
          (`/Game/COMMON/COMPONENTS/BPC_Attacks.FireBullet` (`self.BPC_Attacks`) (`self.K2_GetActorLocation` (`self.WeaponActor`)) (`self.K2_GetActorLocation` AttackTarget) (make `/Game/COMMON/UTILITIES/S_DamageInfo` 5.0 "NewEnumerator2" "NewEnumerator0" false true)))))))

(fn `GetCurrentHealth`
  (returns (Health :type "Float (double-precision)"))
  (return (`/Game/COMMON/COMPONENTS/BPC_DamageSystem.Health` (`self.BPC_DamageSystem`))))

(fn `GetIdealRange`
  (returns (AttackRadius :type "Float (double-precision)") (DefendRadius :type "Float (double-precision)"))
  (return 200.0 200.0))

(fn `GetMaxHealth`
  (returns (MaxHealth :type "Float (double-precision)"))
  (return (`/Game/COMMON/COMPONENTS/BPC_DamageSystem.MaxHealth` (`self.BPC_DamageSystem`))))

(fn `Heal`
  (params (Amount :type "Float (double-precision)"))
  (returns (NewHealth :type "Float (double-precision)"))
  (return 0.0))

(fn `SetMovementSpeed`
  (params (Speed :type "/Game/COMMON/ENTITIES/Enemies/AI/Enums/E_MovementSpeed Enum" :default "NewEnumerator0"))
  (returns (SpeedValue :type "Float (double-precision)"))
  (bind _output_get (set `CharacterMovementComponent.MaxWalkSpeed` (select `/Game/COMMON/ENTITIES/Enemies/AI/Enums/E_MovementSpeed` Speed :`NewEnumerator1` 200.0 :`NewEnumerator2` 300.0 :`NewEnumerator3` 500.0 :!type "Float (single-precision)") (`self.CharacterMovement`)))
  (return _output_get))

(fn `TakeDamage`
  (params (DamageInfo :type "/Game/COMMON/UTILITIES/S_DamageInfo Structure") (`Damage Causer` :type "Actor Object Reference"))
  (returns (WasDamaged :type Boolean))
  (bind _wasdamaged (`/Game/COMMON/COMPONENTS/BPC_DamageSystem.TakeDamage` (`self.BPC_DamageSystem`) DamageInfo `Damage Causer`))
  (return _wasdamaged))

(fn `UserConstructionScript`
  (`parent.UserConstructionScript`))
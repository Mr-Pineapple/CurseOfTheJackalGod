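; BP_EnemyWave tracks the enemies of the first wave and opens doors once none remain.
; StartWave runs once, shows the remaining-enemy count on Character1's HUD and starts a looping timer.
; The timer polls actors tagged "Wave1" to update the count.
; When none are left, it calls OpenDoor on BP_EnemyWaveTrigger and BP_Door, hides the counter and clears the timer.
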(event `StartWave`
  (bind _character_1hud (`self.Character 1HUD`))
  (`/Engine/EditorBlueprintResources/StandardMacros.DoOnce` false
    (:`Completed`
      (bind _returnvalue (`GameplayStatics.GetActorOfClass` "/Game/COMMON/ENTITIES/Characters/Character1.Character1_C"))
      (bind _output_get (set `self.Character1` _returnvalue))
      (`/Engine/EditorBlueprintResources/StandardMacros.IsValid` _output_get
        (:`Is Valid`
          (set `self.Character 1HUD` (`/Game/COMMON/ENTITIES/Characters/Character1.Character1HUD` _output_get))
          (bind _outactors (`GameplayStatics.GetAllActorsWithTag` "Wave1"))
          (bind _output_get_2 (set `self.Wave1Enemies` _outactors))
          (`TextBlock.SetText` (`/Game/CLIENT/RENDERING/Widget/Character1HUD.NumberOfEnemies` (`self.Character 1HUD`)) (`KismetTextLibrary.Conv_IntToText` (`KismetArrayLibrary.Array_Length` _output_get_2)))
          (`/Engine/EditorBlueprintResources/StandardMacros.IsValid` _character_1hud
            (:`Is Valid`
              (`Widget.SetVisibility` (`/Game/CLIENT/RENDERING/Widget/Character1HUD.NumberOfEnemies` _character_1hud) "Visible")
              (`Widget.SetVisibility` (`/Game/CLIENT/RENDERING/Widget/Character1HUD.EnemiesToKill_Text` _character_1hud) "Visible")
              (bind _returnvalue_2 (`KismetSystemLibrary.K2_SetTimerDelegate` (delegate `EnemyWave`) 2.0 true))
              (set `self.EnemyWave_TimeHandle` _returnvalue_2))))))))

(event `EnemyWave`
  (bind _character_1hud (`self.Character 1HUD`))
  (bind _outactors (`GameplayStatics.GetAllActorsWithTag` "Wave1"))
  (bind _output_get (set `self.Wave1Enemies` _outactors))
  (`TextBlock.SetText` (`/Game/CLIENT/RENDERING/Widget/Character1HUD.NumberOfEnemies` (`self.Character 1HUD`)) (`KismetTextLibrary.Conv_IntToText` (`KismetArrayLibrary.Array_Length` _output_get)))
  (if (`KismetArrayLibrary.Array_IsEmpty` _output_get)
    (set `self.IsNoEnemies?` false)
    (bind _returnvalue (`GameplayStatics.GetActorOfClass` "/Game/COMMON/PUZZLES/BP_EnemyWaveTrigger.BP_EnemyWaveTrigger_C"))
    (`/Game/COMMON/PUZZLES/BP_EnemyWaveTrigger.OpenDoor` _returnvalue)
    (bind _returnvalue_2 (`GameplayStatics.GetActorOfClass` "/Game/COMMON/PUZZLES/BP_Door.BP_Door_C"))
    (`/Game/COMMON/PUZZLES/BP_Door.OpenDoor` _returnvalue_2)
    (`Widget.SetVisibility` (`/Game/CLIENT/RENDERING/Widget/Character1HUD.NumberOfEnemies` _character_1hud) "Hidden")
    (`Widget.SetVisibility` (`/Game/CLIENT/RENDERING/Widget/Character1HUD.EnemiesToKill_Text` _character_1hud) "Hidden")
    (`KismetSystemLibrary.K2_ClearAndInvalidateTimerHandle` (`self.EnemyWave_TimeHandle`))))

(fn `UserConstructionScript`)
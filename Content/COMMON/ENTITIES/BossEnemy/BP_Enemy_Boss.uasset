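; Boss enemy character with its own health bar widget, a socketed axe it can equip, and high health set at construction.
; Attack events use BPCAttacks or montage notifies for melee combos, jump, smash, homing axe throw and AOE trail, applying typed damage.
; Teleport is faked by hiding the mesh and flying rapidly via AIMoveTo.
; A float phase spawns a platform and grants invincibility until it descends, with dispatchers signalling each action's completion.
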(event `self.ReceiveBeginPlay`
  (bind _bpc_damagesystem (`self.BPC_DamageSystem`))
  ;[1 1 1] HealthBar
  (`parent.ReceiveBeginPlay`)
  (`WidgetComponent.SetWidget` (`self.HealthBar`) null)
  (bind _returnvalue (`|CreateWidget` null))
  (bind _output_get (set `self.BossHealthbarWidgetRef` _returnvalue))
  (`self.UpdateHealthPercentage` _output_get (`/Game/COMMON/ENTITIES/BossEnemy/BP_Enemy_Boss.Health` _bpc_damagesystem) (`/Game/COMMON/ENTITIES/BossEnemy/BP_Enemy_Boss.MaxHealth` _bpc_damagesystem))
  (add `self.OnDeath` (delegate `Deactivate HealthBar`)))

(event `Deactivate HealthBar`
  ;[1 1 1] HealthBar
  (`Widget.SetVisibility` (`self.BossHealthbarWidgetRef`) "Hidden"))

(event `self.EquipWeapon`
  ;[1 1 1] Equip/Unequip Weapon
  (bind _returnvalue (`|SpawnActorFromClass` null (`KismetMathLibrary.MakeTransform` (0.0 0.0 0.0)) "Undefined" "MultiplyWithRoot" null null))
  (bind _output_get (set `self.WeaponActor` _returnvalue))
  (`self.K2_AttachToComponent` _output_get (`self.Mesh`) "hand_r_axe_socket" "SnapToTarget" "SnapToTarget" "SnapToTarget" true)
  (set `self.IsWieldingWeapon` true)
  (`KismetSystemLibrary.DelayUntilNextTick`)
  (`self.OnWeaponEquipped`))

(event `self.UnequipWeapon`
  ;[1 1 1] Equip/Unequip Weapon
  (`self.K2_DestroyActor` (`self.WeaponActor`))
  (set `self.IsWieldingWeapon` false)
  (`KismetSystemLibrary.DelayUntilNextTick`)
  (`self.OnWeaponUnequipped`))

(event `Teleport`
  (params (Location :type "Vector Structure") (AttackTarget :type "Actor Object Reference"))
  (bind _charactermovement (`self.CharacterMovement`))
  ;[1 1 1] TELEPORT
  (if (not (`self.IsTeleporting`))
    (set `self.IsTeleporting` true)
    (`CharacterMovementComponent.SetMovementMode` _charactermovement "MOVE_Flying" 0)
    (set `CharacterMovementComponent.MaxFlySpeed` 5000.0 _charactermovement)
    (set `CharacterMovementComponent.MaxAcceleration` 99999.0 _charactermovement)
    (`SceneComponent.SetVisibility` (`self.Mesh`) false true)
    (`PrimitiveComponent.SetCollisionResponseToChannel` (`self.CapsuleComponent`) "ECC_Pawn" "ECR_Ignore")
    (`self.StopAnimMontage` null)
    (`|AIMoveTo` self Location AttackTarget 150.0
      (:`OnSuccess`
        _)
      (:`OnFail`
        _))
    (`self.TeleportEnd`)
    (else
      (`KismetSystemLibrary.DelayUntilNextTick`)
      (`self.OnTeleportEnd`))))

(event `TeleportEnd`
  (bind _charactermovement (`self.CharacterMovement`))
  ;[1 1 1] TELEPORT
  (`MovementComponent.StopMovementImmediately` _charactermovement)
  (`CharacterMovementComponent.SetMovementMode` _charactermovement "MOVE_Walking" 0)
  (set `CharacterMovementComponent.MaxAcceleration` 1500.0 _charactermovement)
  (`SceneComponent.SetVisibility` (`self.Mesh`) true true)
  (`PrimitiveComponent.SetCollisionResponseToChannel` (`self.CapsuleComponent`) "ECC_Pawn" "ECR_Block")
  (`self.OnTeleportEnd`)
  (`KismetSystemLibrary.Delay` 0.5)
  (set `self.IsTeleporting` false))

(event `AttackCombo1`
  (params (AttackTarget :type "Actor Object Reference"))
  ;[1 1 1] Attacks
  (`self.PrimaryMeleeAttack` (`self.BPC_Attacks`) (make `` AttackTarget null (make `` 20.0 0 0 false true true)) 40.0 220.0))

(event `StartFloat`
  (bind _returnvalue (`self.K2_GetActorLocation`))
  ;[1 1 1] Floating Pillar Ability
  (set `/Game/COMMON/ENTITIES/BossEnemy/BP_Enemy_Boss.IsInvincible` true (`self.BPC_DamageSystem`))
  (bind _outhit (`KismetSystemLibrary.LineTraceSingle` _returnvalue (* _returnvalue (1.0 1.0 -1000.0)) "TraceTypeQuery1"))
  (bind _returnvalue_2 (`|SpawnActorFromClass` null (`KismetMathLibrary.MakeTransform` (`.Location` (`GameplayStatics.BreakHitResult` _outhit))) "Undefined" "MultiplyWithRoot" null null))
  (bind _output_get (set `self.FloatingPlatformRef` _returnvalue_2))
  (add `self.OnFloatTimelineFinished` _output_get (delegate `OnFloatTimelineFinished_Event`)))

(event `AttackCombo2`
  (params (AttackTarget :type "Actor Object Reference"))
  ;[1 1 1] Attacks
  (`self.Attack` AttackTarget)
  (bind _notifyname (`|PlayMontage` (`self.Mesh`))
    (:`OnCompleted`
      (`self.AttackEnd` AttackTarget :!label _label))
    (:`OnInterrupted`
      (goto _label))
    (:`OnNotifyBegin`
      (switch `name` _notifyname
        (:`Slash`
          (`self.SphereTraceDamage` (`self.BPC_Attacks`) (make `` 10.0 0 0 false true true) 40.0 220.0))
        (:`AOESlash`
          (`self.AOEDamage` (`self.BPC_Attacks`) 300.0 (make `` 10.0 0 0 false false false true)))))))

(event `OnFloatTimelineFinished_Event`
  ;[1 1 1] Floating Pillar Ability
  (remove `self.OnFloatTimelineFinished` (stale `StartFloat` _output_get) (delegate `OnFloatTimelineFinished_Event`))
  (`self.OnFloatHeightReached`))

(event `StopFloat`
  ;[1 1 1] Floating Pillar Ability
  (bind _floatingplatformref (`self.FloatingPlatformRef`)
    (:`then`
      (`self.StopFloating` _floatingplatformref)
      (add `self.OnFloatTimelineFinished` _floatingplatformref (delegate `OnFloatTimelineFinished_Event_0`)))
    (:`else`
      (`KismetSystemLibrary.DelayUntilNextTick`)
      (set `/Game/COMMON/ENTITIES/BossEnemy/BP_Enemy_Boss.IsInvincible` false (`self.BPC_DamageSystem`) :!label _label_2)
      (`self.OnFloatEnded`))))

(event `OnFloatTimelineFinished_Event_0`
  ;[1 1 1] Floating Pillar Ability
  (remove `self.OnFloatTimelineFinished` (stale `StopFloat` _floatingplatformref) (delegate `OnFloatTimelineFinished_Event_0`))
  (`self.K2_DestroyActor` (stale `StopFloat` _floatingplatformref))
  (goto _label_2))

(event `ThrowAxe`
  (params (AttackTarget :type "Actor Object Reference"))
  ;[1 1 1] Attacks
  (`self.Attack` AttackTarget)
  (bind _notifyname (`|PlayMontage` (`self.Mesh`))
    (:`OnCompleted`
      (`SceneComponent.SetVisibility` (`/Game/COMMON/ENTITIES/BossEnemy/BP_Enemy_Boss.Mesh` (`self.WeaponActor`)) true false :!label _label_3)
      (`self.AttackEnd` AttackTarget))
    (:`OnInterrupted`
      (goto _label_3))
    (:`OnNotifyBegin`
      (switch `name` _notifyname
        (:`Throw`
          (`SceneComponent.SetVisibility` (`/Game/COMMON/ENTITIES/BossEnemy/BP_Enemy_Boss.Mesh` (`self.WeaponActor`)) false false)
          (bind _returnvalue (`|SpawnActorFromClass` null (`KismetMathLibrary.MakeTransform` (`SceneComponent.GetSocketLocation` (`self.Mesh`) "hand_r")) "Undefined" "MultiplyWithRoot" null 4000.0 0.0 AttackTarget true self))
          (add `self.OnProjectileImpact` _returnvalue (delegate `OnProjectileImpact_Event`)))))))

(event `self.ReceiveAnyDamage`
  (params (Damage :type "Float (single-precision)") (DamageType :type "DamageType Object Reference") (InstigatedBy :type "Controller Object Reference") (DamageCauser :type "Actor Object Reference"))
  (bind _weaponactor (`self.WeaponActor`))
  (bind _bpc_damagesystem (`self.BPC_DamageSystem`))
  ;[1 1 1] AnyDamage
  (set `/Game/COMMON/ENTITIES/BossEnemy/BP_Enemy_Boss.Health` (- (`/Game/COMMON/ENTITIES/BossEnemy/BP_Enemy_Boss.Health` _bpc_damagesystem) Damage) _bpc_damagesystem)
  (if (<= (`/Game/COMMON/ENTITIES/BossEnemy/BP_Enemy_Boss.Health` _bpc_damagesystem) 0.0)
    (`|ExecutionSequence`
      (:`then_0`
        (`/Engine/EditorBlueprintResources/StandardMacros.IsValid` _weaponactor
          (:`Is Valid`
            (`self.K2_DestroyActor` _weaponactor))))
      (:`then_1`
        (bind _returnvalue (`GameplayStatics.GetActorOfClass` null))
        (`/Engine/EditorBlueprintResources/StandardMacros.IsValid` _returnvalue
          (:`Is Valid`
            (`self.K2_DestroyActor` _returnvalue))))
      (:`then_2`
        (`self.K2_DestroyActor`)))))

(event `OnProjectileImpact_Event` :!signature `self.OnProjectileImpact`
  (params (OtherActor :type "Actor Object Reference") (Hit :type "HitResult Structure"))
  ;[1 1 1] Attacks
  (message `/Game/COMMON/ENTITIES/BossEnemy/BP_Enemy_Boss.TakeDamage` OtherActor (make `` 10.0 0 0 false true) self))

(event `QuickAttack`
  (params (AttackTarget :type "Actor Object Reference"))
  ;[1 1 1] Attacks
  (`self.PrimaryMeleeAttack` (`self.BPC_Attacks`) (make `` AttackTarget null (make `` 10.0 0 0 false true true)) 40.0 220.0))

(event `JumpAttack`
  (params (AttackTarget :type "Actor Object Reference"))
  ;[1 1 1] Attacks
  (`self.LongRangeMeleeAttack` (`self.BPC_Attacks`) (make `` AttackTarget null (make `` 10.0 0 0 false false false true))))

(event `GroundSmash`
  (params (AttackTarget :type "Actor Object Reference"))
  ;[1 1 1] Attacks
  (`self.GroundSmash` (`self.BPC_Attacks`) (make `` AttackTarget null (make `` 10.0 0 0 false false false true)) 1100.0))

(event `AOETrail`
  (params (AttackTarget :type "Actor Object Reference"))
  ;[1 1 1] Attacks
  (`self.Attack` AttackTarget)
  (bind _notifyname (`|PlayMontage` (`self.Mesh`))
    (:`OnCompleted`
      (`self.AttackEnd` AttackTarget :!label _label_4))
    (:`OnInterrupted`
      (goto _label_4))
    (:`OnNotifyBegin`
      (switch `name` _notifyname
        (:`Strike`
          (bind _returnvalue (`|SpawnActorFromClass` null (`KismetMathLibrary.MakeTransform` (0.0 0.0 0.0)) "Undefined" "MultiplyWithRoot" null 1.0 AttackTarget null false false false null))
          (set `/Game/COMMON/ENTITIES/BossEnemy/BP_Enemy_Boss.BlastEffect` null _returnvalue)
          (add `self.OnAOEOverlapActor` _returnvalue (delegate `OnAOEOverlapActor_Event`)))))))

(event `OnAOEOverlapActor_Event` :!signature `self.OnAOEOverlapActor`
  (params (Actor :type "Actor Object Reference"))
  ;[1 1 1] Attacks
  (bind _teamnumber (message `/Game/COMMON/ENTITIES/BossEnemy/BP_Enemy_Boss.GetTeamNumber` Actor))
  (if (!= _teamnumber (`self.TeamNumber`))
    (message `/Game/COMMON/ENTITIES/BossEnemy/BP_Enemy_Boss.TakeDamage` Actor (make `` 10.0 0 0) self)))

(fn `CanBeTargeted`
  (returns (ReturnValue :type Boolean))
  (return false))

(fn `GetCurrentHealth`
  (returns (Health :type "Float (double-precision)"))
  (return 0.0))

(fn `GetMaxHealth`
  (returns (MaxHealth :type "Float (double-precision)"))
  (return 0.0))

(fn `SetMovementSpeed`
  (params (Speed :type Byte :default 0))
  (returns (SpeedValue :type "Float (double-precision)"))
  (bind _output_get (set `CharacterMovementComponent.MaxWalkSpeed` (select `byte` Speed :`NewEnumerator0` 0.0 :`NewEnumerator1` 100.0 :`NewEnumerator2` 200.0 :`NewEnumerator3` 350.0 :!type "Float (single-precision)") (`self.CharacterMovement`)))
  (return _output_get))

(fn `TakeDamage`
  (params (DamageInfo :type " Structure") (`Damage Causer` :type "Actor Object Reference"))
  (returns (WasDamaged :type Boolean))
  (bind _bpc_damagesystem (`self.BPC_DamageSystem`))
  (bind _wasdamaged (`parent.TakeDamage` DamageInfo `Damage Causer`))
  (`/Engine/EditorBlueprintResources/StandardMacros.IsValid` _bpc_damagesystem
    (:`Is Valid`
      (`self.UpdateHealthPercentage` (`self.BossHealthbarWidgetRef`) (`/Game/COMMON/ENTITIES/BossEnemy/BP_Enemy_Boss.Health` _bpc_damagesystem) (`/Game/COMMON/ENTITIES/BossEnemy/BP_Enemy_Boss.MaxHealth` _bpc_damagesystem))
      (return _wasdamaged))))

(fn `UserConstructionScript`
  (bind _bpc_damagesystem (`self.BPC_DamageSystem`))
  (`parent.UserConstructionScript`)
  (bind _output_get (set `/Game/COMMON/ENTITIES/BossEnemy/BP_Enemy_Boss.MaxHealth` 700.0 _bpc_damagesystem))
  (set `/Game/COMMON/ENTITIES/BossEnemy/BP_Enemy_Boss.Health` _output_get _bpc_damagesystem))
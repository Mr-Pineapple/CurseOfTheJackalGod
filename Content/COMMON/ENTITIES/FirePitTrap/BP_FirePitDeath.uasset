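; BP_FirePitDeath is a fire pit trap hazard that kills player characters who enter it.
; The Box overlap event casts the other actor through four character classes in turn and calls Death on the first match, ignoring anything else.
; A separate ActivateVFX event switches on five particle systems and is not called within this Blueprint, so the lethal overlap does not depend on it.
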(event `Activate VFX`
  (`ActorComponent.Activate` (`self.ParticleSystem1`) false)
  (`ActorComponent.Activate` (`self.ParticleSystem2`) false)
  (`ActorComponent.Activate` (`self.ParticleSystem3`) false)
  (`ActorComponent.Activate` (`self.ParticleSystem4`) false)
  (`ActorComponent.Activate` (`self.ParticleSystem5`) false))

(event `self.Box.OnComponentBeginOverlap`
  (params (OverlappedComponent :type "PrimitiveComponent Object Reference") (OtherActor :type "Actor Object Reference") (OtherComp :type "PrimitiveComponent Object Reference") (OtherBodyIndex :type Integer) (bFromSweep :type Boolean) (SweepResult :type "HitResult Structure (by ref)"))
  (bind _ascharacter_1 (cast `/Game/COMMON/ENTITIES/Characters/Character1` OtherActor)
    (:`then`
      (`/Game/COMMON/ENTITIES/Characters/Character1.Death` _ascharacter_1))
    (:`CastFailed`
      (bind _ascharacter_2 (cast `/Game/COMMON/ENTITIES/Characters/Character2` OtherActor)
        (:`then`
          (`/Game/COMMON/ENTITIES/Characters/Character2.Death` _ascharacter_2))
        (:`CastFailed`
          (bind _ascharacter_3 (cast `/Game/COMMON/ENTITIES/Characters/Character3` OtherActor)
            (:`then`
              (`/Game/COMMON/ENTITIES/Characters/Character3.Death` _ascharacter_3))
            (:`CastFailed`
              (bind _ascharacter_4 (cast `/Game/COMMON/ENTITIES/Characters/Character4` OtherActor))
              (`/Game/COMMON/ENTITIES/Characters/Character4.Death` _ascharacter_4))))))))

(fn `UserConstructionScript`)
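; Enemy wave counter that shows how many Wave1-tagged enemies remain and opens doors when none are left.
; StartWave runs once, checks for each of four character classes and starts looping two-second timers sharing one handle variable.
; Each timer event recounts tagged actors; at zero it calls OpenDoor on the wave trigger and three doors, hides the counter and clears the timer.
; Nearly all HUD updates target Character1HUD, even in other characters' branches.
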(event `StartWave`
  (bind _character_1hud (`self.Character 1HUD`))
  (bind _character_1hud_2 (`self.Character 1HUD`))
  (bind _character_1hud_3 (`self.Character 1HUD`))
  (bind _character_1hud_4 (`self.Character 1HUD`))
  (`/Engine/EditorBlueprintResources/StandardMacros.DoOnce` false
    (:`Completed`
      (`|ExecutionSequence`
        (:`then_0`
          (bind _returnvalue (`GameplayStatics.GetActorOfClass` "/Game/COMMON/ENTITIES/Characters/Character1.Character1_C"))
          (bind _output_get (set `self.Character1` _returnvalue))
          (`/Engine/EditorBlueprintResources/StandardMacros.IsValid` _output_get
            (:`Is Valid`
              (bind _character1hud (`/Game/COMMON/ENTITIES/Characters/Character1.Character1HUD` _output_get))
              (`/Engine/EditorBlueprintResources/StandardMacros.IsValid` _character1hud
                (:`Is Valid`
                  (set `self.Character 1HUD` _character1hud)
                  (bind _outactors (`GameplayStatics.GetAllActorsWithTag` "Wave1"))
                  (bind _output_get_2 (set `self.Wave1Enemies` _outactors))
                  (`TextBlock.SetText` (`/Game/CLIENT/RENDERING/Widget/Character1HUD.NumberOfEnemies` (`self.Character 1HUD`)) (`KismetTextLibrary.Conv_IntToText` (`KismetArrayLibrary.Array_Length` _output_get_2)))
                  (`/Engine/EditorBlueprintResources/StandardMacros.IsValid` _character_1hud
                    (:`Is Valid`
                      (`Widget.SetVisibility` (`/Game/CLIENT/RENDERING/Widget/Character1HUD.NumberOfEnemies` _character_1hud) "Visible")
                      (`Widget.SetVisibility` (`/Game/CLIENT/RENDERING/Widget/Character1HUD.EnemiesToKill_Text` _character_1hud) "Visible")
                      (bind _returnvalue_2 (`KismetSystemLibrary.K2_SetTimerDelegate` (delegate `EnemyWave_Character1`) 2.0 true))
                      (set `self.EnemyWave_TimeHandle` _returnvalue_2))))))))
        (:`then_1`
          (bind _returnvalue_3 (`GameplayStatics.GetActorOfClass` "/Game/COMMON/ENTITIES/Characters/Character2.Character2_C"))
          (bind _output_get_3 (set `self.Character2` _returnvalue_3))
          (`/Engine/EditorBlueprintResources/StandardMacros.IsValid` _output_get_3
            (:`Is Valid`
              (bind _characterhud2 (`/Game/COMMON/ENTITIES/Characters/Character2.CharacterHUD2` _output_get_3))
              (`/Engine/EditorBlueprintResources/StandardMacros.IsValid` _characterhud2
                (:`Is Valid`
                  (set `self.Character2 HUD` _characterhud2)
                  (bind _outactors_2 (`GameplayStatics.GetAllActorsWithTag` "Wave1"))
                  (bind _output_get_4 (set `self.Wave1Enemies` _outactors_2))
                  (`TextBlock.SetText` (`KismetTextLibrary.Conv_IntToText` (`KismetArrayLibrary.Array_Length` _output_get_4)))
                  (`/Engine/EditorBlueprintResources/StandardMacros.IsValid` _character_1hud_2
                    (:`Is Valid`
                      (`Widget.SetVisibility` (`/Game/CLIENT/RENDERING/Widget/Character1HUD.NumberOfEnemies` _character_1hud_2) "Visible")
                      (`Widget.SetVisibility` (`/Game/CLIENT/RENDERING/Widget/Character1HUD.EnemiesToKill_Text` _character_1hud_2) "Visible")
                      (bind _returnvalue_4 (`KismetSystemLibrary.K2_SetTimerDelegate` (delegate `EnemyWave_Character2`) 2.0 true))
                      (set `self.EnemyWave_TimeHandle` _returnvalue_4))))))))
        (:`then_2`
          (bind _returnvalue_5 (`GameplayStatics.GetActorOfClass` "/Game/COMMON/ENTITIES/Characters/Character3.Character3_C"))
          (bind _output_get_5 (set `self.Character3` _returnvalue_5))
          (`/Engine/EditorBlueprintResources/StandardMacros.IsValid` _output_get_5
            (:`Is Valid`
              (bind _character3hud (`/Game/COMMON/ENTITIES/Characters/Character3.Character3HUD` _output_get_5))
              (`/Engine/EditorBlueprintResources/StandardMacros.IsValid` _character3hud
                (:`Is Valid`
                  (set `self.Character3 HUD` _character3hud)
                  (bind _outactors_3 (`GameplayStatics.GetAllActorsWithTag` "Wave1"))
                  (bind _output_get_6 (set `self.Wave1Enemies` _outactors_3))
                  (`TextBlock.SetText` (`/Game/CLIENT/RENDERING/Widget/Character1HUD.NumberOfEnemies` (`self.Character 1HUD`)) (`KismetTextLibrary.Conv_IntToText` (`KismetArrayLibrary.Array_Length` _output_get_6)))
                  (`/Engine/EditorBlueprintResources/StandardMacros.IsValid` _character_1hud_3
                    (:`Is Valid`
                      (`Widget.SetVisibility` (`/Game/CLIENT/RENDERING/Widget/Character1HUD.NumberOfEnemies` _character_1hud_3) "Visible")
                      (`Widget.SetVisibility` (`/Game/CLIENT/RENDERING/Widget/Character1HUD.EnemiesToKill_Text` _character_1hud_3) "Visible")
                      (bind _returnvalue_6 (`KismetSystemLibrary.K2_SetTimerDelegate` (delegate `EnemyWave_Character3`) 2.0 true))
                      (set `self.EnemyWave_TimeHandle` _returnvalue_6))))))))
        (:`then_3`
          (bind _returnvalue_7 (`GameplayStatics.GetActorOfClass` "/Game/COMMON/ENTITIES/Characters/Character4.Character4_C"))
          (bind _output_get_7 (set `self.Character4` _returnvalue_7))
          (`/Engine/EditorBlueprintResources/StandardMacros.IsValid` (`/Game/COMMON/ENTITIES/Characters/Character4.Character4HUD` _output_get_7)
            (:`Is Valid`
              (bind _outactors_4 (`GameplayStatics.GetAllActorsWithTag` "Wave1"))
              (bind _output_get_8 (set `self.Wave1Enemies` _outactors_4))
              (`TextBlock.SetText` (`/Game/CLIENT/RENDERING/Widget/Character1HUD.NumberOfEnemies` (`self.Character 1HUD`)) (`KismetTextLibrary.Conv_IntToText` (`KismetArrayLibrary.Array_Length` _output_get_8)))
              (`/Engine/EditorBlueprintResources/StandardMacros.IsValid` _character_1hud_4
                (:`Is Valid`
                  (`Widget.SetVisibility` (`/Game/CLIENT/RENDERING/Widget/Character1HUD.NumberOfEnemies` _character_1hud_4) "Visible")
                  (`Widget.SetVisibility` (`/Game/CLIENT/RENDERING/Widget/Character1HUD.EnemiesToKill_Text` _character_1hud_4) "Visible")
                  (bind _returnvalue_8 (`KismetSystemLibrary.K2_SetTimerDelegate` (delegate `EnemyWave_Character4`) 2.0 true))
                  (set `self.EnemyWave_TimeHandle` _returnvalue_8))))))))))

(event `EnemyWave_Character1`
  (bind _character_1hud (`self.Character 1HUD`))
  (bind _outactors (`GameplayStatics.GetAllActorsWithTag` "Wave1"))
  (bind _output_get (set `self.Wave1Enemies` _outactors))
  (`TextBlock.SetText` (`/Game/CLIENT/RENDERING/Widget/Character1HUD.NumberOfEnemies` (`self.Character 1HUD`)) (`KismetTextLibrary.Conv_IntToText` (`KismetArrayLibrary.Array_Length` _output_get)))
  (if (`KismetArrayLibrary.Array_IsEmpty` _output_get)
    (set `self.IsNoEnemies?` false)
    (bind _returnvalue (`GameplayStatics.GetActorOfClass` "/Game/COMMON/PUZZLES/BP_EnemyWaveTrigger.BP_EnemyWaveTrigger_C"))
    (`/Game/COMMON/PUZZLES/BP_EnemyWaveTrigger.OpenDoor` _returnvalue)
    (bind _returnvalue_2 (`GameplayStatics.GetActorOfClass` "/Game/COMMON/PUZZLES/BP_Door.BP_Door_C"))
    (`/Game/COMMON/PUZZLES/BP_Door.OpenDoor` _returnvalue_2)
    (bind _returnvalue_3 (`GameplayStatics.GetActorOfClass` "/Game/COMMON/ENTITIES/Doors/BPDoor2.BPDoor2_C"))
    (`/Game/COMMON/ENTITIES/Doors/BPDoor2.OpenDoor` _returnvalue_3)
    (bind _returnvalue_4 (`GameplayStatics.GetActorOfClass` "/Game/COMMON/ENTITIES/Doors/BPDoor3.BPDoor3_C"))
    (`/Game/COMMON/ENTITIES/Doors/BPDoor3.OpenDoor` _returnvalue_4)
    (`Widget.SetVisibility` (`/Game/CLIENT/RENDERING/Widget/Character1HUD.NumberOfEnemies` _character_1hud) "Hidden")
    (`Widget.SetVisibility` (`/Game/CLIENT/RENDERING/Widget/Character1HUD.EnemiesToKill_Text` _character_1hud) "Hidden")
    (`KismetSystemLibrary.K2_ClearAndInvalidateTimerHandle` (`self.EnemyWave_TimeHandle`))))

(event `EnemyWave_Character2`
  (bind _character_1hud (`self.Character 1HUD`))
  (bind _outactors (`GameplayStatics.GetAllActorsWithTag` "Wave1"))
  (bind _output_get (set `self.Wave1Enemies` _outactors))
  (`TextBlock.SetText` (`/Game/CLIENT/RENDERING/Widget/Character1HUD.NumberOfEnemies` (`self.Character 1HUD`)) (`KismetTextLibrary.Conv_IntToText` (`KismetArrayLibrary.Array_Length` _output_get)))
  (if (`KismetArrayLibrary.Array_IsEmpty` _output_get)
    (set `self.IsNoEnemies?` false)
    (bind _returnvalue (`GameplayStatics.GetActorOfClass` "/Game/COMMON/PUZZLES/BP_EnemyWaveTrigger.BP_EnemyWaveTrigger_C"))
    (`/Game/COMMON/PUZZLES/BP_EnemyWaveTrigger.OpenDoor` _returnvalue)
    (bind _returnvalue_2 (`GameplayStatics.GetActorOfClass` "/Game/COMMON/PUZZLES/BP_Door.BP_Door_C"))
    (`/Game/COMMON/PUZZLES/BP_Door.OpenDoor` _returnvalue_2)
    (bind _returnvalue_3 (`GameplayStatics.GetActorOfClass` "/Game/COMMON/ENTITIES/Doors/BPDoor2.BPDoor2_C"))
    (`/Game/COMMON/ENTITIES/Doors/BPDoor2.OpenDoor` _returnvalue_3)
    (bind _returnvalue_4 (`GameplayStatics.GetActorOfClass` "/Game/COMMON/ENTITIES/Doors/BPDoor3.BPDoor3_C"))
    (`/Game/COMMON/ENTITIES/Doors/BPDoor3.OpenDoor` _returnvalue_4)
    (`Widget.SetVisibility` (`/Game/CLIENT/RENDERING/Widget/Character1HUD.NumberOfEnemies` _character_1hud) "Hidden")
    (`Widget.SetVisibility` (`/Game/CLIENT/RENDERING/Widget/Character1HUD.EnemiesToKill_Text` _character_1hud) "Hidden")
    (`KismetSystemLibrary.K2_ClearAndInvalidateTimerHandle` (`self.EnemyWave_TimeHandle`))))

(event `EnemyWave_Character3`
  (bind _character_1hud (`self.Character 1HUD`))
  (bind _outactors (`GameplayStatics.GetAllActorsWithTag` "Wave1"))
  (bind _output_get (set `self.Wave1Enemies` _outactors))
  (`TextBlock.SetText` (`/Game/CLIENT/RENDERING/Widget/Character1HUD.NumberOfEnemies` (`self.Character 1HUD`)) (`KismetTextLibrary.Conv_IntToText` (`KismetArrayLibrary.Array_Length` _output_get)))
  (if (`KismetArrayLibrary.Array_IsEmpty` _output_get)
    (set `self.IsNoEnemies?` false)
    (bind _returnvalue (`GameplayStatics.GetActorOfClass` "/Game/COMMON/PUZZLES/BP_EnemyWaveTrigger.BP_EnemyWaveTrigger_C"))
    (`/Game/COMMON/PUZZLES/BP_EnemyWaveTrigger.OpenDoor` _returnvalue)
    (bind _returnvalue_2 (`GameplayStatics.GetActorOfClass` "/Game/COMMON/PUZZLES/BP_Door.BP_Door_C"))
    (`/Game/COMMON/PUZZLES/BP_Door.OpenDoor` _returnvalue_2)
    (bind _returnvalue_3 (`GameplayStatics.GetActorOfClass` "/Game/COMMON/ENTITIES/Doors/BPDoor2.BPDoor2_C"))
    (`/Game/COMMON/ENTITIES/Doors/BPDoor2.OpenDoor` _returnvalue_3)
    (bind _returnvalue_4 (`GameplayStatics.GetActorOfClass` "/Game/COMMON/ENTITIES/Doors/BPDoor3.BPDoor3_C"))
    (`/Game/COMMON/ENTITIES/Doors/BPDoor3.OpenDoor` _returnvalue_4)
    (`Widget.SetVisibility` (`/Game/CLIENT/RENDERING/Widget/Character1HUD.NumberOfEnemies` _character_1hud) "Hidden")
    (`Widget.SetVisibility` (`/Game/CLIENT/RENDERING/Widget/Character1HUD.EnemiesToKill_Text` _character_1hud) "Hidden")
    (`KismetSystemLibrary.K2_ClearAndInvalidateTimerHandle` (`self.EnemyWave_TimeHandle`))))

(event `EnemyWave_Character4`
  (bind _character_1hud (`self.Character 1HUD`))
  (bind _outactors (`GameplayStatics.GetAllActorsWithTag` "Wave1"))
  (bind _output_get (set `self.Wave1Enemies` _outactors))
  (`TextBlock.SetText` (`/Game/CLIENT/RENDERING/Widget/Character1HUD.NumberOfEnemies` (`self.Character 1HUD`)) (`KismetTextLibrary.Conv_IntToText` (`KismetArrayLibrary.Array_Length` _output_get)))
  (if (`KismetArrayLibrary.Array_IsEmpty` _output_get)
    (set `self.IsNoEnemies?` false)
    (bind _returnvalue (`GameplayStatics.GetActorOfClass` "/Game/COMMON/PUZZLES/BP_EnemyWaveTrigger.BP_EnemyWaveTrigger_C"))
    (`/Game/COMMON/PUZZLES/BP_EnemyWaveTrigger.OpenDoor` _returnvalue)
    (bind _returnvalue_2 (`GameplayStatics.GetActorOfClass` "/Game/COMMON/PUZZLES/BP_Door.BP_Door_C"))
    (`/Game/COMMON/PUZZLES/BP_Door.OpenDoor` _returnvalue_2)
    (bind _returnvalue_3 (`GameplayStatics.GetActorOfClass` "/Game/COMMON/ENTITIES/Doors/BPDoor2.BPDoor2_C"))
    (`/Game/COMMON/ENTITIES/Doors/BPDoor2.OpenDoor` _returnvalue_3)
    (bind _returnvalue_4 (`GameplayStatics.GetActorOfClass` "/Game/COMMON/ENTITIES/Doors/BPDoor3.BPDoor3_C"))
    (`/Game/COMMON/ENTITIES/Doors/BPDoor3.OpenDoor` _returnvalue_4)
    (`Widget.SetVisibility` (`/Game/CLIENT/RENDERING/Widget/Character1HUD.NumberOfEnemies` _character_1hud) "Hidden")
    (`Widget.SetVisibility` (`/Game/CLIENT/RENDERING/Widget/Character1HUD.EnemiesToKill_Text` _character_1hud) "Hidden")
    (`KismetSystemLibrary.K2_ClearAndInvalidateTimerHandle` (`self.EnemyWave_TimeHandle`))))

(fn `UserConstructionScript`)
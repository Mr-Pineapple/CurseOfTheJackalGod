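; BP_HealingAbility is a spawned area-heal ability that boosts playable characters' health on BeginPlay.
; It spawns a healing Niagara effect beneath itself, but centres its sphere overlap on the first Character1 found.
; A cast chain adds a fixed, unclamped amount to Character1–3 in range and refreshes each HUD bar.
; Character4 only gets the raised value sent to its HUD; its Health is never written.
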(event `self.ReceiveBeginPlay`
  (`NiagaraFunctionLibrary.SpawnSystemAtLocation` "/Game/CLIENT/UTILITIES/VFX/HealingVFX/NS_HealingAOE.NS_HealingAOE" (- (`self.K2_GetActorLocation`) (0.0 0.0 100.0)) (struct) (3.0 3.0 3.0))
  (bind _returnvalue (`GameplayStatics.GetActorOfClass` "/Game/COMMON/ENTITIES/Characters/Character1.Character1_C"))
  (`/Engine/EditorBlueprintResources/StandardMacros.IsValid` _returnvalue
    (:`Is Valid`
      (bind _outactors (`KismetSystemLibrary.SphereOverlapActors` (`self.K2_GetActorLocation` _returnvalue) 500.0 (`self.Object Type`) null (`|MakeArray` self :!type "Actor Object Reference")))
      (for _array_element _outactors
        (bind _ascharacter_1 (cast `/Game/COMMON/ENTITIES/Characters/Character1` _array_element)
          (:`then`
            (`/Engine/EditorBlueprintResources/StandardMacros.IsValid` _ascharacter_1
              (:`Is Valid`
                (bind _output_get (set `/Game/COMMON/ENTITIES/Characters/Character1.Health` (+ (`/Game/COMMON/ENTITIES/Characters/Character1.Health` _ascharacter_1) 50.0) _ascharacter_1))
                (`/Game/CLIENT/RENDERING/Widget/Character1HUD.UpdateHealthBar` (`/Game/COMMON/ENTITIES/Characters/Character1.Character1HUD` _ascharacter_1) _output_get))))
          (:`CastFailed`
            (bind _ascharacter_2 (cast `/Game/COMMON/ENTITIES/Characters/Character2` _array_element)
              (:`then`
                (`/Engine/EditorBlueprintResources/StandardMacros.IsValid` _ascharacter_2
                  (:`Is Valid`
                    (bind _output_get_2 (set `/Game/COMMON/ENTITIES/Characters/Character2.Health` (+ (`/Game/COMMON/ENTITIES/Characters/Character2.Health` _ascharacter_2) 50.0) _ascharacter_2))
                    (`/Game/CLIENT/RENDERING/Widget/Character2HUD.UpdateHealthBar` (`/Game/COMMON/ENTITIES/Characters/Character2.CharacterHUD2` _ascharacter_2) _output_get_2))))
              (:`CastFailed`
                (bind _ascharacter_3 (cast `/Game/COMMON/ENTITIES/Characters/Character3` _array_element)
                  (:`then`
                    (`/Engine/EditorBlueprintResources/StandardMacros.IsValid` _ascharacter_3
                      (:`Is Valid`
                        (bind _output_get_3 (set `/Game/COMMON/ENTITIES/Characters/Character3.Health` (+ (`/Game/COMMON/ENTITIES/Characters/Character3.Health` _ascharacter_3) 50.0) _ascharacter_3))
                        (`/Game/CLIENT/RENDERING/Widget/Character3HUD.UpdateHealthBar` (`/Game/COMMON/ENTITIES/Characters/Character3.Character3HUD` _ascharacter_3) _output_get_3))))
                  (:`CastFailed`
                    (bind _ascharacter_4 (cast `/Game/COMMON/ENTITIES/Characters/Character4` _array_element))
                    (`/Engine/EditorBlueprintResources/StandardMacros.IsValid` _ascharacter_4
                      (:`Is Valid`
                        (`/Game/CLIENT/RENDERING/Widget/Character4HUD.UpdateHealthBar` (`/Game/COMMON/ENTITIES/Characters/Character4.Character4HUD` _ascharacter_4) (+ (`/Game/COMMON/ENTITIES/Characters/Character4.Health` _ascharacter_4) 50.0))))))))))))))

(fn `UserConstructionScript`)
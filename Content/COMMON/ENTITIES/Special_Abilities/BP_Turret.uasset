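; Automated turret that uses pawn sensing to track and shoot guards, AI demo characters and enemy bosses.
; OnSeePawn caches the target by type and raises CanSeeEnemy for roughly one sensing interval.
; Tick keeps the stand fixed while interpolating actor yaw toward each cached target, snapping faster onto bosses.
; Each target branch spawns a projectile from the head socket with a sound, throttled by a DoOnce and one-second Delay.
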(event `self.ReceiveTick`
  (params (DeltaSeconds :type "Float (single-precision)"))
  (bind (_returnvalue_roll _returnvalue_pitch) (`KismetMathLibrary.BreakRotator` (`self.K2_GetActorRotation`)))
  (bind (_returnvalue_roll_2 _returnvalue_pitch_2) (`KismetMathLibrary.BreakRotator` (`self.K2_GetActorRotation`)))
  (bind (_returnvalue_roll_3 _returnvalue_pitch_3) (`KismetMathLibrary.BreakRotator` (`self.K2_GetActorRotation`)))
  (bind _head (`self.Head`))
  (bind _bp_enemy_boss (`self.BP Enemy Boss`))
  (bind _head_2 (`self.Head`))
  (bind _bp_ai_demo_character (`self.BP AI Demo Character`))
  (bind _bp_guard (`self.BP Guard`))
  (bind _head_3 (`self.Head`))
  (bind (_returnvalue_roll_4 _returnvalue_pitch_4 _returnvalue_yaw) (`KismetMathLibrary.BreakRotator` (`KismetMathLibrary.FindLookAtRotation` (`self.K2_GetActorLocation`) (`self.K2_GetActorLocation` _bp_enemy_boss))))
  (bind (_returnvalue_roll_5 _returnvalue_pitch_5 _returnvalue_yaw_2) (`KismetMathLibrary.BreakRotator` (`KismetMathLibrary.FindLookAtRotation` (`self.K2_GetActorLocation`) (`self.K2_GetActorLocation` _bp_guard))))
  (bind (_returnvalue_roll_6 _returnvalue_pitch_6 _returnvalue_yaw_3) (`KismetMathLibrary.BreakRotator` (`KismetMathLibrary.FindLookAtRotation` (`self.K2_GetActorLocation`) (`self.K2_GetActorLocation` _bp_ai_demo_character))))
  (`SceneComponent.K2_SetWorldRotation` :`self` (`self.Stand`) :!label _label)
  (`|ExecutionSequence`
    (:`then_0`
      (`/Engine/EditorBlueprintResources/StandardMacros.IsValid` _bp_guard
        (:`Is Valid`
          (if (`self.CanSeeEnemy?`)
            (`self.K2_SetActorRotation` (`KismetMathLibrary.RInterpTo` (`self.K2_GetActorRotation`) (`KismetMathLibrary.MakeRotator` _returnvalue_roll_3 _returnvalue_pitch_3 _returnvalue_yaw_2) (`GameplayStatics.GetWorldDeltaSeconds`) 10.0))
            (`/Engine/EditorBlueprintResources/StandardMacros.DoOnce` false :!label _label_2
              (:`Completed`
                (`|ExecutionSequence`
                  (:`then_0`
                    (`GameplayStatics.PlaySoundAtLocation` "/Game/CLIENT/SOUNDCUES/Explosion01.Explosion01" (0.0 0.0 0.0) (struct) 1.0 1.0 0.0 null null null null)
                    (`|SpawnActorFromClass` "/Game/COMMON/ENTITIES/Projectiles/Turret/BP_TurretProjectile.BP_TurretProjectile_C" (`KismetMathLibrary.MakeTransform` (`SceneComponent.GetSocketLocation` _head_2 "TurretSocket") (`SceneComponent.K2_GetComponentRotation` _head_2)) "AlwaysSpawn" "MultiplyWithRoot" null null))
                  (:`then_1`
                    (`KismetSystemLibrary.Delay` 1.0)
                    (goto _label_2 :!via `Reset`)))))))))
    (:`then_1`
      (`/Engine/EditorBlueprintResources/StandardMacros.IsValid` _bp_ai_demo_character
        (:`Is Valid`
          (if (`self.CanSeeEnemy?`)
            (`self.K2_SetActorRotation` (`KismetMathLibrary.RInterpTo` (`self.K2_GetActorRotation`) (`KismetMathLibrary.MakeRotator` _returnvalue_roll_2 _returnvalue_pitch_2 _returnvalue_yaw_3) (`GameplayStatics.GetWorldDeltaSeconds`) 10.0))
            (`/Engine/EditorBlueprintResources/StandardMacros.DoOnce` false :!label _label_3
              (:`Completed`
                (`|ExecutionSequence`
                  (:`then_0`
                    (`GameplayStatics.PlaySoundAtLocation` "/Game/CLIENT/SOUNDCUES/Explosion01.Explosion01" (0.0 0.0 0.0) (struct) 1.0 1.0 0.0 null null null null)
                    (`|SpawnActorFromClass` "/Game/COMMON/ENTITIES/Projectiles/Turret/BP_TurretProjectile.BP_TurretProjectile_C" (`KismetMathLibrary.MakeTransform` (`SceneComponent.GetSocketLocation` _head "TurretSocket") (`SceneComponent.K2_GetComponentRotation` _head)) "AlwaysSpawn" "MultiplyWithRoot" null null))
                  (:`then_1`
                    (`KismetSystemLibrary.Delay` 1.0)
                    (goto _label_3 :!via `Reset`)))))))))
    (:`then_2`
      (`/Engine/EditorBlueprintResources/StandardMacros.IsValid` _bp_enemy_boss
        (:`Is Valid`
          (if (`self.CanSeeEnemy?`)
            (`self.K2_SetActorRotation` (`KismetMathLibrary.RInterpTo` (`self.K2_GetActorRotation`) (`KismetMathLibrary.MakeRotator` _returnvalue_roll _returnvalue_pitch _returnvalue_yaw) (`GameplayStatics.GetWorldDeltaSeconds`) 100.0))
            (`/Engine/EditorBlueprintResources/StandardMacros.DoOnce` false :!label _label_4
              (:`Completed`
                (`|ExecutionSequence`
                  (:`then_0`
                    (`GameplayStatics.PlaySoundAtLocation` "/Game/CLIENT/SOUNDCUES/Explosion01.Explosion01" (0.0 0.0 0.0) (struct) 1.0 1.0 0.0 null null null null)
                    (`|SpawnActorFromClass` "/Game/COMMON/ENTITIES/Projectiles/Turret/BP_TurretProjectile.BP_TurretProjectile_C" (`KismetMathLibrary.MakeTransform` (`SceneComponent.GetSocketLocation` _head_3 "TurretSocket") (`SceneComponent.K2_GetComponentRotation` _head_3)) "AlwaysSpawn" "MultiplyWithRoot" null null))
                  (:`then_1`
                    (`KismetSystemLibrary.Delay` 1.0)
                    (goto _label_4 :!via `Reset`)))))))))))

(event `self.ReceiveBeginPlay`
  (`|ExecutionSequence`
    (:`then_0`
      (goto _label))
    (:`then_1`
      (`|ExecutionSequence` :!label _label_5
        (:`then_0`
          (bind _asbp_ai_demo_character (cast `/Game/COMMON/COMPONENTS/AI_Component/Demo/DemoAi/BP_AI_DemoCharacter` (stale `self.PawnSensing.OnSeePawn` Pawn)))
          (set `self.BP AI Demo Character` _asbp_ai_demo_character))
        (:`then_1`
          (bind _asbp_guard (cast `/Game/COMMON/ENTITIES/AI/AI_Guard/BP_Guard` (stale `self.PawnSensing.OnSeePawn` Pawn)))
          (set `self.BP Guard` _asbp_guard))
        (:`then_2`
          (bind _asbp_enemy_boss (cast `/Game/COMMON/ENTITIES/AI/Enemies/BossEnemy/BP_Enemy_Boss` (stale `self.PawnSensing.OnSeePawn` Pawn)))
          (set `self.BP Enemy Boss` _asbp_enemy_boss)))
      (set `self.CanSeeEnemy?` true)
      (`KismetSystemLibrary.Delay` (- (`PawnSensingComponent.SensingInterval` (`self.PawnSensing`)) (`self.GetActorTickInterval`)))
      (set `self.CanSeeEnemy?` false))))

(event `self.PawnSensing.OnSeePawn`
  (params (Pawn :type "Pawn Object Reference"))
  (goto _label_5))

(fn `UserConstructionScript`)
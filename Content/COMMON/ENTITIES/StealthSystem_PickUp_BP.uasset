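; Stealth system pickup actor that gives the player either a rock or a smoke bomb on overlap.
; When player character 0 enters its Box, it finds the first component on that character implementing PickUp_BPI.
; The SmokebombRock boolean selects which interface message is sent, rock when true and smoke bomb otherwise, then the actor destroys itself.
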(event `self.Box.OnComponentBeginOverlap`
  (params (OverlappedComponent :type "PrimitiveComponent Object Reference") (OtherActor :type "Actor Object Reference") (OtherComp :type "PrimitiveComponent Object Reference") (OtherBodyIndex :type Integer) (bFromSweep :type Boolean) (SweepResult :type "HitResult Structure (by ref)"))
  (bind _returnvalue (`GameplayStatics.GetPlayerCharacter` 0))
  (bind _output (`|GetArrayItem` (`self.GetComponentsByInterface` _returnvalue "/Game/COMMON/UTILITIES/WeaponBlueprints/PickUp_BPI.PickUp_BPI_C")))
  ;[0.1094 0.1094 0.1094] This logic adds the item to the player inventory upon overlap.
  (if (== OtherActor _returnvalue)
    (`/Engine/EditorBlueprintResources/StandardMacros.IsValid` _output
      (:`Is Valid`
        (if (`self.Smokebomb/Rock`)
          (message `/Game/COMMON/UTILITIES/WeaponBlueprints/PickUp_BPI.PickUpRock` _output)
          (else
            (message `/Game/COMMON/UTILITIES/WeaponBlueprints/PickUp_BPI.PickUpSmokeBomb` _output)))
        (`self.K2_DestroyActor`)))))

(fn `UserConstructionScript`)
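; Checkpoint actor that updates a player character's respawn location when that character enters it.
; Overlapping the Trigger component starts a chain of casts to the four character classes, Character1 through Character4.
; The first matching character gets its SpawnTransform set to the world transform of the SpawnPosition component, and other actors are ignored.
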(event `self.Trigger.OnComponentBeginOverlap`
  (params (OverlappedComponent :type "PrimitiveComponent Object Reference") (OtherActor :type "Actor Object Reference") (OtherComp :type "PrimitiveComponent Object Reference") (OtherBodyIndex :type Integer) (bFromSweep :type Boolean) (SweepResult :type "HitResult Structure (by ref)"))
  (bind _ascharacter_1 (cast `/Game/COMMON/ENTITIES/Characters/Character1` OtherActor)
    (:`then`
      (set `/Game/COMMON/ENTITIES/Characters/Character1.SpawnTransform` (`SceneComponent.K2_GetComponentToWorld` (`self.SpawnPosition`)) _ascharacter_1))
    (:`CastFailed`
      (bind _ascharacter_2 (cast `/Game/COMMON/ENTITIES/Characters/Character2` OtherActor)
        (:`then`
          (set `/Game/COMMON/ENTITIES/Characters/Character2.SpawnTransform` (`SceneComponent.K2_GetComponentToWorld` (`self.SpawnPosition`)) _ascharacter_2))
        (:`CastFailed`
          (bind _ascharacter_3 (cast `/Game/COMMON/ENTITIES/Characters/Character3` OtherActor)
            (:`then`
              (set `/Game/COMMON/ENTITIES/Characters/Character3.SpawnTransform` (`SceneComponent.K2_GetComponentToWorld` (`self.SpawnPosition`)) _ascharacter_3))
            (:`CastFailed`
              (bind _ascharacter_4 (cast `/Game/COMMON/ENTITIES/Characters/Character4` OtherActor))
              (set `/Game/COMMON/ENTITIES/Characters/Character4.SpawnTransform` (`SceneComponent.K2_GetComponentToWorld` (`self.SpawnPosition`)) _ascharacter_4))))))))

(fn `UserConstructionScript`)
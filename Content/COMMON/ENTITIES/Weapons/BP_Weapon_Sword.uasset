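; Sword weapon Blueprint that animates an effect component moving along its vertical axis.
; On BeginPlay it runs the parent logic, then starts a timeline whose Z track sets the relative location of MoveEffect.
; The timeline's Finished output calls the same custom event again, so the motion repeats endlessly without using Tick.
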(event `self.ReceiveBeginPlay`
  (`parent.ReceiveBeginPlay`)
  (`self.MoveEffectUpAndDown`))

(event `MoveEffectUpAndDown`
  (bind (_direction _zlocation) (`Timeline|MoveEffectTimeline` :!via `PlayFromStart`)
    (:`Update`
      (`SceneComponent.K2_SetRelativeLocation` (`self.MoveEffect`) (`KismetMathLibrary.MakeVector` 0.0 0.0 _zlocation) false false))
    (:`Finished`
      (`self.MoveEffectUpAndDown`))))

(fn `UserConstructionScript`
  (`parent.UserConstructionScript`))
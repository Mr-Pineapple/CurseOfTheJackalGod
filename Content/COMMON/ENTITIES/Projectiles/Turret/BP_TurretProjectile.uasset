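; Turret projectile that damages enemies on overlap and expires after a short lifespan set at BeginPlay.
; Sphere overlap casts to demo AI, guard or boss, then triggers damage VFX and applies damage credited to player 0.
; Guards and bosses also get their movement disabled; bosses destroy the projectile immediately, while guards delay destruction beyond its lifespan.
; Explosion, Environment-tag handling and the demo AI's movement disable sit in unreachable logic.
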(event `self.ReceiveBeginPlay`
  (`self.SetLifeSpan` 2.0))

(event `self.Sphere1.OnComponentBeginOverlap`
  (params (OverlappedComponent :type "PrimitiveComponent Object Reference") (OtherActor :type "Actor Object Reference") (OtherComp :type "PrimitiveComponent Object Reference") (OtherBodyIndex :type Integer) (bFromSweep :type Boolean) (SweepResult :type "HitResult Structure (by ref)"))
  (bind _bp_enemy_boss (`self.BP Enemy Boss`))
  (bind _bp_guard (`self.BP Guard`))
  (bind _bp_enemy_boss_2 (`self.BP Enemy Boss`))
  (bind _bp_enemy_boss_3 (`self.BP Enemy Boss`))
  (`|ExecutionSequence`
    (:`then_0`
      (bind _asbp_ai_demo_character (cast `/Game/COMMON/COMPONENTS/AI_Component/Demo/DemoAi/BP_AI_DemoCharacter` OtherActor)
        (:`then`
          (`/Engine/EditorBlueprintResources/StandardMacros.IsValid` _asbp_ai_demo_character
            (:`Is Valid`
              (`/Game/COMMON/COMPONENTS/AI_Component/Demo/DemoAi/BP_AI_DemoCharacter.VFXDamage` _asbp_ai_demo_character "NewEnumerator1")
              (`/Engine/EditorBlueprintResources/StandardMacros.IsValid` _asbp_ai_demo_character
                (:`Is Valid`
                  (`GameplayStatics.ApplyDamage` _asbp_ai_demo_character 20.0 (`GameplayStatics.GetPlayerController` 0) self "/Script/Engine.DamageType")
                  (`KismetSystemLibrary.PrintString` "Hello"))))))
        (:`CastFailed`
          (bind _asbp_guard (cast `/Game/COMMON/ENTITIES/AI/AI_Guard/BP_Guard` OtherActor)
            (:`then`
              (bind _output_get (set `self.BP Guard` _asbp_guard))
              (`/Engine/EditorBlueprintResources/StandardMacros.IsValid` _output_get
                (:`Is Valid`
                  (`/Game/COMMON/ENTITIES/AI/AI_Guard/BP_Guard.VFXDamage` _output_get "NewEnumerator1")
                  (`/Engine/EditorBlueprintResources/StandardMacros.IsValid` _output_get
                    (:`Is Valid`
                      (`GameplayStatics.ApplyDamage` _output_get 10.0 (`GameplayStatics.GetPlayerController` 0) self "/Script/Engine.DamageType")
                      (`/Engine/EditorBlueprintResources/StandardMacros.IsValid` _bp_guard
                        (:`Is Valid`
                          (`/Game/COMMON/ENTITIES/AI/AI_Guard/BP_Guard.Disable Enemy Movement Over Time` _bp_guard)
                          (`KismetSystemLibrary.Delay` 5.0)
                          (`self.K2_DestroyActor`))))))))
            (:`CastFailed`
              (bind _asbp_enemy_boss (cast `/Game/COMMON/ENTITIES/AI/Enemies/BossEnemy/BP_Enemy_Boss` OtherActor))
              (set `self.BP Enemy Boss` _asbp_enemy_boss)
              (`/Engine/EditorBlueprintResources/StandardMacros.IsValid` _bp_enemy_boss
                (:`Is Valid`
                  (`/Game/COMMON/ENTITIES/AI/Enemies/BossEnemy/BP_Enemy_Boss.VFXDamage` _bp_enemy_boss "NewEnumerator1")
                  (`/Engine/EditorBlueprintResources/StandardMacros.IsValid` _bp_enemy_boss_3
                    (:`Is Valid`
                      (`GameplayStatics.ApplyDamage` _bp_enemy_boss_3 20.0 (`GameplayStatics.GetPlayerController` 0) self "/Script/Engine.DamageType")
                      (`/Engine/EditorBlueprintResources/StandardMacros.IsValid` _bp_enemy_boss_2
                        (:`Is Valid`
                          (`/Game/COMMON/ENTITIES/AI/Enemies/BossEnemy/BP_Enemy_Boss.Disable Enemy Movement Over Time` _bp_enemy_boss_2)
                          (`self.K2_DestroyActor`))))))))))))))

(fn `UserConstructionScript`)
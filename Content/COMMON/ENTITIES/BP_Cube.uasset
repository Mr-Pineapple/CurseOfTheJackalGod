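; BP_Cube is an interactable box that Character1 can engage with and that can be moved along its own axes.
; Four Fwd trigger components set the character's CanInteractBox flag on overlap, then clear both interaction flags and reset walk speed on exit, with debug prints.
; Speed/Direction eases SMCube's relative location with VInterpTo along its right or forward vector, chosen by a boolean and scaled by DirectionSpeed.
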(event `self.Fwd.OnComponentBeginOverlap`
  (params (OverlappedComponent :type "PrimitiveComponent Object Reference") (OtherActor :type "Actor Object Reference") (OtherComp :type "PrimitiveComponent Object Reference") (OtherBodyIndex :type Integer) (bFromSweep :type Boolean) (SweepResult :type "HitResult Structure (by ref)"))
  (bind _ascharacter_1 (cast `/Game/COMMON/ENTITIES/Character1` OtherActor))
  (`KismetSystemLibrary.PrintString` "Character Can Interact " true true (struct :`R` 0.001298 :`G` 1.0 :`A` 1.0) 2.0 "432342")
  (`/Engine/EditorBlueprintResources/StandardMacros.IsValid` _ascharacter_1
    (:`Is Valid`
      (set `/Game/COMMON/ENTITIES/Character1.CanInteractBox?` true _ascharacter_1))
    (:`Is Not Valid`
      (`KismetSystemLibrary.PrintString` "Hello"))))

(event `self.Fwd.OnComponentEndOverlap`
  (params (OverlappedComponent :type "PrimitiveComponent Object Reference") (OtherActor :type "Actor Object Reference") (OtherComp :type "PrimitiveComponent Object Reference") (OtherBodyIndex :type Integer))
  (bind _ascharacter_1 (cast `/Game/COMMON/ENTITIES/Character1` OtherActor))
  (`KismetSystemLibrary.PrintString` "Character Cannot Interact " true true (struct :`R` 1.0 :`B` 0.035135 :`A` 1.0) 2.0 "3423423423")
  (`/Engine/EditorBlueprintResources/StandardMacros.IsValid` _ascharacter_1
    (:`Is Valid`
      (set `/Game/COMMON/ENTITIES/Character1.CanInteractBox?` false _ascharacter_1)
      (set `/Game/COMMON/ENTITIES/Character1.IsInteractingBox?` false _ascharacter_1)
      (set `CharacterMovementComponent.MaxWalkSpeed` 400.0 (`Character.CharacterMovement` _ascharacter_1)))))

(event `self.Fwd1.OnComponentBeginOverlap`
  (params (OverlappedComponent :type "PrimitiveComponent Object Reference") (OtherActor :type "Actor Object Reference") (OtherComp :type "PrimitiveComponent Object Reference") (OtherBodyIndex :type Integer) (bFromSweep :type Boolean) (SweepResult :type "HitResult Structure (by ref)"))
  (bind _ascharacter_1 (cast `/Game/COMMON/ENTITIES/Character1` OtherActor))
  (`KismetSystemLibrary.PrintString` "Character Can Interact " true true (struct :`R` 0.001298 :`G` 1.0 :`A` 1.0) 2.0 "432342")
  (`/Engine/EditorBlueprintResources/StandardMacros.IsValid` _ascharacter_1
    (:`Is Valid`
      (set `/Game/COMMON/ENTITIES/Character1.CanInteractBox?` true _ascharacter_1))
    (:`Is Not Valid`
      (`KismetSystemLibrary.PrintString` "Hello"))))

(event `self.Fwd1.OnComponentEndOverlap`
  (params (OverlappedComponent :type "PrimitiveComponent Object Reference") (OtherActor :type "Actor Object Reference") (OtherComp :type "PrimitiveComponent Object Reference") (OtherBodyIndex :type Integer))
  (bind _ascharacter_1 (cast `/Game/COMMON/ENTITIES/Character1` OtherActor))
  (`KismetSystemLibrary.PrintString` "Character Cannot Interact " true true (struct :`R` 1.0 :`B` 0.035135 :`A` 1.0) 2.0 "3423423423")
  (`/Engine/EditorBlueprintResources/StandardMacros.IsValid` _ascharacter_1
    (:`Is Valid`
      (set `/Game/COMMON/ENTITIES/Character1.CanInteractBox?` false _ascharacter_1)
      (set `/Game/COMMON/ENTITIES/Character1.IsInteractingBox?` false _ascharacter_1)
      (set `CharacterMovementComponent.MaxWalkSpeed` 400.0 (`Character.CharacterMovement` _ascharacter_1)))))

(event `self.Fwd2.OnComponentBeginOverlap`
  (params (OverlappedComponent :type "PrimitiveComponent Object Reference") (OtherActor :type "Actor Object Reference") (OtherComp :type "PrimitiveComponent Object Reference") (OtherBodyIndex :type Integer) (bFromSweep :type Boolean) (SweepResult :type "HitResult Structure (by ref)"))
  (bind _ascharacter_1 (cast `/Game/COMMON/ENTITIES/Character1` OtherActor))
  (`KismetSystemLibrary.PrintString` "Character Can Interact " true true (struct :`R` 0.001298 :`G` 1.0 :`A` 1.0) 2.0 "432342")
  (`/Engine/EditorBlueprintResources/StandardMacros.IsValid` _ascharacter_1
    (:`Is Valid`
      (set `/Game/COMMON/ENTITIES/Character1.CanInteractBox?` true _ascharacter_1))
    (:`Is Not Valid`
      (`KismetSystemLibrary.PrintString` "Hello"))))

(event `self.Fwd2.OnComponentEndOverlap`
  (params (OverlappedComponent :type "PrimitiveComponent Object Reference") (OtherActor :type "Actor Object Reference") (OtherComp :type "PrimitiveComponent Object Reference") (OtherBodyIndex :type Integer))
  (bind _ascharacter_1 (cast `/Game/COMMON/ENTITIES/Character1` OtherActor))
  (`KismetSystemLibrary.PrintString` "Character Cannot Interact " true true (struct :`R` 1.0 :`B` 0.035135 :`A` 1.0) 2.0 "3423423423")
  (`/Engine/EditorBlueprintResources/StandardMacros.IsValid` _ascharacter_1
    (:`Is Valid`
      (set `/Game/COMMON/ENTITIES/Character1.CanInteractBox?` false _ascharacter_1)
      (set `/Game/COMMON/ENTITIES/Character1.IsInteractingBox?` false _ascharacter_1)
      (set `CharacterMovementComponent.MaxWalkSpeed` 400.0 (`Character.CharacterMovement` _ascharacter_1)))))

(event `self.Fwd3.OnComponentBeginOverlap`
  (params (OverlappedComponent :type "PrimitiveComponent Object Reference") (OtherActor :type "Actor Object Reference") (OtherComp :type "PrimitiveComponent Object Reference") (OtherBodyIndex :type Integer) (bFromSweep :type Boolean) (SweepResult :type "HitResult Structure (by ref)"))
  (bind _ascharacter_1 (cast `/Game/COMMON/ENTITIES/Character1` OtherActor))
  (`KismetSystemLibrary.PrintString` "Character Can Interact " true true (struct :`R` 0.001298 :`G` 1.0 :`A` 1.0) 2.0 "432342")
  (`/Engine/EditorBlueprintResources/StandardMacros.IsValid` _ascharacter_1
    (:`Is Valid`
      (set `/Game/COMMON/ENTITIES/Character1.CanInteractBox?` true _ascharacter_1))
    (:`Is Not Valid`
      (`KismetSystemLibrary.PrintString` "Hello"))))

(event `self.Fwd3.OnComponentEndOverlap`
  (params (OverlappedComponent :type "PrimitiveComponent Object Reference") (OtherActor :type "Actor Object Reference") (OtherComp :type "PrimitiveComponent Object Reference") (OtherBodyIndex :type Integer))
  (bind _ascharacter_1 (cast `/Game/COMMON/ENTITIES/Character1` OtherActor))
  (`KismetSystemLibrary.PrintString` "Character Cannot Interact " true true (struct :`R` 1.0 :`B` 0.035135 :`A` 1.0) 2.0 "3423423423")
  (`/Engine/EditorBlueprintResources/StandardMacros.IsValid` _ascharacter_1
    (:`Is Valid`
      (set `/Game/COMMON/ENTITIES/Character1.CanInteractBox?` false _ascharacter_1)
      (set `/Game/COMMON/ENTITIES/Character1.IsInteractingBox?` false _ascharacter_1)
      (set `CharacterMovementComponent.MaxWalkSpeed` 400.0 (`Character.CharacterMovement` _ascharacter_1)))))

(fn `UserConstructionScript`)
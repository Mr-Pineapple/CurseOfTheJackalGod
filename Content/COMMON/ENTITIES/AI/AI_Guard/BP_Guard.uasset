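; Targetable AI guard enemy with a modular body, random melee montages that sphere-trace to damage four player classes, and health bar widgets.
; AnyDamage branches on causer class (players, rock, turret projectile), with player and rock kills clearing lock-on and updating special bars.
; Looping timers share one counter for elemental damage-over-time with VFX and an ice freeze that disables movement.
; Most combat query functions, including TakeDamage and Heal, are stubs.
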(event `Launch Character`
  (`self.LaunchCharacter` (`KismetMathLibrary.MakeVector` (`KismetMathLibrary.RandomFloatInRange` 100.0 1000.0) (`KismetMathLibrary.RandomFloatInRange` 100.0 1000.0) (`KismetMathLibrary.RandomFloatInRange` 100.0 500.0)) true true))

(event `/Game/COMMON/UTILITIES/Interfaces/BPI_Guard.Run`
  ;[1 1 1] Run Speed
  (set `CharacterMovementComponent.MaxWalkSpeed` 400.0 (`self.CharacterMovement`)))

(event `/Game/COMMON/UTILITIES/Interfaces/BPITargeting.OnTargeted`
  (params (`bIsTargeted?` :type Boolean))
  ;[1 1 1] Target Lockon Widget
  (`SceneComponent.SetVisibility` (`self.LockonWidget`) `bIsTargeted?` false))

(event `/Game/COMMON/UTILITIES/Interfaces/BPI_Guard.Attack`
  (bind _returnvalue (`self.K2_GetActorLocation`))
  ;[1 1 1] Attack
  (if (not (`self.is attacking`))
    (`KismetSystemLibrary.Delay` 0.2)
    (`|PlayMontage` (`self.Mesh`) (select `int` (`KismetMathLibrary.RandomInteger` 3) :`0` (`self.Montage to Play1`) :`1` (`self.Montage to Play2`) :`2` (`self.MontageToPlay3`))
      (:`then`
        (set `self.is attacking` true))
      (:`OnCompleted`
        (set `self.is attacking` false))
      (:`OnNotifyBegin`
        (bind (_outhit _returnvalue_2) (`KismetSystemLibrary.SphereTraceSingleForObjects` _returnvalue (+ _returnvalue (* (`self.GetActorForwardVector`) 100.0)) 20.0 (`|MakeArray` "ObjectTypeQuery3" :!type "EObjectTypeQuery Enum") false (`|MakeArray` self :!type "Actor Object Reference")))
        (if _returnvalue_2
          (bind (_bblockinghit _binitialoverlap _time _distance _location _impactpoint _normal _impactnormal _physmat _hitactor) (`GameplayStatics.BreakHitResult` _outhit))
          (if (`self.ActorHasTag` _hitactor "Player")
            (bind _ascharacter_1 (cast `/Game/COMMON/ENTITIES/Characters/Character1` _hitactor)
              (:`then`
                (`GameplayStatics.ApplyDamage` _ascharacter_1 10.0 null self "/Script/Engine.DamageType"))
              (:`CastFailed`
                (bind _ascharacter_2 (cast `/Game/COMMON/ENTITIES/Characters/Character2` _hitactor)
                  (:`then`
                    (`GameplayStatics.ApplyDamage` _ascharacter_2 10.0 null self "/Script/Engine.DamageType"))
                  (:`CastFailed`
                    (bind _ascharacter_3 (cast `/Game/COMMON/ENTITIES/Characters/Character3` _hitactor)
                      (:`then`
                        (`GameplayStatics.ApplyDamage` _ascharacter_3 10.0 null self "/Script/Engine.DamageType"))
                      (:`CastFailed`
                        (bind _ascharacter_4 (cast `/Game/COMMON/ENTITIES/Characters/Character4` _hitactor))
                        (`GameplayStatics.ApplyDamage` _ascharacter_4 10.0 null self "/Script/Engine.DamageType")))))))))))))

(event `self.ReceiveAnyDamage`
  (params (Damage :type "Float (single-precision)") (DamageType :type "DamageType Object Reference") (InstigatedBy :type "Controller Object Reference") (DamageCauser :type "Actor Object Reference"))
  (bind _character3 (`self.Character3`))
  (bind _character_4 (`self.Character 4`))
  (bind _character3_2 (`self.Character3`))
  (bind _character_2 (`self.Character 2`))
  (bind _character_2_2 (`self.Character 2`))
  ;[1 1 1] AnyDamage Event
  (bind _ascharacter_1 (cast `/Game/COMMON/ENTITIES/Characters/Character1` DamageCauser)
    (:`then`
      (`/Engine/EditorBlueprintResources/StandardMacros.IsValid` _ascharacter_1
        (:`Is Valid`
          (bind _output_get (set `self.Health` (- (`self.Health`) Damage)))
          (bind _asw_health_bar (cast `/Game/CLIENT/UI/W_HealthBar` (`WidgetComponent.GetWidget` (`self.HealthbarWidget`))))
          (`/Game/CLIENT/UI/W_HealthBar.UpdateHealthBar` _asw_health_bar _output_get)
          (bind _asw_health_bar_2 (cast `/Game/CLIENT/UI/W_HealthBar` (`WidgetComponent.GetWidget` (`self.HealthbarWidget2`))))
          (`/Game/CLIENT/UI/W_HealthBar.UpdateHealthBar` _asw_health_bar_2 _output_get)
          (if (<= (`self.Health`) 0.0)
            (set `/Game/COMMON/ENTITIES/Characters/Character1. BP Guard` null _ascharacter_1)
            (if (`SceneComponent.IsVisible` (`self.LockonWidget`))
              (set `/Game/COMMON/ENTITIES/Characters/Character1.Guard_Lockon` false _ascharacter_1)
              (set `/Game/COMMON/ENTITIES/Characters/Character1.LockOn` false _ascharacter_1))
            (bind _output_get_2 (set `/Game/COMMON/ENTITIES/Characters/Character1.SpecialAttackAmount` (+ (`self.SpecialAddAmount`) (`/Game/COMMON/ENTITIES/Characters/Character1.SpecialAttackAmount` _ascharacter_1)) _ascharacter_1))
            (`/Game/CLIENT/RENDERING/Widget/Character1HUD.UpdateSpecialBar` (`/Game/COMMON/ENTITIES/Characters/Character1.Character1HUD` _ascharacter_1) (`KismetMathLibrary.Conv_IntToDouble` _output_get_2))
            (`self.K2_DestroyActor`)))))
    (:`CastFailed`
      (bind _ascharacter_2 (cast `/Game/COMMON/ENTITIES/Characters/Character2` DamageCauser)
        (:`then`
          (bind _output_get_3 (set `self.Character 2` _ascharacter_2))
          (`/Engine/EditorBlueprintResources/StandardMacros.IsValid` _output_get_3
            (:`Is Valid`
              (bind _output_get_4 (set `self.Health` (- (`self.Health`) Damage)))
              (bind _asw_health_bar_3 (cast `/Game/CLIENT/UI/W_HealthBar` (`WidgetComponent.GetWidget` (`self.HealthbarWidget`))))
              (`/Game/CLIENT/UI/W_HealthBar.UpdateHealthBar` _asw_health_bar_3 _output_get_4)
              (bind _asw_health_bar_4 (cast `/Game/CLIENT/UI/W_HealthBar` (`WidgetComponent.GetWidget` (`self.HealthbarWidget2`))))
              (`/Game/CLIENT/UI/W_HealthBar.UpdateHealthBar` _asw_health_bar_4 _output_get_4)
              (`AISense_Damage.ReportDamageEvent` self _character_2 0.0 (`self.K2_GetActorLocation` _character_2))
              (if (<= (`self.Health`) 0.0)
                (set `/Game/COMMON/ENTITIES/Characters/Character2. BP Guard` null _character_2_2)
                (set `/Game/COMMON/ENTITIES/Characters/Character2.Guard_Lockon` false _character_2_2)
                (set `/Game/COMMON/ENTITIES/Characters/Character2.IsStrafing?` false _character_2_2)
                (`/Game/CLIENT/RENDERING/Widget/Character2HUD.UpdateSpecialBar` (`/Game/COMMON/ENTITIES/Characters/Character2.CharacterHUD2` _character_2_2) (`KismetMathLibrary.Conv_IntToDouble` (`self.SpecialAddAmount`)))
                (`self.K2_DestroyActor`)))))
        (:`CastFailed`
          (bind _ascharacter_3 (cast `/Game/COMMON/ENTITIES/Characters/Character3` DamageCauser)
            (:`then`
              (bind _output_get_5 (set `self.Character3` _ascharacter_3))
              (`/Engine/EditorBlueprintResources/StandardMacros.IsValid` _output_get_5
                (:`Is Valid`
                  (bind _output_get_6 (set `self.Health` (- (`self.Health`) Damage)))
                  (bind _asw_health_bar_5 (cast `/Game/CLIENT/UI/W_HealthBar` (`WidgetComponent.GetWidget` (`self.HealthbarWidget`))))
                  (`/Game/CLIENT/UI/W_HealthBar.UpdateHealthBar` _asw_health_bar_5 _output_get_6)
                  (bind _asw_health_bar_6 (cast `/Game/CLIENT/UI/W_HealthBar` (`WidgetComponent.GetWidget` (`self.HealthbarWidget2`))))
                  (`/Game/CLIENT/UI/W_HealthBar.UpdateHealthBar` _asw_health_bar_6 _output_get_6)
                  (`AISense_Damage.ReportDamageEvent` self _character3_2 0.0 (`self.K2_GetActorLocation` _character3_2))
                  (if (<= (`self.Health`) 0.0)
                    (set `/Game/COMMON/ENTITIES/Characters/Character3.BP_Guard` null _character3)
                    (set `/Game/COMMON/ENTITIES/Characters/Character3.Guard_Lockon` false _character3)
                    (set `/Game/COMMON/ENTITIES/Characters/Character3.IsStrafing?` false _character3)
                    (set `/Game/COMMON/ENTITIES/Characters/Character3.LockOn` false _character3)
                    (`/Game/CLIENT/RENDERING/Widget/Character3HUD.UpdateSpecialBar` (`/Game/COMMON/ENTITIES/Characters/Character3.Character3HUD` _character3) (`KismetMathLibrary.Conv_IntToDouble` (`self.SpecialAddAmount`)))
                    (`self.K2_DestroyActor`)))))
            (:`CastFailed`
              (bind _ascharacter_4 (cast `/Game/COMMON/ENTITIES/Characters/Character4` DamageCauser)
                (:`then`
                  (bind _output_get_7 (set `self.Character 4` _ascharacter_4))
                  (`/Engine/EditorBlueprintResources/StandardMacros.IsValid` _output_get_7
                    (:`Is Valid`
                      (bind _output_get_8 (set `self.Health` (- (`self.Health`) Damage)))
                      (bind _asw_health_bar_7 (cast `/Game/CLIENT/UI/W_HealthBar` (`WidgetComponent.GetWidget` (`self.HealthbarWidget`))))
                      (`/Game/CLIENT/UI/W_HealthBar.UpdateHealthBar` _asw_health_bar_7 _output_get_8)
                      (bind _asw_health_bar_8 (cast `/Game/CLIENT/UI/W_HealthBar` (`WidgetComponent.GetWidget` (`self.HealthbarWidget2`))))
                      (`/Game/CLIENT/UI/W_HealthBar.UpdateHealthBar` _asw_health_bar_8 _output_get_8)
                      (if (<= (`self.Health`) 0.0)
                        (set `/Game/COMMON/ENTITIES/Characters/Character4. BP Guard` null _character_4)
                        (if (`SceneComponent.IsVisible` (`self.LockonWidget`))
                          (`/Game/COMMON/ENTITIES/Characters/Character4.StopTargeting` _character_4))
                        (bind _output_get_9 (set `self.SpecialAddAmount` (+ (`self.SpecialAddAmount`) (`/Game/COMMON/ENTITIES/Characters/Character4.SpecialAttackAmount` _character_4))))
                        (`/Game/CLIENT/RENDERING/Widget/Character4HUD.UpdateSpecialBar` (`/Game/COMMON/ENTITIES/Characters/Character4.Character4HUD` _character_4) (`KismetMathLibrary.Conv_IntToDouble` _output_get_9))
                        (`KismetSystemLibrary.Delay` 0.5)
                        (`self.K2_DestroyActor`)))))
                (:`CastFailed`
                  (bind _asrock_bp (cast `/Game/COMMON/UTILITIES/Pickups/Rock_BP` DamageCauser)
                    (:`then`
                      (`/Engine/EditorBlueprintResources/StandardMacros.IsValid` _asrock_bp
                        (:`Is Valid`
                          (bind _output_get_10 (set `self.Health` (- (`self.Health`) Damage)))
                          (bind _asw_health_bar_9 (cast `/Game/CLIENT/UI/W_HealthBar` (`WidgetComponent.GetWidget` (`self.HealthbarWidget`))))
                          (`/Game/CLIENT/UI/W_HealthBar.UpdateHealthBar` _asw_health_bar_9 _output_get_10)
                          (bind _asw_health_bar_10 (cast `/Game/CLIENT/UI/W_HealthBar` (`WidgetComponent.GetWidget` (`self.HealthbarWidget2`))))
                          (`/Game/CLIENT/UI/W_HealthBar.UpdateHealthBar` _asw_health_bar_10 _output_get_10)
                          (if (<= (`self.Health`) 0.0)
                            (bind _returnvalue (`GameplayStatics.GetActorOfClass` "/Game/COMMON/ENTITIES/Characters/Character3.Character3_C"))
                            (bind _output_get_11 (set `self.Character3` _returnvalue))
                            (`/Engine/EditorBlueprintResources/StandardMacros.IsValid` _output_get_11
                              (:`Is Valid`
                                (set `/Game/COMMON/ENTITIES/Characters/Character3.Guard_Lockon` false _output_get_11)
                                (set `/Game/COMMON/ENTITIES/Characters/Character3.IsStrafing?` false _output_get_11)
                                (set `/Game/COMMON/ENTITIES/Characters/Character3.LockOn` false _output_get_11)
                                (bind _output_get_12 (set `self.SpecialAddAmount` (+ (`self.SpecialAddAmount`) (`/Game/COMMON/ENTITIES/Characters/Character3.SpecialAttackAmount` _output_get_11))))
                                (`/Game/CLIENT/RENDERING/Widget/Character3HUD.UpdateSpecialBar` (`/Game/COMMON/ENTITIES/Characters/Character3.Character3HUD` _output_get_11) (`KismetMathLibrary.Conv_IntToDouble` _output_get_12))
                                (set `/Game/COMMON/COMPONENTS/BPC_Throwing.Rock_Aiming` false (`/Game/COMMON/ENTITIES/Characters/Character3.BPC_Throwing` _output_get_11))
                                (`self.K2_DestroyActor`)))))))
                    (:`CastFailed`
                      (bind _asbp_turret_projectile (cast `/Game/COMMON/ENTITIES/Projectiles/Turret/BP_TurretProjectile` DamageCauser))
                      (`/Engine/EditorBlueprintResources/StandardMacros.IsValid` _asbp_turret_projectile
                        (:`Is Valid`
                          (bind _output_get_13 (set `self.Health` (- (`self.Health`) Damage)))
                          (bind _asw_health_bar_11 (cast `/Game/CLIENT/UI/W_HealthBar` (`WidgetComponent.GetWidget` (`self.HealthbarWidget`))))
                          (`/Game/CLIENT/UI/W_HealthBar.UpdateHealthBar` _asw_health_bar_11 _output_get_13)
                          (bind _asw_health_bar_12 (cast `/Game/CLIENT/UI/W_HealthBar` (`WidgetComponent.GetWidget` (`self.HealthbarWidget2`))))
                          (`/Game/CLIENT/UI/W_HealthBar.UpdateHealthBar` _asw_health_bar_12 _output_get_13)
                          (if (<= (`self.Health`) 0.0)
                            (`self.K2_DestroyActor`)))))))))))))))

(event `Damage Over Time`
  (params (Damage :type "Float (double-precision)") (AmmoType :type "/Game/COMMON/UTILITIES/Enums/Pickups/PickupAmmoTypes Enum" :default "NewEnumerator0"))
  ;[1 1 1] Damage Over Time
  (if (<= (`self.Health`) 0.0)
    (`self.K2_DestroyActor`)
    (`KismetSystemLibrary.K2_ClearAndInvalidateTimerHandle` (`self.DamageOvertime_TimerHandle`))
    (else
      (bind _returnvalue (`KismetSystemLibrary.K2_SetTimerDelegate` (delegate `Damage Overtime`) 1.0 true))
      (set `self.DamageOvertime_TimerHandle` _returnvalue))))

(event `Damage Overtime`
  (bind _vfx_poison (`self.VFX_Poison`))
  (bind _vfx_poison_2 (`self.VFX_Poison`))
  (bind _vfx_fire (`self.VFX_Fire`))
  (bind _vfx_fire_2 (`self.VFX_Fire`))
  ;[1 1 1] Damage Over Time
  (bind _result (`/Engine/EditorBlueprintResources/StandardMacros.IncrementInt` (`self.DamageOvertimeCounter`))
    (:`  `
      (bind _output_get (set `self.DamageOvertimeCounter` _result))
      (bind _output_get_2 (set `self.Health` (- (`self.Health`) (stale `Damage Over Time` Damage))))
      (bind _asw_health_bar (cast `/Game/CLIENT/UI/W_HealthBar` (`WidgetComponent.GetWidget` (`self.HealthbarWidget`))))
      (`/Game/CLIENT/UI/W_HealthBar.UpdateHealthBar` _asw_health_bar _output_get_2)
      (bind _asw_health_bar_2 (cast `/Game/CLIENT/UI/W_HealthBar` (`WidgetComponent.GetWidget` (`self.HealthbarWidget2`))))
      (`/Game/CLIENT/UI/W_HealthBar.UpdateHealthBar` _asw_health_bar_2 _output_get_2)
      (`self.VFXDamage` (stale `Damage Over Time` AmmoType))
      (if (<= (`self.Health`) 0.0)
        (`self.K2_DestroyActor`)
        (`KismetSystemLibrary.K2_ClearAndInvalidateTimerHandle` (`self.DamageOvertime_TimerHandle`))
        (`/Engine/EditorBlueprintResources/StandardMacros.IsValid` _vfx_fire_2
          (:`Is Valid`
            (`ActorComponent.Deactivate` _vfx_fire_2)
            (`/Engine/EditorBlueprintResources/StandardMacros.IsValid` _vfx_poison_2
              (:`Is Valid`
                (`ActorComponent.Deactivate` _vfx_poison_2)))))
        (elif (>= _output_get 5)
          (`KismetSystemLibrary.K2_ClearAndInvalidateTimerHandle` (`self.DamageOvertime_TimerHandle`))
          (set `self.DamageOvertimeCounter` 0)
          (`/Engine/EditorBlueprintResources/StandardMacros.IsValid` _vfx_fire
            (:`Is Valid`
              (`ActorComponent.Deactivate` _vfx_fire)
              (`/Engine/EditorBlueprintResources/StandardMacros.IsValid` _vfx_poison
                (:`Is Valid`
                  (`ActorComponent.Deactivate` _vfx_poison))))))))))

(event `VFXDamage`
  (params (AmmoType :type "/Game/COMMON/UTILITIES/Enums/Pickups/PickupAmmoTypes Enum" :default "NewEnumerator0"))
  ;[1 1 1] VFXDamage
  (switch `/Game/COMMON/UTILITIES/Enums/Pickups/PickupAmmoTypes` AmmoType
    (:`NewEnumerator0`
      (`ActorComponent.Activate` (`self.VFX_Fire`) false))
    (:`NewEnumerator1`
      (bind _returnvalue (`GameplayStatics.SpawnEmitterAttached` "/Game/CLIENT/UTILITIES/VFX/TurretVFX/Particles/PS_Turret_Explosion.PS_Turret_Explosion" (`self.DamageVFXLocation`)))
      (set `self.IceEmitter` _returnvalue))
    (:`NewEnumerator2`
      (`GameplayStatics.SpawnEmitterAttached` "/Game/CLIENT/UTILITIES/Particles/Particles/P_Explosion.P_Explosion" (`self.DamageVFXLocation`)))
    (:`NewEnumerator3`
      (`ActorComponent.Activate` (`self.VFX_Poison`) false))
    (:`NewEnumerator4`
      (`GameplayStatics.SpawnEmitterAttached` "/Game/CLIENT/UTILITIES/Particles/PS_AssualtRifle_Impact.PS_AssualtRifle_Impact" (`self.DamageVFXLocation`)))))

(event `Disable Enemy Movement Over Time`
  ;[1 1 1] Disable Enemy Movement Over Time
  (bind _returnvalue (`|SpawnActorFromClass` "/Game/COMMON/ENTITIES/BP_IceMesh.BP_IceMesh_C" (`KismetMathLibrary.MakeTransform` (`SceneComponent.K2_GetComponentLocation` (`self.IceLocation`))) "Undefined" "MultiplyWithRoot" null null))
  (set `self.IceMesh` _returnvalue)
  (if (<= (`self.Health`) 0.0)
    (`KismetSystemLibrary.K2_ClearAndInvalidateTimerHandle` (`self.DisableMovement_TimerHandle`))
    (else
      (`CharacterMovementComponent.SetMovementMode` (`self.CharacterMovement`) "MOVE_None" 0)
      (bind _returnvalue_2 (`KismetSystemLibrary.K2_SetTimerDelegate` (delegate `Guard Enemy Ice Decrease Speed`) 1.0 true))
      (set `self.DisableMovement_TimerHandle` _returnvalue_2))))

(event `Guard Enemy Ice Decrease Speed`
  (bind _iceemitter (`self.IceEmitter`))
  (bind _iceemitter_2 (`self.IceEmitter`))
  (bind _icemesh (`self.IceMesh`))
  (bind _icemesh_2 (`self.IceMesh`))
  ;[1 1 1] Disable Enemy Movement Over Time
  (bind _result (`/Engine/EditorBlueprintResources/StandardMacros.IncrementInt` (`self.DamageOvertimeCounter`))
    (:`  `
      (bind _output_get (set `self.DamageOvertimeCounter` _result))
      (if (<= (`self.Health`) 0.0)
        (`KismetSystemLibrary.K2_ClearAndInvalidateTimerHandle` (`self.DamageOvertime_TimerHandle`))
        (`/Engine/EditorBlueprintResources/StandardMacros.IsValid` _icemesh
          (:`Is Valid`
            (`self.K2_DestroyActor` _icemesh))
          (:`Is Not Valid`
            _))
        (`/Engine/EditorBlueprintResources/StandardMacros.IsValid` _iceemitter
          (:`Is Valid`
            (`ActorComponent.Deactivate` _iceemitter))
          (:`Is Not Valid`
            _))
        (`self.K2_DestroyActor`)
        (elif (>= _output_get 5)
          (`KismetSystemLibrary.K2_ClearAndInvalidateTimerHandle` (`self.DamageOvertime_TimerHandle`))
          (set `self.DamageOvertimeCounter` 0)
          (`CharacterMovementComponent.SetMovementMode` (`self.CharacterMovement`) "MOVE_Walking" 0)
          (`/Engine/EditorBlueprintResources/StandardMacros.IsValid` _icemesh_2
            (:`Is Valid`
              (`self.K2_DestroyActor` _icemesh_2))
            (:`Is Not Valid`
              _))
          (`/Engine/EditorBlueprintResources/StandardMacros.IsValid` _iceemitter_2
            (:`Is Valid`
              (`ActorComponent.Deactivate` _iceemitter_2))))))))

(fn `CanBeTargeted`
  (returns (ReturnValue :type Boolean))
  (return (> (`self.Health`) 0.0)))

(fn `GetCharacterTargetLocation`
  (returns (ReturnValue :type "Vector Structure"))
  (return (`KismetMathLibrary.TransformLocation` (`self.GetTransform`) (`self.CharacterOffset`))))

(fn `GetCurrentHealth`
  (returns (Health :type "Float (double-precision)"))
  (return 0.0))

(fn `GetMaxHealth`
  (returns (MaxHealth :type "Float (double-precision)"))
  (return 0.0))

(fn `GetTeamNumber`
  (returns (TeamNumber :type Integer))
  (return 2))

(fn `Heal`
  (params (Amount :type "Float (double-precision)"))
  (returns (NewHealth :type "Float (double-precision)"))
  (return 0.0))

(fn `IsAttacking`
  (returns (Attacking :type Boolean))
  (return false))

(fn `IsDead`
  (returns (Dead :type Boolean))
  (return false))

(fn `ReserveAttackToken`
  (params (Amount :type Integer))
  (returns (Success :type Boolean))
  (return false))

(fn `SetActive`
  (params (Active :type Boolean))
  (`SceneComponent.SetVisibility` (`self.Widget`) Active false))

(fn `TakeDamage`
  (params (DamageInfo :type "/Game/COMMON/UTILITIES/Structs/S_DamageInfo Structure") (`Damage Causer` :type "Actor Object Reference"))
  (returns (WasDamaged :type Boolean))
  (return false))

(fn `UserConstructionScript`
  (`SkinnedMeshComponent.SetLeaderPoseComponent` (`self.Torso`) (`self.Mesh`) false false)
  (`SkinnedMeshComponent.SetLeaderPoseComponent` (`self.Pants`) (`self.Mesh`) false false)
  (`SkinnedMeshComponent.SetLeaderPoseComponent` (`self.Foot`) (`self.Mesh`) false false)
  (`SkinnedMeshComponent.SetLeaderPoseComponent` (`self.Head`) (`self.Mesh`) false false)
  (`SkinnedMeshComponent.SetLeaderPoseComponent` (`self.Hands`) (`self.Mesh`) false false))
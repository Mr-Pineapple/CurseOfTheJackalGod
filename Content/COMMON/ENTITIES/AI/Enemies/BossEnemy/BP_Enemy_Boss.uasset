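; Axe-wielding boss enemy character with its own health bar widget, a set of melee and ranged attacks, and damage and death handling.
; Attack events run montages through BPCAttacks or notifies that trigger traces, a homing axe projectile or lightning AOE.
; Teleport is a hidden high-speed flying AI move, while the float ability grants invincibility on a spawned platform.
; Death awards special-bar charge to the damaging player character; poison ticks use looping timers.
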(event `self.ReceiveBeginPlay`
  (bind _bpc_damagesystem (`self.BPC_DamageSystem`))
  ;[1 1 1] HealthBar
  (`parent.ReceiveBeginPlay`)
  (`WidgetComponent.SetWidget` (`self.HealthBar`) null)
  (bind _returnvalue (`|CreateWidget` "/Game/CLIENT/UI/W_BossHealthBar.W_BossHealthBar_C"))
  (bind _output_get (set `self.BossHealthbarWidgetRef` _returnvalue))
  (`/Game/CLIENT/UI/W_BossHealthBar.UpdateHealthPercentage` _output_get (`/Game/COMMON/COMPONENTS/BPC_DamageSystem.Health` _bpc_damagesystem) (`/Game/COMMON/COMPONENTS/BPC_DamageSystem.MaxHealth` _bpc_damagesystem))
  (add `self.OnDeath` (delegate `Deactivate HealthBar`)))

(event `Deactivate HealthBar`
  ;[1 1 1] HealthBar
  (`Widget.SetVisibility` (`self.BossHealthbarWidgetRef`) "Hidden"))

(event `/Game/COMMON/ENTITIES/AI/Enemies/AI/BPI_EnemyAI.EquipWeapon`
  ;[1 1 1] Equip/Unequip Weapon
  (bind _returnvalue (`|SpawnActorFromClass` "/Game/COMMON/ENTITIES/BP_Weapon_Axe.BP_Weapon_Axe_C" (`KismetMathLibrary.MakeTransform` (0.0 0.0 0.0)) "Undefined" "MultiplyWithRoot" (`self.WeaponActor`) null))
  (bind _output_get (set `self.WeaponActor` _returnvalue))
  (`self.K2_AttachToComponent` _output_get (`self.Mesh`) "hand_r_axe_socket" "SnapToTarget" "SnapToTarget" "SnapToTarget" true)
  (set `self.IsWieldingWeapon` true)
  (`KismetSystemLibrary.DelayUntilNextTick`)
  (`self.OnWeaponEquipped`))

(event `/Game/COMMON/ENTITIES/AI/Enemies/AI/BPI_EnemyAI.UnequipWeapon`
  ;[1 1 1] Equip/Unequip Weapon
  (`self.K2_DestroyActor` (`self.WeaponActor`))
  (set `self.IsWieldingWeapon` false)
  (`KismetSystemLibrary.DelayUntilNextTick`)
  (`self.OnWeaponUnequipped`))

(event `Teleport`
  (params (Location :type "Vector Structure") (AttackTarget :type "Actor Object Reference"))
  (bind _charactermovement (`self.CharacterMovement`))
  ;[1 1 1] TELEPORT
  (if (not (`self.IsTeleporting`))
    (set `self.IsTeleporting` true)
    (`CharacterMovementComponent.SetMovementMode` _charactermovement "MOVE_Flying" 0)
    (set `CharacterMovementComponent.MaxFlySpeed` 5000.0 _charactermovement)
    (set `CharacterMovementComponent.MaxAcceleration` 99999.0 _charactermovement)
    (`SceneComponent.SetVisibility` (`self.Mesh`) false true)
    (`PrimitiveComponent.SetCollisionResponseToChannel` (`self.CapsuleComponent`) "ECC_Pawn" "ECR_Ignore")
    (`self.StopAnimMontage` null)
    (`|AIMoveTo` self Location AttackTarget 150.0
      (:`OnSuccess`
        _)
      (:`OnFail`
        _))
    (`self.TeleportEnd`)
    (else
      (`KismetSystemLibrary.DelayUntilNextTick`)
      (`self.OnTeleportEnd`))))

(event `TeleportEnd`
  (bind _charactermovement (`self.CharacterMovement`))
  ;[1 1 1] TELEPORT
  (`MovementComponent.StopMovementImmediately` _charactermovement)
  (`CharacterMovementComponent.SetMovementMode` _charactermovement "MOVE_Walking" 0)
  (set `CharacterMovementComponent.MaxAcceleration` 1500.0 _charactermovement)
  (`SceneComponent.SetVisibility` (`self.Mesh`) true true)
  (`PrimitiveComponent.SetCollisionResponseToChannel` (`self.CapsuleComponent`) "ECC_Pawn" "ECR_Block")
  (`self.OnTeleportEnd`)
  (`KismetSystemLibrary.Delay` 0.5)
  (set `self.IsTeleporting` false))

(event `AttackCombo1`
  (params (AttackTarget :type "Actor Object Reference"))
  ;[1 1 1] Attacks
  (`/Game/COMMON/COMPONENTS/BPC_Attacks.PrimaryMeleeAttack` (`self.BPC_Attacks`) (make `/Game/COMMON/UTILITIES/S_AttackInfo` AttackTarget "/Game/COMMON/UTILITIES/Animations/Axe/Montage_Axe_Combo_1.Montage_Axe_Combo_1" (make `/Game/COMMON/UTILITIES/S_DamageInfo` 20.0 "NewEnumerator1" "NewEnumerator1" false true true)) 40.0 220.0))

(event `StartFloat`
  (bind _returnvalue (`self.K2_GetActorLocation`))
  ;[1 1 1] Floating Pillar Ability
  (set `/Game/COMMON/COMPONENTS/BPC_DamageSystem.IsInvincible` true (`self.BPC_DamageSystem`))
  (bind _outhit (`KismetSystemLibrary.LineTraceSingle` _returnvalue (* _returnvalue (1.0 1.0 -1000.0)) "TraceTypeQuery1"))
  (bind _returnvalue_2 (`|SpawnActorFromClass` "/Game/COMMON/ENTITIES/Props/BP_FloatingPlatform.BP_FloatingPlatform_C" (`KismetMathLibrary.MakeTransform` (`.Location` (`GameplayStatics.BreakHitResult` _outhit))) "Undefined" "MultiplyWithRoot" null null))
  (bind _output_get (set `self.FloatingPlatformRef` _returnvalue_2))
  (add `/Game/COMMON/ENTITIES/Props/BP_FloatingPlatform.OnFloatTimelineFinished` _output_get (delegate `OnFloatTimelineFinished_Event`)))

(event `AttackCombo2`
  (params (AttackTarget :type "Actor Object Reference"))
  ;[1 1 1] Attacks
  (`self.Attack` AttackTarget)
  (bind _notifyname (`|PlayMontage` (`self.Mesh`) "/Game/COMMON/UTILITIES/Animations/Axe/Montage_Axe_Combo_2.Montage_Axe_Combo_2")
    (:`OnCompleted`
      (`self.AttackEnd` AttackTarget :!label _label))
    (:`OnInterrupted`
      (goto _label))
    (:`OnNotifyBegin`
      (switch `name` _notifyname
        (:`Slash`
          (`/Game/COMMON/COMPONENTS/BPC_Attacks.SphereTraceDamage` (`self.BPC_Attacks`) (make `/Game/COMMON/UTILITIES/S_DamageInfo` 10.0 "NewEnumerator1" "NewEnumerator1" false true true) 40.0 220.0))
        (:`AOESlash`
          (`/Game/COMMON/COMPONENTS/BPC_Attacks.AOEDamage` (`self.BPC_Attacks`) 300.0 (make `/Game/COMMON/UTILITIES/S_DamageInfo` 10.0 "NewEnumerator3" "NewEnumerator1" false false false true)))))))

(event `OnFloatTimelineFinished_Event`
  ;[1 1 1] Floating Pillar Ability
  (remove `/Game/COMMON/ENTITIES/Props/BP_FloatingPlatform.OnFloatTimelineFinished` (stale `StartFloat` _output_get) (delegate `OnFloatTimelineFinished_Event`))
  (`self.OnFloatHeightReached`))

(event `StopFloat`
  ;[1 1 1] Floating Pillar Ability
  (bind _floatingplatformref (`self.FloatingPlatformRef`)
    (:`then`
      (`/Game/COMMON/ENTITIES/Props/BP_FloatingPlatform.StopFloating` _floatingplatformref)
      (add `/Game/COMMON/ENTITIES/Props/BP_FloatingPlatform.OnFloatTimelineFinished` _floatingplatformref (delegate `OnFloatTimelineFinished_Event_0`)))
    (:`else`
      (`KismetSystemLibrary.DelayUntilNextTick`)
      (set `/Game/COMMON/COMPONENTS/BPC_DamageSystem.IsInvincible` false (`self.BPC_DamageSystem`) :!label _label_2)
      (`self.OnFloatEnded`))))

(event `OnFloatTimelineFinished_Event_0`
  ;[1 1 1] Floating Pillar Ability
  (remove `/Game/COMMON/ENTITIES/Props/BP_FloatingPlatform.OnFloatTimelineFinished` (stale `StopFloat` _floatingplatformref) (delegate `OnFloatTimelineFinished_Event_0`))
  (`self.K2_DestroyActor` (stale `StopFloat` _floatingplatformref))
  (goto _label_2))

(event `ThrowAxe`
  (params (AttackTarget :type "Actor Object Reference"))
  ;[1 1 1] Attacks
  (`self.Attack` AttackTarget)
  (bind _notifyname (`|PlayMontage` (`self.Mesh`) "/Game/COMMON/UTILITIES/Animations/Axe/Montage_Axe_Throw.Montage_Axe_Throw")
    (:`OnCompleted`
      (`SceneComponent.SetVisibility` (`/Game/COMMON/ENTITIES/BP_Weapon_Base.Mesh` (`self.WeaponActor`)) true false :!label _label_3)
      (`/Game/COMMON/ENTITIES/AI/Enemies/AI/BPI_EnemyAI.AttackEnd` AttackTarget))
    (:`OnInterrupted`
      (goto _label_3))
    (:`OnNotifyBegin`
      (switch `name` _notifyname
        (:`Throw`
          (`SceneComponent.SetVisibility` (`/Game/COMMON/ENTITIES/BP_Weapon_Base.Mesh` (`self.WeaponActor`)) false false)
          (bind _returnvalue (`|SpawnActorFromClass` "/Game/COMMON/ENTITIES/Projectiles/BP_Projectile_SpinningAxe.BP_Projectile_SpinningAxe_C" (`KismetMathLibrary.MakeTransform` (`SceneComponent.GetSocketLocation` (`self.Mesh`) "hand_r")) "Undefined" "MultiplyWithRoot" null 4000.0 0.0 AttackTarget true self))
          (add `/Game/COMMON/ENTITIES/Projectiles/BP_Projectile_Base.OnProjectileImpact` _returnvalue (delegate `OnProjectileImpact_Event`)))))))

(event `self.ReceiveAnyDamage`
  (params (Damage :type "Float (single-precision)") (DamageType :type "DamageType Object Reference") (InstigatedBy :type "Controller Object Reference") (DamageCauser :type "Actor Object Reference"))
  (bind _bpc_damagesystem (`self.BPC_DamageSystem`))
  ;[1 1 1] AnyDamage
  (set `/Game/COMMON/COMPONENTS/BPC_DamageSystem.Health` (- (`/Game/COMMON/COMPONENTS/BPC_DamageSystem.Health` _bpc_damagesystem) Damage) _bpc_damagesystem)
  (if (<= (`/Game/COMMON/COMPONENTS/BPC_DamageSystem.Health` _bpc_damagesystem) 0.0)
    (`|ExecutionSequence`
      (:`then_0`
        (`/Engine/EditorBlueprintResources/StandardMacros.IsValid` (`self.WeaponActor`)
          (:`Is Valid`
            (`self.K2_DestroyActor` null))))
      (:`then_1`
        (bind _returnvalue (`GameplayStatics.GetActorOfClass` "/Game/COMMON/ENTITIES/BP_Weapon_Axe.BP_Weapon_Axe_C"))
        (`/Engine/EditorBlueprintResources/StandardMacros.IsValid` _returnvalue
          (:`Is Valid`
            (`self.K2_DestroyActor` _returnvalue))))
      (:`then_2`
        (bind _ascharacter_1 (cast `/Game/COMMON/ENTITIES/Characters/Character1` DamageCauser)
          (:`then`
            (`/Engine/EditorBlueprintResources/StandardMacros.IsValid` _ascharacter_1
              (:`Is Valid`
                (set `/Game/COMMON/ENTITIES/Characters/Character1.LockOn` false _ascharacter_1)
                (bind _output_get (set `/Game/COMMON/ENTITIES/Characters/Character1.SpecialAttackAmount` (+ (`self.SpecialAddAmount`) (`/Game/COMMON/ENTITIES/Characters/Character1.SpecialAttackAmount` _ascharacter_1)) _ascharacter_1))
                (`/Game/CLIENT/RENDERING/Widget/Character1HUD.UpdateSpecialBar` (`/Game/COMMON/ENTITIES/Characters/Character1.Character1HUD` _ascharacter_1) (`KismetMathLibrary.Conv_IntToDouble` _output_get)))))
          (:`CastFailed`
            (bind _ascharacter_2 (cast `/Game/COMMON/ENTITIES/Characters/Character2` DamageCauser)
              (:`then`
                (`/Engine/EditorBlueprintResources/StandardMacros.IsValid` _ascharacter_2
                  (:`Is Valid`
                    (bind _output_get_2 (set `/Game/COMMON/ENTITIES/Characters/Character2.SpecialAttackAmount` (+ (`self.SpecialAddAmount`) (`/Game/COMMON/ENTITIES/Characters/Character2.SpecialAttackAmount` _ascharacter_2)) _ascharacter_2))
                    (`/Game/CLIENT/RENDERING/Widget/Character2HUD.UpdateSpecialBar` (`/Game/COMMON/ENTITIES/Characters/Character2.CharacterHUD2` _ascharacter_2) (`KismetMathLibrary.Conv_IntToDouble` _output_get_2)))))
              (:`CastFailed`
                (bind _ascharacter_3 (cast `/Game/COMMON/ENTITIES/Characters/Character3` DamageCauser)
                  (:`then`
                    (`/Engine/EditorBlueprintResources/StandardMacros.IsValid` _ascharacter_3
                      (:`Is Valid`
                        (set `/Game/COMMON/ENTITIES/Characters/Character3.IsStrafing?` false _ascharacter_3)
                        (set `/Game/COMMON/ENTITIES/Characters/Character3.LockOn` false _ascharacter_3)
                        (bind _output_get_3 (set `/Game/COMMON/ENTITIES/Characters/Character3.SpecialAttackAmount` (+ (`self.SpecialAddAmount`) (`/Game/COMMON/ENTITIES/Characters/Character3.SpecialAttackAmount` _ascharacter_3)) _ascharacter_3))
                        (`/Game/CLIENT/RENDERING/Widget/Character3HUD.UpdateSpecialBar` (`/Game/COMMON/ENTITIES/Characters/Character3.Character3HUD` _ascharacter_3) (`KismetMathLibrary.Conv_IntToDouble` _output_get_3)))))
                  (:`CastFailed`
                    (bind _ascharacter_4 (cast `/Game/COMMON/ENTITIES/Characters/Character4` DamageCauser)
                      (:`then`
                        (`/Engine/EditorBlueprintResources/StandardMacros.IsValid` _ascharacter_4
                          (:`Is Valid`
                            (bind _output_get_4 (set `/Game/COMMON/ENTITIES/Characters/Character4.SpecialAttackAmount` (+ (`self.SpecialAddAmount`) (`/Game/COMMON/ENTITIES/Characters/Character4.SpecialAttackAmount` _ascharacter_4)) _ascharacter_4))
                            (`/Game/CLIENT/RENDERING/Widget/Character4HUD.UpdateSpecialBar` (`/Game/COMMON/ENTITIES/Characters/Character4.Character4HUD` _ascharacter_4) (`KismetMathLibrary.Conv_IntToDouble` _output_get_4)))))
                      (:`CastFailed`
                        (bind _asrock_bp (cast `/Game/COMMON/UTILITIES/Pickups/Rock_BP` DamageCauser))
                        (`/Engine/EditorBlueprintResources/StandardMacros.IsValid` _asrock_bp
                          (:`Is Valid`
                            (bind _returnvalue_2 (`GameplayStatics.GetActorOfClass` "/Game/COMMON/ENTITIES/Characters/Character3.Character3_C"))
                            (`/Engine/EditorBlueprintResources/StandardMacros.IsValid` _returnvalue_2
                              (:`Is Valid`
                                (bind _output_get_5 (set `self.SpecialAddAmount` (+ (`self.SpecialAddAmount`) (`/Game/COMMON/ENTITIES/Characters/Character3.SpecialAttackAmount` _returnvalue_2) 0)))
                                (`/Game/CLIENT/RENDERING/Widget/Character3HUD.UpdateSpecialBar` (`/Game/COMMON/ENTITIES/Characters/Character3.Character3HUD` _returnvalue_2) (`KismetMathLibrary.Conv_IntToDouble` _output_get_5)))))))))))))))
      (:`then_3`
        (`self.K2_DestroyActor`)))))

(event `OnProjectileImpact_Event`
  (params (OtherActor :type "Actor Object Reference") (Hit :type "HitResult Structure"))
  ;[1 1 1] Attacks
  (message `/Game/COMMON/UTILITIES/BPI_Damagable.TakeDamage` OtherActor (make `/Game/COMMON/UTILITIES/S_DamageInfo` 10.0 "NewEnumerator2" "NewEnumerator1" false true) self))

(event `QuickAttack`
  (params (AttackTarget :type "Actor Object Reference"))
  ;[1 1 1] Attacks
  (`/Game/COMMON/COMPONENTS/BPC_Attacks.PrimaryMeleeAttack` (`self.BPC_Attacks`) (make `/Game/COMMON/UTILITIES/S_AttackInfo` AttackTarget "/Game/COMMON/UTILITIES/Animations/Axe/Montage_Axe_QuickAttack.Montage_Axe_QuickAttack" (make `/Game/COMMON/UTILITIES/S_DamageInfo` 10.0 "NewEnumerator1" "NewEnumerator1" false true true)) 40.0 220.0))

(event `VFXDamage`
  (params (AmmoType :type "/Game/COMMON/UTILITIES/Enums/PickupAmmoTypes Enum" :default "NewEnumerator0"))
  ;[1 1 1] VFX Damage Event
  (switch `/Game/COMMON/UTILITIES/Enums/PickupAmmoTypes` AmmoType
    (:`NewEnumerator0`
      (`GameplayStatics.SpawnEmitterAttached` "/Game/CLIENT/UTILITIES/VFX/FXVarietyPack/Particles/P_ky_magicCircle1.P_ky_magicCircle1" (`self.DamageVFXLocation`)))
    (:`NewEnumerator1`
      (`GameplayStatics.SpawnEmitterAttached` "/Game/CLIENT/UTILITIES/VFX/FXVarietyPack/Particles/P_ky_healAura.P_ky_healAura" (`self.DamageVFXLocation`)))
    (:`NewEnumerator2`
      (`GameplayStatics.SpawnEmitterAttached` "/Game/CLIENT/UTILITIES/Particles/Particles/P_Explosion.P_Explosion" (`self.DamageVFXLocation`)))
    (:`NewEnumerator3`
      (`GameplayStatics.SpawnEmitterAttached` "/Game/CLIENT/UTILITIES/Particles/Particles_Smoke/P_Smoke.P_Smoke" (`self.DamageVFXLocation`)))
    (:`NewEnumerator4`
      (`GameplayStatics.SpawnEmitterAttached` "/Game/CLIENT/UTILITIES/Particles/PS_AssualtRifle_Impact.PS_AssualtRifle_Impact" (`self.DamageVFXLocation`)))))

(event `JumpAttack`
  (params (AttackTarget :type "Actor Object Reference"))
  ;[1 1 1] Attacks
  (`/Game/COMMON/COMPONENTS/BPC_Attacks.LongRangeMeleeAttack` (`self.BPC_Attacks`) (make `/Game/COMMON/UTILITIES/S_AttackInfo` AttackTarget "/Game/COMMON/UTILITIES/Animations/Axe/Montage_Axe_JumpAttack.Montage_Axe_JumpAttack" (make `/Game/COMMON/UTILITIES/S_DamageInfo` 10.0 "NewEnumerator3" "NewEnumerator1" false false false true))))

(event `GroundSmash`
  (params (AttackTarget :type "Actor Object Reference"))
  ;[1 1 1] Attacks
  (`/Game/COMMON/COMPONENTS/BPC_Attacks.GroundSmash` (`self.BPC_Attacks`) (make `/Game/COMMON/UTILITIES/S_AttackInfo` AttackTarget "/Game/COMMON/UTILITIES/Animations/Axe/Montage_Axe_GroundSmash.Montage_Axe_GroundSmash" (make `/Game/COMMON/UTILITIES/S_DamageInfo` 10.0 "NewEnumerator3" "NewEnumerator1" false false false true)) 1100.0))

(event `Damage Over Time`
  (params (Damage :type "Float (double-precision)"))
  ;[1 1 1] Damage Over Time
  (if (<= (`self.Health`) 0.0)
    (`self.K2_DestroyActor`)
    (`KismetSystemLibrary.K2_ClearAndInvalidateTimerHandle` (`self.DamageOvertime_TimerHandle`))
    (else
      (bind _returnvalue (`KismetSystemLibrary.K2_SetTimerDelegate` (delegate `Damage Overtime Poison`) 1.0 true))
      (set `self.DamageOvertime_TimerHandle` _returnvalue))))

(event `AOETrail`
  (params (AttackTarget :type "Actor Object Reference"))
  ;[1 1 1] Attacks
  (`self.Attack` AttackTarget)
  (bind _notifyname (`|PlayMontage` (`self.Mesh`) "/Game/COMMON/UTILITIES/Animations/Axe/Montage_Axe_Battlecry.Montage_Axe_Battlecry")
    (:`OnCompleted`
      (`self.AttackEnd` AttackTarget :!label _label_4))
    (:`OnInterrupted`
      (goto _label_4))
    (:`OnNotifyBegin`
      (switch `name` _notifyname
        (:`Strike`
          (bind _returnvalue (`|SpawnActorFromClass` "/Game/COMMON/ENTITIES/AbilitiesAndAOE/BP_AOE_LightningStrike.BP_AOE_LightningStrike_C" (`KismetMathLibrary.MakeTransform` (0.0 0.0 0.0)) "Undefined" "MultiplyWithRoot" null 1.0 AttackTarget "/Game/COMMON/ENTITIES/AbilitiesAndAOE/Decals/Decal_AOE_LightningStrike_RED.Decal_AOE_LightningStrike_RED" false false false null))
          (set `/Game/COMMON/ENTITIES/AbilitiesAndAOE/BP_AOE_Blast_Base.BlastEffect` "/Game/CLIENT/UTILITIES/VFX/FXVarietyPack/Particles/P_ky_lightning3_RED.P_ky_lightning3_RED" _returnvalue)
          (add `/Game/COMMON/ENTITIES/AbilitiesAndAOE/BP_AOE_Base.OnAOEOverlapActor` _returnvalue (delegate `OnAOEOverlapActor_Event`)))))))

(event `Damage Overtime Poison`
  ;[1 1 1] Damage Over Time
  (bind _result (`/Engine/EditorBlueprintResources/StandardMacros.IncrementInt` (`self.DamageOvertimeCounter`))
    (:`  `
      (bind _output_get (set `self.DamageOvertimeCounter` _result))
      (set `self.Health` (- (`self.Health`) (stale `Damage Over Time` Damage)))
      (if (<= (`self.Health`) 0.0)
        (`self.K2_DestroyActor`)
        (`KismetSystemLibrary.K2_ClearAndInvalidateTimerHandle` (`self.DamageOvertime_TimerHandle`))
        (elif (>= _output_get 5)
          (`KismetSystemLibrary.K2_ClearAndInvalidateTimerHandle` (`self.DamageOvertime_TimerHandle`))
          (set `self.DamageOvertimeCounter` 0))))))

(event `OnAOEOverlapActor_Event`
  (params (Actor :type "Actor Object Reference"))
  ;[1 1 1] Attacks
  (bind _teamnumber (message `/Game/COMMON/UTILITIES/BPI_Damagable.GetTeamNumber` Actor))
  (if (!= _teamnumber (`self.TeamNumber`))
    (message `/Game/COMMON/UTILITIES/BPI_Damagable.TakeDamage` Actor (make `/Game/COMMON/UTILITIES/S_DamageInfo` 10.0 "NewEnumerator3" "NewEnumerator1") self)))

(fn `CanBeTargeted`
  (returns (ReturnValue :type Boolean))
  (return false))

(fn `GetCurrentHealth`
  (returns (Health :type "Float (double-precision)"))
  (return 0.0))

(fn `GetMaxHealth`
  (returns (MaxHealth :type "Float (double-precision)"))
  (return 0.0))

(fn `SetMovementSpeed`
  (params (Speed :type "/Game/COMMON/ENTITIES/AI/Enemies/AI/Enums/E_MovementSpeed Enum" :default "NewEnumerator0"))
  (returns (SpeedValue :type "Float (double-precision)"))
  (bind _output_get (set `CharacterMovementComponent.MaxWalkSpeed` (select `/Game/COMMON/ENTITIES/AI/Enemies/AI/Enums/E_MovementSpeed` Speed :`NewEnumerator1` 100.0 :`NewEnumerator2` 200.0 :`NewEnumerator3` 350.0 :!type "Float (single-precision)") (`self.CharacterMovement`)))
  (return _output_get))

(fn `TakeDamage`
  (params (DamageInfo :type "/Game/COMMON/UTILITIES/S_DamageInfo Structure") (`Damage Causer` :type "Actor Object Reference"))
  (returns (WasDamaged :type Boolean))
  (bind _bpc_damagesystem (`self.BPC_DamageSystem`))
  (bind _wasdamaged (`parent.TakeDamage` DamageInfo `Damage Causer`))
  (`/Engine/EditorBlueprintResources/StandardMacros.IsValid` _bpc_damagesystem
    (:`Is Valid`
      (`/Game/CLIENT/UI/W_BossHealthBar.UpdateHealthPercentage` (`self.BossHealthbarWidgetRef`) (`/Game/COMMON/COMPONENTS/BPC_DamageSystem.Health` _bpc_damagesystem) (`/Game/COMMON/COMPONENTS/BPC_DamageSystem.MaxHealth` _bpc_damagesystem))
      (return _wasdamaged))))

(fn `UserConstructionScript`
  (bind _bpc_damagesystem (`self.BPC_DamageSystem`))
  (`parent.UserConstructionScript`)
  (bind _output_get (set `/Game/COMMON/COMPONENTS/BPC_DamageSystem.MaxHealth` 700.0 _bpc_damagesystem))
  (set `/Game/COMMON/COMPONENTS/BPC_DamageSystem.Health` _output_get _bpc_damagesystem))
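; Player throwing component that manages rock and smoke bomb counts, updating the Character3 HUD.
; While aiming with lock-on, Throw plays a montage whose notify spawns a Rock_BP that homes on the locked guard, demo AI or boss.
; Helper functions predict the rock's arc, adjust aim distance by mouse or gamepad, and pitch the view toward a location.
; Smoke bomb spawning is unconnected and spline deletion is an empty stub.
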(event `self.ReceiveBeginPlay`
  (bind _returnvalue (`self.GetOwner`))
  ;[0.08507 0.08507 0.08507] BeginPlay
  ;;[0.07812 0.07812 0.07812] Hud
  (`self.UpdateInventory`)
  ;;[0.05729 0.05729 0.05729] Components References
  (set `self.SplineRef` (`Actor.GetComponentByClass` _returnvalue "/Script/Engine.SplineComponent"))
  (set `self.PostProcessRef` (`Actor.GetComponentByClass` _returnvalue "/Script/Engine.PostProcessComponent"))
  (set `self.MotionWarpRef` (`Actor.GetComponentByClass` _returnvalue "/Script/MotionWarping.MotionWarpingComponent"))
  (set `self.ThrowLocationRef` (`|GetArrayItem` (`Actor.GetComponentsByTag` (`self.GetOwner`) "/Script/Engine.ArrowComponent" "Stealth")))
  (set `self.RockRef` (`|GetArrayItem` (`Actor.GetComponentsByTag` (`self.GetOwner`) "/Script/Engine.StaticMeshComponent" "Rock")))
  (bind _ascharacter_3 (cast `/Game/COMMON/ENTITIES/Characters/Character3` (`GameplayStatics.GetPlayerCharacter` 0)))
  (set `self.Character 3` _ascharacter_3))

(event `Key|Two`
  (params (Key :type "Key Structure"))
  ;[0.09896 0.09896 0.09896] SmokeBomb
)

(event `InputAction|Throw`
  (params (Key :type "Key Structure"))
  ;[0.07118 0.07118 0.07118] Throw Input Actions
  (:`Pressed`
    (bind _returnvalue (`GameplayStatics.GetActorOfClass` "/Game/COMMON/ENTITIES/Characters/Character3.Character3_C"))
    (if (and (`self.Rock_Aiming`) (`/Game/COMMON/ENTITIES/Characters/Character3.LockOn` _returnvalue))
      (`self.ThrowRock`))))

(event `ThrowRock`
  ;[0.03993 0.03993 0.03993] Throw The Seed
  (if (`self.Rock_Aiming`)
    (if (> (`self.Rocks`) 0)
      (if (`/Game/COMMON/ENTITIES/Characters/Character3.LockOn` (stale `InputAction|Throw` _returnvalue))
        (`/Engine/EditorBlueprintResources/StandardMacros.DoOnce` false :!label _label
          (:`Completed`
            (`|PlayMontage` (`Character.Mesh` (`GameplayStatics.GetPlayerCharacter` 0)) "/Game/COMMON/UTILITIES/Animations/Throw.Throw" 2.0
              (:`OnCompleted`
                (goto _label :!via `Reset`))
              (:`OnBlendOut`
                (if (`self.Rock_Aiming`)
                  _))
              (:`OnNotifyBegin`
                (`self.SpawnRock`)))))))))

(event `SpawnRock`
  ;[0.05382 0.05382 0.05382] SpawnRockProjectile
  (bind _returnvalue (`GameplayStatics.GetActorOfClass` "/Game/COMMON/ENTITIES/Characters/Character3.Character3_C"))
  (`KismetSystemLibrary.Delay` 0.1)
  (if (> (`self.Rocks`) 0)
    (`/Engine/EditorBlueprintResources/StandardMacros.IsValid` _returnvalue
      (:`Is Valid`
        (bind _found_target (`/Game/COMMON/ENTITIES/Characters/Character3.Found Target` _returnvalue))
        (cast `/Game/COMMON/ENTITIES/AI/AI_Guard/BP_Guard` _found_target
          (:`then`
            _)
          (:`CastFailed`
            (cast `/Game/COMMON/COMPONENTS/AI_Component/Demo/DemoAi/BP_AI_DemoCharacter` _found_target
              (:`then`
                _)
              (:`CastFailed`
                (cast `/Game/COMMON/ENTITIES/AI/Enemies/BossEnemy/BP_Enemy_Boss` _found_target)))))
        (set `self.Hit Component` (`/Game/COMMON/ENTITIES/Characters/Character3.Target Component` _returnvalue))
        (bind _returnvalue_2 (`|SpawnActorFromClass` "/Game/COMMON/UTILITIES/Pickups/Rock_BP.Rock_BP_C" (`SceneComponent.K2_GetComponentToWorld` (`self.ThrowLocationRef`)) "AlwaysSpawn" "MultiplyWithRoot" null null))
        (bind _output_get (set `self.Rock_Ref` _returnvalue_2))
        (set `ProjectileMovementComponent.HomingTargetComponent` (`self.Hit Component`) (`/Game/COMMON/UTILITIES/Pickups/StealthSystem_Throwable_BaseClass.ProjectileMovement` _output_get))
        (`/Engine/EditorBlueprintResources/StandardMacros.DecrementInt` (`self.Rocks`)
          (:`  `
            (`self.UpdateInventory`)))))))

(event `/Game/COMMON/UTILITIES/WeaponBlueprints/PickUp_BPI.PickUpSmokeBomb`
  ;[0.09201 0.09201 0.09201] Inventory Changes
  (`/Engine/EditorBlueprintResources/StandardMacros.IncrementInt` (`self.SmokeBombs`)
    (:`  `
      (`self.UpdateInventory`))))

(event `/Game/COMMON/UTILITIES/WeaponBlueprints/PickUp_BPI.PickUpRock`
  ;[0.09201 0.09201 0.09201] Inventory Changes
  (`/Engine/EditorBlueprintResources/StandardMacros.IncrementInt` (`self.Rocks`)
    (:`  `
      (`self.UpdateInventory`))))

(event `UpdateInventory`
  ;[0.09201 0.09201 0.09201] Inventory Changes
  (bind _returnvalue (`GameplayStatics.GetActorOfClass` "/Game/COMMON/ENTITIES/Characters/Character3.Character3_C"))
  (`/Engine/EditorBlueprintResources/StandardMacros.IsValid` _returnvalue
    (:`Is Valid`
      (bind _character3hud (`/Game/COMMON/ENTITIES/Characters/Character3.Character3HUD` _returnvalue))
      (`/Engine/EditorBlueprintResources/StandardMacros.IsValid` _character3hud
        (:`Is Valid`
          (`/Game/CLIENT/RENDERING/Widget/Character3HUD.UpdateInventory` _character3hud (`KismetTextLibrary.Conv_IntToText` (`self.Rocks`)) (`KismetTextLibrary.Conv_IntToText` (`self.SmokeBombs`))))))))

(fn `Aim Distance Gamepad`
  (params (A :type "Float (double-precision)"))
  (bind _returnvalue (`KismetMathLibrary.FInterpTo` (`self.Rock_Direction`) (+ (`self.Rock_Direction`) (* A -1.0)) (`GameplayStatics.GetWorldDeltaSeconds`) 1.0))
  (if (`self.Rock_Aiming`)
    (if (and (> _returnvalue -0.75) (< _returnvalue 1.5))
      (set `self.Rock_Direction` _returnvalue))))

(fn `AimDistance_Mouse`
  (params (A :type "Float (double-precision)"))
  (bind _returnvalue (`KismetMathLibrary.FInterpTo` (`self.Rock_Direction`) (+ (`self.Rock_Direction`) (* A 1.3)) (`GameplayStatics.GetWorldDeltaSeconds`) 1.0))
  (if (`self.Rock_Aiming`)
    (if (and (> _returnvalue -0.5) (< _returnvalue 0.9))
      (set `self.Rock_Direction` _returnvalue))))

(fn `RockTrajectory`
  (returns (OutPathPositions :type "Array of Vector Structure") (Distance :type "Float (single-precision)") (Location :type "Vector Structure"))
  (bind _throwlocationref (`self.ThrowLocationRef`))
  (bind _rock_direction (`self.Rock_Direction`))
  (bind _returnvalue (`KismetMathLibrary.GetForwardVector` (`SceneComponent.K2_GetComponentRotation` _throwlocationref)))
  (bind _output_get (set `self.Rock_Velocity` (* (+ _returnvalue (* _returnvalue _rock_direction)) (`self.Rock_ProjectileSpeed`))))
  (bind (_outhit _outpathpositions) (`GameplayStatics.Blueprint_PredictProjectilePath_ByTraceChannel` (+ (`SceneComponent.K2_GetComponentLocation` _throwlocationref) _returnvalue) _output_get true 10.0 "ECC_Visibility" false (`|MakeArray` (`self.Rock_Ref`) :!type "Actor Object Reference") "None" 0.0 (`KismetMathLibrary.Lerp` 3.0 14.0 (+ _rock_direction 0.5))))
  (bind (_bblockinghit _binitialoverlap _time _distance _location) (`GameplayStatics.BreakHitResult` _outhit))
  (return _outpathpositions _distance _location))

(fn `StealthInterface_DeleteSplines`
  (params (SplineArray :type "Array of SplineMeshComponent Object Reference (by ref)"))
  (return))

(fn `ThrowRock_PitchTowardsTarget`
  (params (Location :type "Vector Structure"))
  (bind _returnvalue (`GameplayStatics.GetPlayerCharacter` 0))
  (bind _returnvalue_2 (`Pawn.GetController` _returnvalue))
  (bind _returnvalue_3 (`Controller.GetControlRotation` _returnvalue_2))
  (bind (_returnvalue_roll _returnvalue_pitch _returnvalue_yaw) (`KismetMathLibrary.BreakRotator` (`KismetMathLibrary.FindLookAtRotation` (`SceneComponent.K2_GetComponentLocation` (`self.CameraRef`)) Location)))
  (`/Engine/EditorBlueprintResources/StandardMacros.IsValid` _returnvalue
    (:`Is Valid`
      (`/Engine/EditorBlueprintResources/StandardMacros.IsValid` _returnvalue_2
        (:`Is Valid`
          (`Controller.SetControlRotation` _returnvalue_2 (`KismetMathLibrary.MakeRotator` (.roll _returnvalue_3) (.pitch (`KismetMathLibrary.RInterpTo` _returnvalue_3 (`KismetMathLibrary.MakeRotator` _returnvalue_roll _returnvalue_pitch _returnvalue_yaw) (`GameplayStatics.GetWorldDeltaSeconds`) 7.0)) (.yaw _returnvalue_3))))))))